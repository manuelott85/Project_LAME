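; Base class for defender pickups, which only the defending player can see and interact with via a billboard and sphere.
; BeginPlay disables collision, then, only if the local pawn is a BP_VillainGameplay, enables query collision and shows the billboard after a random delay.
; When destroyed, the authority asks the parent generator to spawn a new pickup, and any referenced billboard actor is removed.
; A separate event plays the pickup sound client-side.
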(event `self.ReceiveDestroyed`
  (bind _billboardreference (`self.BillboardReference`))
  ;[1 1 1] Destroyed
  (`|ExecutionSequence`
    (:`then_0`
      (`/Engine/EditorBlueprintResources/ActorMacros.Switch Has Authority`
        (:`Authority`
          ;[1 1 1] Spawn a new Pickup
          (`/Game/Blueprints/BP_DroneSpawner.Server_SpawnPickup` (`self.ParentGenerator`)))))
    (:`then_1`
      ;[1 1 1] Remove the billboard
      (`/Engine/EditorBlueprintResources/StandardMacros.IsValid` _billboardreference
        (:`Is Valid`
          (`self.K2_DestroyActor` _billboardreference))))))

(event `PlayClientsideEffects`
  ;[1 1 1] Play a sound
  (`GameplayStatics.PlaySoundAtLocation` (`self.SoundPlayedByPickingUp`) (`self.K2_GetActorLocation`) (struct) 1.0 1.0 0.0 null null null))

(event `self.ReceiveBeginPlay`
  ;[1 1 1] Deactivate Collision for everyone
  (`PrimitiveComponent.SetCollisionEnabled` (`self.Sphere`) "NoCollision")
  ;[1 1 1] Only the Defending player should proceed
  (bind _asbp_player_controller (cast `/Game/Blueprints/BP_PlayerController` (`GameplayStatics.GetPlayerController` 0)))
  (cast `/Game/Blueprints/BP_VillainGameplay` (`Controller.K2_GetPawn` _asbp_player_controller))
  ;[1 1 1] Activate the posibility for the defender to interact/click on that actor after the delay
  (`KismetSystemLibrary.Delay` (`KismetMathLibrary.RandomFloatInRange` (`self.MinSpawnTimeInSec`) (`self.MaxSpawnTimeInSec`)))
  (`PrimitiveComponent.SetCollisionEnabled` (`self.Sphere`) "QueryOnly")
  ;[1 1 1] Show the billboard if defending player
  (`SceneComponent.SetVisibility` (`self.Billboard`) true true))

(fn `UserConstructionScript`)