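; Spawning component that lets a BP_Defender_Base owner spend energy to spawn drones at the current spawner position.
; SpawnDrone checks and deducts the drone class's energy cost, then a server event spawns it inside the DoN navigable world, trying a random nearby point if outside.
; A replicated drone count, seeded at BeginPlay from existing non-carrier drones, refreshes the HUD through OnRep.
; It also toggles the spawn-menu widget and creates in-world spawn widget actors.
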(event `self.ReceiveBeginPlay`
  ;[1 1 1] Only the owning client should execute
  (if (== (`Controller.K2_GetPawn` (`GameplayStatics.GetPlayerController` 0)) (`self.GetOwner` self))
    ;[1 1 1] Wait for the HUD reference
    (`KismetSystemLibrary.Delay` 1.0)
    (`self.Server_InitCurrentNumberOfDrones`)
    (`self.UpdateHUD_CurrentNumberOfDrones`)))

(event `Server_InitCurrentNumberOfDrones`
  ;[1 1 1] Get all drones
  (bind _outactors (`GameplayStatics.GetAllActorsOfClass` "/Game/Blueprints/AI/BP_Drone_Base.BP_Drone_Base_C"))
  (if (> (`KismetArrayLibrary.Array_Length` _outactors) 0)
    ;[1 1 1] Increment the current number for every drone except carriers
    (for _array_element _outactors
      (cast `/Game/Blueprints/AI/EnergyDelivery/BP_CarrierDrone_Base` _array_element
        (:`CastFailed`
          (set `self.CurrentNumberOfDrones` (+ (`self.CurrentNumberOfDrones`) 1)))))))

(event `Server_SpawnDrone`
  (params (SpawnObject :type "/Game/Blueprints/AI/BP_Drone_Base Class Reference") (SpawnLocation :type "Vector Structure") (InvestigateLocation :type "Vector Structure"))
  ;[1 1 1] Spawn a Drone
  (bind _asbp_game_state (cast `/Game/Blueprints/BP_GameState` (`GameplayStatics.GetGameState`))
    (:`then`
      (bind _donnavigationmanager (`/Game/Blueprints/BP_GameState.DonNavigationManager` _asbp_game_state))
      (`/Engine/EditorBlueprintResources/StandardMacros.IsValid` _donnavigationmanager
        (:`Is Valid`
          (if (`DonNavigationManager.IsLocationWithinNavigableWorld` _donnavigationmanager SpawnLocation)
            (bind _returnvalue (`|SpawnActorFromClass` SpawnObject (`KismetMathLibrary.MakeTransform` SpawnLocation) "DontSpawnIfColliding" "OverrideRootScale" null InvestigateLocation null))
            (`/Engine/EditorBlueprintResources/StandardMacros.IsValid` _returnvalue
              (:`Is Valid`
                (set `self.CurrentNumberOfDrones` (+ (`self.CurrentNumberOfDrones`) 1) :!label _label))
              (:`Is Not Valid`
                (`KismetSystemLibrary.PrintString` (`KismetStringLibrary.Conv_VectorToString` SpawnLocation))))
            (else
              (bind (_bfoundvalidresult _returnvalue_2) (`DonNavigationManager.FindRandomPointAroundOriginInNavWorld` _donnavigationmanager null SpawnLocation 300.0 -1.0 50.0 5))
              (if _bfoundvalidresult
                (bind _returnvalue_3 (`|SpawnActorFromClass` SpawnObject (`KismetMathLibrary.MakeTransform` _returnvalue_2) "DontSpawnIfColliding" "OverrideRootScale" null InvestigateLocation null))
                (`/Engine/EditorBlueprintResources/StandardMacros.IsValid` _returnvalue_3
                  (:`Is Valid`
                    (goto _label)))
                (else
                  (`KismetSystemLibrary.PrintString` "BP_SpawningComponent: No valid location to spawn at found!"))))))))
    (:`CastFailed`
      (`KismetSystemLibrary.PrintString` "BP_SpawningComponent: No Navigation Manager found!" true true (struct :`R` 1.0 :`B` 0.016369 :`A` 1.0) 60.0))))

(event `UpdateHUD_CurrentNumberOfDrones`
  (bind _activehud (`self.ActiveHUD`))
  ;[1 1 1] Update Drone HUD
  (`/Engine/EditorBlueprintResources/StandardMacros.IsValid` _activehud
    (:`Is Valid`
      (`TextBlock.SetText` (`/Game/Widget/W_VillainHUD.AmountDrones` _activehud) (`KismetTextLibrary.Conv_StringToText` (`KismetStringLibrary.Concat_StrStr` (`KismetStringLibrary.Conv_IntToString` (`self.CurrentNumberOfDrones`)) "/" (`KismetStringLibrary.Conv_IntToString` (`self.MaxNumberOfDrones`))))))))

(fn `AlterCurNumDrones`
  (params (Value :type Integer))
  (set `self.CurrentNumberOfDrones` (+ (`self.CurrentNumberOfDrones`) Value)))

(fn `CreateSpawningWidget`
  ;[1 1 1] destroy any old ones before
  (bind _outactors (`GameplayStatics.GetAllActorsOfClass` "/Game/Blueprints/BP_DroidSpawnWidget.BP_DroidSpawnWidget_C"))
  (for _array_element _outactors
    (`Actor.K2_DestroyActor` _array_element))
  ;[1 1 1] Create the widget
  (`|SpawnActorFromClass` "/Game/Blueprints/BP_DroidSpawnWidget.BP_DroidSpawnWidget_C" (`KismetMathLibrary.MakeTransform` (+ (`self.CurrentSpawnerPosition`) (`KismetMathLibrary.MakeVector` 0.0 0.0 (`self.WidgetSpawnHeight`))) (struct :`Pitch` 90.0 :`Yaw` 174.289398 :`Roll` 84.28952) (`self.WidgetScale`)) "AlwaysSpawn" "OverrideRootScale" null (`self.DroneTypes`) null))

(fn `OnRep_CurrentNumberOfDrones`
  (`self.UpdateHUD_CurrentNumberOfDrones`))

(fn `SpawnDrone`
  (params (DroneType :type "/Game/Blueprints/AI/BP_Drone_Base Class Reference") (InvestigateLocation :type "Vector Structure"))
  (bind (_dronename _dronedescription _energycosts) (defaults `/Game/Blueprints/Components/BP_SpawningComponent` DroneType))
  (bind _asbp_defender_base (cast `/Game/Blueprints/BP_Defender_Base` (`self.GetOwner`)))
  (bind _bp_energycomponent (`/Game/Blueprints/BP_Defender_Base.BP_EnergyComponent` _asbp_defender_base))
  (bind _currentenergy (`/Game/Blueprints/Components/BP_EnergyComponent.CurrentEnergy` _bp_energycomponent))
  (if (>= _currentenergy (`KismetMathLibrary.Conv_IntToDouble` _energycosts))
    (`/Game/Blueprints/Components/BP_EnergyComponent.AlterEnergy` _bp_energycomponent (* -1 (`KismetMathLibrary.Conv_IntToDouble` _energycosts)))
    (`self.Server_SpawnDrone` DroneType (`self.CurrentSpawnerPosition`) (`local.InvestigateLocation`))
    (else
      (`KismetSystemLibrary.PrintString` (`KismetStringLibrary.Concat_StrStr` "Insufficient Energy! You need " (`KismetStringLibrary.Conv_DoubleToString` (- (`KismetMathLibrary.Conv_IntToDouble` _energycosts) _currentenergy)) " more Energy") true true (struct :`R` 1.0 :`G` 0.927642 :`A` 1.0) 10.0))))

(fn `ToggleHUD`
  (bind _spawningwidget (`self.SpawningWidget`))
  (if (not (`KismetSystemLibrary.IsValid` _spawningwidget))
    (bind _returnvalue (`|CreateWidget` "/Game/Widget/W_SpawnDroneContainer.W_SpawnDroneContainer_C"))
    (bind _output_get (set `self.SpawningWidget` _returnvalue))
    (`UserWidget.AddToViewport` _output_get 0)
    (elif (`Widget.IsVisible` _spawningwidget)
      (`Widget.SetVisibility` (`self.SpawningWidget`) "Collapsed")
      (else
        (`Widget.SetVisibility` (`self.SpawningWidget`) "Visible")))))