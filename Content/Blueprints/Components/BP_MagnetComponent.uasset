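; Grappling-hook "magnet" component that pulls a BP_Attacker_Base character to the top of aimed-at meshes, using recharging charges.
; ActivateMagnetV2 traces for a ledge height, checks line of sight and charges, then spawns BP_GrappleProjectile.
; Once StartMovement runs, server Tick drives Flying movement input until arrival and recharges charges.
; RepNotifies toggle input, acceleration and audio and refresh the HUD; older ActivateMagnet and MoveToTarget versions remain, uncalled here.
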(event `self.ReceiveBeginPlay`
  ;[1 1 1] BeginPlay = Initialization
  (set `self.CurrentCharges` (`self.MaximumCharges`))
  (bind _asbp_attacker_base (cast `/Game/Blueprints/BP_Attacker_Base` (`self.GetOwner`)))
  (set `self.DefaultAcceleration` (`CharacterMovementComponent.GetMaxAcceleration` (`Character.CharacterMovement` _asbp_attacker_base)))
  (`KismetSystemLibrary.Delay` 0.2)
  (`self.UpdateUI`))

(event `StartMovement`
  ;[1 1 1] Start Moving Towards Target
  (set `self.MagnetActive` true)
  (`self.PlayGrapplePullOnClient`))

(event `self.ReceiveTick`
  (params (DeltaSeconds :type "Float (single-precision)"))
  ;[1 1 1] EventTick = Update Cooldown And Tell Client To Move To Target
  (if (or (`KismetSystemLibrary.IsServer`) (`KismetSystemLibrary.IsDedicatedServer`))
    (`|ExecutionSequence`
      (:`then_0`
        (if (`self.MagnetActive`)
          (`self.MoveToTargetV2` DeltaSeconds)))
      (:`then_1`
        (`self.UpdateCooldown` DeltaSeconds)))))

(event `SetPlayerLocation`
  (params (TargetLocation :type "Vector Structure") (PlayerCharacter :type "/Game/Blueprints/BP_Attacker_Base Object Reference"))
  (bind _charactermovement (`Character.CharacterMovement` PlayerCharacter))
  ;[1 1 1] Move To Target Location (Client)
  (if (`|EnumInequality` (`CharacterMovementComponent.MovementMode` _charactermovement) "MOVE_Flying")
    (`CharacterMovementComponent.SetMovementMode` _charactermovement "MOVE_Flying" 0))
  (`Pawn.AddMovementInput` PlayerCharacter (`KismetMathLibrary.Normal` (- TargetLocation (`Actor.K2_GetActorLocation` PlayerCharacter))) 1.0 true))

(event `PlayGrappleShotOnClient`
  ;[1 1 1] Play Sound Effect On Client
  (`GameplayStatics.PlaySoundAtLocation` "/Game/Sounds/Grappeling_firing.Grappeling_firing" (`Actor.K2_GetActorLocation` (`self.GetOwner`)) (struct) 1.0 1.0 0.0 null null null))

(event `PlayGrapplePullOnClient`
  (bind _asbp_attacker_base (cast `/Game/Blueprints/BP_Attacker_Base` (`self.GetOwner`)))
  (`AudioComponent.Play` (`/Game/Blueprints/BP_Attacker_Base.Grappeling_pulling_Cue` _asbp_attacker_base) 0.0))

(fn `ActivateMagnet`
  (params (StartPosition :type "Vector Structure") (Direction :type "Vector Structure"))
  (locals (Debug :type Boolean :default false) (ObjectLocation :type "Vector Structure"))
  (bind (_outhit _returnvalue) (`KismetSystemLibrary.LineTraceSingle` :`Start` StartPosition :`End` (+ StartPosition (* Direction (`self.Range`))) :`TraceChannel` "TraceTypeQuery1" :`DrawDebugType` "ForOneFrame" :`DrawTime` 1000.0))
  (if _returnvalue
    (bind (_bblockinghit _binitialoverlap _time _distance _location _impactpoint _normal _impactnormal _physmat _hitactor _hitcomponent) (`GameplayStatics.BreakHitResult` _outhit))
    (if (`KismetSystemLibrary.IsValid` _hitactor)
      (set `self.Target` _hitactor)
      (set `local.ObjectLocation` (`Actor.K2_GetActorLocation` _hitactor))
      (else
        (set `self.Target` _hitcomponent)
        (set `local.ObjectLocation` (`SceneComponent.K2_GetComponentLocation` _hitcomponent))))
    (if (`local.Debug`)
      (`KismetSystemLibrary.DrawDebugSphere` StartPosition 50.0 4 (struct :`R` 0.035435 :`G` 1.0 :`A` 1.0) 500.0 3.0)
      (`KismetSystemLibrary.DrawDebugSphere` _location 50.0 4 (struct :`R` 1.0 :`B` 0.265872 :`A` 1.0) 500.0 3.0)
      (`KismetSystemLibrary.PrintText` (`KismetTextLibrary.Conv_VectorToText` _location)))
    (bind _output_get (set `self.ImpactLocationOffset` (- (`local.ObjectLocation`) _location)))
    (if (`local.Debug`)
      (`KismetSystemLibrary.PrintText` (`KismetTextLibrary.Conv_VectorToText` _output_get)))
    (set `self.MagnetActive` true)
    (`GameplayStatics.PlaySoundAtLocation` "/Game/Sounds/Grappeling_firing.Grappeling_firing" (`Actor.K2_GetActorLocation` (`self.GetOwner`)) (struct) 1.0 1.0 0.0 null null null)
    (bind _asbp_attacker_base (cast `/Game/Blueprints/BP_Attacker_Base` (`self.GetOwner`)))
    (`AudioComponent.Play` (`/Game/Blueprints/BP_Attacker_Base.Grappeling_pulling_Cue` _asbp_attacker_base) 0.0)))

(fn `ActivateMagnetV2`
  (params (StartPosition :type "Vector Structure") (Direction :type "Vector Structure"))
  (locals (Debug :type Boolean :default false) (TargetLocation :type "Vector Structure") (GrappleGunLocation :type "Vector Structure"))
  (if (not (`self.MagnetActive`))
    (bind _output_get (set `local.GrappleGunLocation` StartPosition))
    (bind (_grapplelocation _hittarget) (`self.FindGrappleTarget` _output_get Direction))
    (if _hittarget
      (set `local.TargetLocation` _grapplelocation)
      (if (<= (`KismetMathLibrary.VSize` (- (`local.TargetLocation`) (`local.GrappleGunLocation`))) (`self.Range`))
        (bind _asprimitive_component (cast `PrimitiveComponent` (`self.Target`)))
        (bind _asbp_attacker_base (cast `/Game/Blueprints/BP_Attacker_Base` (`self.GetOwner`)))
        (if (`local.Debug`)
          (bind _returnvalue (+ (`local.TargetLocation`) (`KismetMathLibrary.MakeVector` 0.0 0.0 (`CapsuleComponent.GetScaledCapsuleHalfHeight` (`Character.CapsuleComponent` _asbp_attacker_base)))))
          (`KismetSystemLibrary.DrawDebugSphere` _returnvalue 1.0 4 (struct :`G` 1.0 :`B` 0.306961 :`A` 1.0) 20.0 5.0))
        (bind (_outhit _returnvalue_2) (`KismetSystemLibrary.LineTraceSingle` (`local.GrappleGunLocation`) _returnvalue "TraceTypeQuery1"))
        (if (not _returnvalue_2)
          (bind _sufficientcharges (`self.CheckCharges`))
          (if _sufficientcharges
            (bind _output_get_2 (set `self.ImpactLocationOffset` (- (`SceneComponent.K2_GetComponentLocation` _asprimitive_component) _returnvalue)))
            (if (`local.Debug`)
              (`KismetSystemLibrary.PrintText` (`KismetTextLibrary.Conv_VectorToText` _output_get_2)))
            (bind _returnvalue_3 (`|SpawnActorFromClass` "/Game/Blueprints/BP_GrappleProjectile.BP_GrappleProjectile_C" (`KismetMathLibrary.MakeTransform` (`local.GrappleGunLocation`) (`KismetMathLibrary.FindLookAtRotation` (`local.GrappleGunLocation`) (`local.TargetLocation`)) (1.0 1.0 1.0)) "Undefined" "OverrideRootScale" (`self.GetOwner`) null))
            (set `/Game/Blueprints/BP_GrappleProjectile.Target` (`self.Target`) _returnvalue_3)
            (bind _asbp_attacker_base_2 (cast `/Game/Blueprints/BP_Attacker_Base` (`self.GetOwner`)))
            (set `/Game/Blueprints/BP_GrappleProjectile.ImpactLocationOffset` (+ (`self.ImpactLocationOffset`) (`KismetMathLibrary.MakeVector` 0.0 0.0 (`CapsuleComponent.GetScaledCapsuleHalfHeight` (`Character.CapsuleComponent` _asbp_attacker_base_2)))) _returnvalue_3)
            (`self.PlayGrappleShotOnClient`)
            (set `self.ProjectileShot` true)))))))

(fn `CalculateTargetLocation`
  (returns (HitLocation :type "Vector Structure"))
  (bind _target (`self.Target`))
  (bind _asactor (cast `Actor` _target)
    (:`then`
      (return (- (`Actor.K2_GetActorLocation` _asactor) (`self.ImpactLocationOffset`))))
    (:`CastFailed`
      (bind _asprimitive_component (cast `PrimitiveComponent` _target))
      (return (- (`SceneComponent.K2_GetComponentLocation` _asprimitive_component) (`self.ImpactLocationOffset`))))))

(fn `CalculateUpRotation`
  (params (Rotation :type "Rotator Structure"))
  (returns (CalculatedRotation :type "Rotator Structure"))
  (`|ExecutionSequence`
    (:`then_0`
      (bind _cleanedrotationvalue (`self.CleanupRotation` (.roll Rotation))))
    (:`then_1`
      (bind _cleanedrotationvalue_2 (`self.CleanupRotation` (.pitch Rotation))))
    (:`then_2`
      (return (`KismetMathLibrary.MakeRotator` _cleanedrotationvalue _cleanedrotationvalue_2 (.yaw Rotation))))))

(fn `CheckCharges`
  (returns (SufficientCharges :type Boolean))
  (if (>= (`self.CurrentCharges`) 1)
    (`/Engine/EditorBlueprintResources/StandardMacros.DecrementInt` (`self.CurrentCharges`)
      (:`  `
        (if (<= (`self.CurrentCooldown`) 0.0)
          (set `self.CurrentCooldown` (`self.ChargeCooldown`)))
        (return true)))
    (else
      (`KismetSystemLibrary.PrintString` "Insufficient Magnet Charges")
      (return false))))

(fn `CheckDistance`
  (params (TargetLocation :type "Vector Structure"))
  (returns (LocationReached :type Boolean))
  (locals (Debug :type Boolean))
  (bind _returnvalue (`Actor.K2_GetActorLocation` (`self.GetOwner`)))
  (if (`local.Debug`)
    (`KismetSystemLibrary.DrawDebugSphere` _returnvalue 1.0 4 (struct :`R` 1.0 :`G` 0.021407 :`A` 1.0) 20.0 5.0)
    (`KismetSystemLibrary.DrawDebugSphere` TargetLocation 1.0 4 (struct :`G` 0.356638 :`B` 1.0 :`A` 1.0) 20.0 5.0))
  (return (and (>= (.z _returnvalue) (.z TargetLocation)) (<= (`KismetMathLibrary.VSize` (- TargetLocation _returnvalue)) (`self.DistanceTolerance`)))))

(fn `CleanupRotation`
  (params (RotationValue :type "Float (double-precision)"))
  (returns (CleanedRotationValue :type "Float (double-precision)"))
  (locals (MaxRotation :type "Float (double-precision)" :default 45.0))
  (if (> RotationValue (`local.MaxRotation`))
    (return (- RotationValue (* (`KismetMathLibrary.FFloor` (/ RotationValue (`local.MaxRotation`))) (`local.MaxRotation`))))
    (else
      (return RotationValue))))

(fn `DisableMagnet`
  (locals (PlayerCharacter :type "/Game/Blueprints/BP_Attacker_Base Object Reference"))
  (bind _charactermovement (`Character.CharacterMovement` (`local.PlayerCharacter`)))
  (set `self.MagnetActive` false)
  (bind _asbp_attacker_base (cast `/Game/Blueprints/BP_Attacker_Base` (`self.GetOwner`)))
  (set `local.PlayerCharacter` _asbp_attacker_base)
  (bind _hitlocation (`self.CalculateTargetLocation`))
  (bind _locationreached (`self.CheckDistance` _hitlocation))
  (if _locationreached
    (`MovementComponent.StopMovementImmediately` _charactermovement)
    (else
      (set `MovementComponent.Velocity` (/ (`MovementComponent.Velocity` _charactermovement) (`self.DecelerationSpeed`)) _charactermovement)))
  (`CharacterMovementComponent.SetMovementMode` _charactermovement "MOVE_Falling" 0)
  (`AudioComponent.Stop` (`/Game/Blueprints/BP_Attacker_Base.Grappeling_pulling_Cue` (`local.PlayerCharacter`)))
  (bind _outactors (`GameplayStatics.GetAllActorsOfClass` "/Game/Blueprints/BP_GrappleProjectile.BP_GrappleProjectile_C"))
  (for _array_element _outactors
    (`Actor.K2_DestroyActor` _array_element))
  (set `self.ProjectileShot` false))

(fn `FindGrappleTarget`
  (params (GrappleGunLocation :type "Vector Structure") (GrappleDirection :type "Vector Structure"))
  (returns (GrappleLocation :type "Vector Structure") (HitTarget :type Boolean))
  (locals (TargetLocation :type "Vector Structure") (Debug :type Boolean :default false))
  (bind (_outhit _returnvalue) (`KismetSystemLibrary.LineTraceSingle` :`Start` GrappleGunLocation :`End` (+ GrappleGunLocation (* GrappleDirection (`self.Range`))) :`TraceChannel` "TraceTypeQuery1" :`DrawTime` 1000.0))
  (if _returnvalue
    (if (`local.Debug`)
      (bind (_bblockinghit _binitialoverlap _time _distance _location _impactpoint _normal _impactnormal _physmat _hitactor _hitcomponent) (`GameplayStatics.BreakHitResult` _outhit))
      (`KismetSystemLibrary.PrintString` (`KismetSystemLibrary.GetDisplayName` _hitcomponent)))
    (bind _asstatic_mesh_component (cast `StaticMeshComponent` _hitcomponent)
      (:`then`
        (bind _returnvalue_2 (`self.FindHighestPointInMesh` _asstatic_mesh_component _impactpoint))
        (set `self.Target` _hitcomponent)
        (set `local.TargetLocation` (`KismetMathLibrary.MakeVector` (.x _impactpoint) (.y _impactpoint) _returnvalue_2)))
      (:`CastFailed`
        (bind _asmodel_component (cast `ModelComponent` _hitcomponent))
        (set `self.Target` _asmodel_component)
        (set `local.TargetLocation` _impactpoint)))
    (return (`local.TargetLocation`) true)
    (else
      (return (0.0 0.0 0.0) false))))

(fn `FindHighestPointInMesh`
  (params (StaticMesh :type "StaticMeshComponent Object Reference") (ImpactLocation :type "Vector Structure"))
  (returns (ReturnValue :type "Float (double-precision)"))
  (locals (Rotation :type "Rotator Structure") (Debug :type Boolean :default false) (StartLocation :type "Vector Structure") (EndLocation :type "Vector Structure"))
  (bind (_returnvalue_x _returnvalue_y _returnvalue_z) (`KismetMathLibrary.BreakVector` (`SceneComponent.K2_GetComponentScale` StaticMesh)))
  (bind (_returnvalue_x_2 _returnvalue_y_2 _returnvalue_z_2) (`KismetMathLibrary.BreakVector` (`SceneComponent.K2_GetComponentLocation` StaticMesh)))
  (bind _returnvalue (* (.z (`.Max` (`StaticMeshComponent.GetLocalBounds` StaticMesh))) _returnvalue_z))
  (bind _calculatedrotation (`self.CalculateUpRotation` (`SceneComponent.RelativeRotation` StaticMesh)))
  (if (`local.Debug`)
    (bind _returnvalue_2 (* (`KismetMathLibrary.GreaterGreater_VectorRotator` (0.0 0.0 2.0) _calculatedrotation) _returnvalue))
    (bind _returnvalue_3 (+ _returnvalue_2 ImpactLocation))
    (`KismetSystemLibrary.DrawDebugCircle` _returnvalue_3 1.0 12 (struct :`R` 1.0 :`B` 0.255358 :`A` 1.0) 1.0 4.0)
    (`KismetSystemLibrary.DrawDebugCircle` ImpactLocation 1.0 12 (struct :`G` 0.219651 :`B` 1.0 :`A` 1.0) 1.0 4.0))
  (bind _outhit (`KismetSystemLibrary.LineTraceSingle` _returnvalue_3 (- ImpactLocation _returnvalue_2) "TraceTypeQuery1" true))
  (if (`GameplayStatics.BreakHitResult` _outhit)
    (return (.z (`.Location` (`GameplayStatics.BreakHitResult` _outhit))))
    (else
      (return (+ _returnvalue_z_2 _returnvalue)))))

(fn `MoveToTarget`
  (params (DeltaSeconds :type "Float (double-precision)"))
  (locals (HitLocation :type "Vector Structure") (Debug :type Boolean :default false) (ElapsedTime :type "Float (double-precision)"))
  (bind _hitlocation (`local.HitLocation`))
  (bind (_hitlocation_x _hitlocation_y _hitlocation_z) (`KismetMathLibrary.BreakVector` (`local.HitLocation`)))
  (bind _hitlocation_2 (`local.HitLocation`))
  (bind _hitlocation_3 (`self.CalculateTargetLocation`))
  (bind _output_get (set `local.HitLocation` _hitlocation_3))
  (bind _locationreached (`self.CheckDistance` _output_get))
  (if _locationreached
    (if (`self.LooseVelocityOnLocationReached`)
      ;[1 1 1] Stop moving when reaching target location
      (bind _asbp_attacker_base (cast `/Game/Blueprints/BP_Attacker_Base` (`self.GetOwner`)))
      (set `MovementComponent.Velocity` (0.0 0.0 0.0) (`Character.CharacterMovement` _asbp_attacker_base)))
    (else
      (if (`local.Debug`)
        (`KismetSystemLibrary.DrawDebugSphere` _hitlocation 200.0 4 (struct :`G` 0.140895 :`B` 1.0 :`A` 1.0) 1000.0 5.0)
        (`KismetSystemLibrary.PrintText` (`KismetTextLibrary.Conv_VectorToText` _hitlocation)))
      (bind _asbp_attacker_base_2 (cast `/Game/Blueprints/BP_Attacker_Base` (`self.GetOwner`)))
      (bind _charactermovement (`Character.CharacterMovement` _asbp_attacker_base_2))
      (if (`|EnumInequality` (`CharacterMovementComponent.MovementMode` _charactermovement) "MOVE_Flying")
        (`CharacterMovementComponent.SetMovementMode` _charactermovement "MOVE_Flying" 0))
      (set `CharacterMovementComponent.MaxAcceleration` (`self.MaxTravelSpeed`) _charactermovement)
      (bind _returnvalue (`Actor.K2_GetActorLocation` _asbp_attacker_base_2))
      (`Pawn.AddMovementInput` _asbp_attacker_base_2 (- _hitlocation_2 _returnvalue) 1.0 false)
      (`KismetSystemLibrary.DrawDebugLine` _hitlocation_2 _returnvalue (struct :`G` 0.490464 :`B` 0.647569 :`A` 1.0) 0.0 2.0)
      (bind (_returnvalue_x _returnvalue_y _returnvalue_z) (`KismetMathLibrary.BreakVector` (`Actor.K2_GetActorLocation` _asbp_attacker_base_2)))
      (bind _velocity (`MovementComponent.Velocity` _charactermovement))
      (if (and (>= _returnvalue_z _hitlocation_z) (> (.z _velocity) 0.0))
        (set `MovementComponent.Velocity` (* _velocity (1.0 1.0 0.0)) _charactermovement)))))

(fn `MoveToTargetV2`
  (params (DeltaSeconds :type "Float (double-precision)"))
  (locals (HitLocationLoc :type "Vector Structure") (Debug :type Boolean :default false) (ElapsedTime :type "Float (double-precision)") (PlayerCharacter :type "/Game/Blueprints/BP_Attacker_Base Object Reference"))
  (bind _hitloaction (`self.HitLoaction`))
  (set `local.ElapsedTime` DeltaSeconds)
  (bind _hitlocation (`self.CalculateTargetLocation`))
  (bind _output_get (set `self.HitLoaction` _hitlocation))
  (bind _locationreached (`self.CheckDistance` _output_get))
  (if _locationreached
    ;[1 1 1] Disable grapple when reaching target
    (`self.DisableMagnet`)
    (else
      (if (`local.Debug`)
        (`KismetSystemLibrary.DrawDebugSphere` _hitloaction 200.0 4 (struct :`G` 0.140895 :`B` 1.0 :`A` 1.0) 1000.0 5.0)
        (`KismetSystemLibrary.PrintText` (`KismetTextLibrary.Conv_VectorToText` _hitloaction)))
      (bind _asbp_attacker_base (cast `/Game/Blueprints/BP_Attacker_Base` (`self.GetOwner`)))
      (bind _output_get_2 (set `local.PlayerCharacter` _asbp_attacker_base))
      (bind _charactermovement (`Character.CharacterMovement` _output_get_2))
      (if (`|EnumInequality` (`CharacterMovementComponent.MovementMode` _charactermovement) "MOVE_Flying")
        (`CharacterMovementComponent.SetMovementMode` _charactermovement "MOVE_Flying" 0))
      (`self.SetPlayerLocation` (`KismetMathLibrary.VInterpTo_Constant` (`Actor.K2_GetActorLocation` _output_get_2) (`self.HitLoaction`) (`local.ElapsedTime`) (* (`self.GrappleSpeed`) 300.0)) (`local.PlayerCharacter`)))))

(fn `OnRep_CurrentCooldown`
  (`self.UpdateUI`))

(fn `OnRep_MagnetActive`
  (bind _returnvalue (`self.GetOwner`))
  (bind _returnvalue_2 (`Pawn.GetController` (`Actor.Instigator` (`self.GetOwner`))))
  (bind _returnvalue_3 (`Pawn.GetController` (`Actor.Instigator` _returnvalue)))
  (if (not (`self.MagnetActive`))
    (`/Engine/EditorBlueprintResources/StandardMacros.IsValid` _returnvalue_3
      (:`Is Valid`
        (`Controller.SetIgnoreMoveInput` _returnvalue_3 false)
        (bind _asbp_attacker_base (cast `/Game/Blueprints/BP_Attacker_Base` _returnvalue))
        (set `CharacterMovementComponent.MaxAcceleration` (`self.DefaultAcceleration`) (`Character.CharacterMovement` _asbp_attacker_base))
        (`AudioComponent.Stop` (`/Game/Blueprints/BP_Attacker_Base.Grappeling_pulling_Cue` _asbp_attacker_base))
        (`GameplayStatics.PlaySoundAtLocation` "/Game/Sounds/Grappeling_Reconnecting_Cue.Grappeling_Reconnecting_Cue" (`Actor.K2_GetActorLocation` _asbp_attacker_base) (struct) 1.0 1.0 0.0 null null null)))
    (else
      (bind _asbp_attacker_base_2 (cast `/Game/Blueprints/BP_Attacker_Base` (`self.GetOwner`)))
      (set `CharacterMovementComponent.MaxAcceleration` 50000.0 (`Character.CharacterMovement` _asbp_attacker_base_2))
      (`/Engine/EditorBlueprintResources/StandardMacros.IsValid` _returnvalue_2
        (:`Is Valid`
          (`Controller.SetIgnoreMoveInput` _returnvalue_2 true))))))

(fn `OnRep_MaximumCharges`
  (`self.UpdateUI`))

(fn `UpdateCooldown`
  (params (ElapsedTime :type "Float (double-precision)"))
  (if (and (<= (`self.CurrentCooldown`) 0.0) (< (`self.CurrentCharges`) (`self.MaximumCharges`)))
    (`/Engine/EditorBlueprintResources/StandardMacros.IncrementInt` (`self.CurrentCharges`)
      (:`  `
        (if (< (`self.CurrentCharges`) (`self.MaximumCharges`))
          (set `self.CurrentCooldown` (`self.ChargeCooldown`))
          (else
            (set `self.CurrentCooldown` 0.0)))))
    (elif (> (`self.CurrentCooldown`) 0.0)
      (set `self.CurrentCooldown` (- (`self.CurrentCooldown`) ElapsedTime)))))

(fn `UpdateUI`
  (locals (VisibleCharges :type Integer))
  (bind _asbp_attacker_base (cast `/Game/Blueprints/BP_Attacker_Base` (`self.GetOwner`)))
  (bind _asw_hero_hud (cast `/Game/Widget/W_HeroHUD` (`/Game/Blueprints/BP_Attacker_Base.ActiveHUD` _asbp_attacker_base)))
  (bind _magnetcharges (`/Game/Widget/W_HeroHUD.MagnetCharges` _asw_hero_hud))
  (for _index (range (`PanelWidget.GetChildrenCount` _magnetcharges))
    (if (< (`local.VisibleCharges`) (`self.CurrentCharges`))
      (bind _returnvalue (`PanelWidget.GetChildAt` _magnetcharges _index))
      (bind _asimage (cast `Image` _returnvalue)
        (:`then`
          (`Widget.SetVisibility` _asimage "SelfHitTestInvisible")
          (`/Engine/EditorBlueprintResources/StandardMacros.IncrementInt` (`local.VisibleCharges`)))
        (:`CastFailed`
          (`Widget.SetVisibility` _returnvalue "SelfHitTestInvisible")))
      (else
        (`Widget.SetVisibility` _returnvalue "Collapsed")))))