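; Health component for the attacker, drones, generators and mainframe, handling damage, death and segmented regeneration.
; The server applies scaled damage and delayed regeneration through AlterHealth, with regeneration capped by the remaining health segments.
; Attacker death restarts the level, other deaths award attacker XP and can destroy the owner, and damage to the attacker awards defender XP.
; Segment bars are built in the owner's HUD or widget and refreshed by OnRep_CurrentHealth.
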(event `Client_CallClientSideEffects`
  (if (`self.CameraShake`)
    (`self.PerformCameraShake`)))

(event `AlterHealth`
  (params (AmountToAlter :type "Float (double-precision)"))
  (bind _returnvalue (`self.GetOwner`))
  (bind _returnvalue_2 (`GameplayStatics.GetGameMode`))
  (bind _returnvalue_3 (+ AmountToAlter (`self.CurrentHealth`)))
  ;[1 1 1] Alter Health
  (if (or (`KismetSystemLibrary.IsServer`) (`KismetSystemLibrary.IsDedicatedServer`))
    (if (and (`self.ShouldRegenerate`) (> (`self.CurrentHealth`) 0.0))
      (`self.CheckNumberOfHealthSegments`)
      (set `self.CurrentHealth` (`KismetMathLibrary.FClamp` _returnvalue_3 0.0 (`self.MaxHealthToRestore`)))
      (else
        (set `self.CurrentHealth` (`KismetMathLibrary.FClamp` _returnvalue_3 0.0 (`self.MaxHealth`)))))
    (`|ExecutionSequence`
      (:`then_0`
        ;[1 1 1] Is actor dead?
        (if (<= (`self.CurrentHealth`) 0.0)
          ;[1 1 1] Destroy the actor if is not the player or the drone spawner
          (cast `/Game/Blueprints/BP_Attacker_Base` (`self.GetOwner`)
            (:`then`
              ;[1 1 1] Restart current level
              (`/Engine/EditorBlueprintResources/StandardMacros.IsValid` _returnvalue_2
                (:`Is Valid`
                  (bind _asbp_game_mode (cast `/Game/Blueprints/BP_GameMode` _returnvalue_2))
                  (`/Game/Blueprints/BP_GameMode.RestartLevel` _asbp_game_mode))))
            (:`CastFailed`
              (bind _outactors (`GameplayStatics.GetAllActorsOfClass` "/Game/Blueprints/BP_Attacker_Balance.BP_Attacker_Balance_C"))
              (bind _output (`|GetArrayItem` _outactors))
              (`/Game/Blueprints/Components/BP_XPComponent.Alter XP` (`/Game/Blueprints/BP_Attacker_Base.BP_XPComponent` _output) 200)
              (if (`self.ShouldActorBeDestroyed`)
                (cast `/Game/Blueprints/AI/BP_Drone_Base` _returnvalue
                  (:`then`
                    (`/Game/Blueprints/BP_Attacker_Base.DroneDestroyed` _output (`Actor.K2_GetActorLocation` _returnvalue)))
                  (:`CastFailed`
                    _))
                (`Actor.K2_DestroyActor` _returnvalue)
                (`KismetSystemLibrary.PrintString` "destroyed"))))))
      (:`then_1`
        (if (< AmountToAlter 0.0)
          (cast `/Game/Blueprints/BP_Attacker_Base` (`self.GetOwner`))
          (bind _outactors_2 (`GameplayStatics.GetAllActorsOfClass` "/Game/Blueprints/BP_Defender_Base.BP_Defender_Base_C"))
          (if (> (`KismetArrayLibrary.Array_Length` _outactors_2) 0)
            (`/Game/Blueprints/Components/BP_XPComponent.Alter XP` (`/Game/Blueprints/BP_Defender_Base.BP_XPComponent` (`|GetArrayItem` _outactors_2)) (* (`KismetMathLibrary.FTrunc` AmountToAlter) -1))))))))

(event `Remote: Event any Damage`
  (params (Damage :type "Float (double-precision)") (DamageType :type "DamageType Object Reference") (InstigatedBy :type "Controller Object Reference") (DamageCauser :type "Actor Object Reference"))
  ;[1 1 1] ServerOnly! Handle Damage
  (`self.Client_CallClientSideEffects`)
  (`self.AlterHealth` (* (* Damage (`self.DamageMultiplier`)) -1.0))
  (set `self.TimeSinceLastHit` 0.0))

(event `self.ReceiveBeginPlay`
  (bind _returnvalue (`self.GetOwner`))
  (bind _amountofhealthsegments (`self.AmountOfHealthSegments`))
  (bind _activehud (`self.ActiveHUD`))
  (`KismetSystemLibrary.Delay` 0.2)
  (`|ExecutionSequence`
    (:`then_0`
      ;[1 1 1] Initialize Health Segments
      (if (or (`KismetSystemLibrary.IsServer`) (`KismetSystemLibrary.IsDedicatedServer`))
        (for _ (range 1 (+ _amountofhealthsegments 1))
          (`KismetArrayLibrary.Array_Add` (`self.HealthPerSegment`) (/ (`self.MaxHealth`) (`KismetMathLibrary.Conv_IntToDouble` _amountofhealthsegments))))))
    (:`then_1`
      ;[1 1 1] Get a HUD reference
      ;;[1 1 1] Player Widget
      (bind _asbp_attacker_base (cast `/Game/Blueprints/BP_Attacker_Base` _returnvalue)
        (:`then`
          (set `self.ActiveHUD` (`/Game/Blueprints/BP_Attacker_Base.ActiveHUD` _asbp_attacker_base)))
        (:`CastFailed`
          ;;[1 1 1] Drone Widget
          (bind _asbp_drone_base (cast `/Game/Blueprints/AI/BP_Drone_Base` _returnvalue)
            (:`then`
              (set `self.ActiveHUD` (`WidgetComponent.GetUserWidgetObject` (`/Game/Blueprints/AI/BP_Drone_Base.HealthWidget` _asbp_drone_base))))
            (:`CastFailed`
              ;;[1 1 1] DroneSpawner Widget
              (bind _asbp_generator (cast `/Game/Blueprints/BP_Generator` _returnvalue)
                (:`then`
                  (set `self.ActiveHUD` (`WidgetComponent.GetUserWidgetObject` (`/Game/Blueprints/BP_Generator.HealthWidget` _asbp_generator))))
                (:`CastFailed`
                  ;;[1 1 1] Mainframe Widget
                  (bind _asbp_mainframe (cast `/Game/Blueprints/Towers/BP_Mainframe` _returnvalue))
                  (set `self.ActiveHUD` (`WidgetComponent.GetUserWidgetObject` (`/Game/Blueprints/Towers/BP_Mainframe.HealthWidget` _asbp_mainframe))))))))))
    (:`then_2`
      ;[1 1 1] Add HealthBars to HUD
      (bind _asw_hero_hud (cast `/Game/Widget/W_HeroHUD` _activehud)
        (:`then`
          (set `self.HealthBarItem` "/Game/Widget/W_HealthBarElementAttacker.W_HealthBarElementAttacker_C")
          (set `self.HealthbarContainer` (`/Game/Widget/W_HeroHUD.HealthBarContainer` _asw_hero_hud)))
        (:`CastFailed`
          (bind _asw_healthbar (cast `/Game/Widget/W_Healthbar` _activehud))
          (set `self.HealthBarItem` "/Game/Widget/W_HealthBarElement.W_HealthBarElement_C")
          (set `self.HealthbarContainer` (`/Game/Widget/W_Healthbar.HealthbarContainer` _asw_healthbar))))
      (for _ (range 1 (+ (`self.AmountOfHealthSegments`) 1))
        (bind _returnvalue_2 (`|CreateWidget` (`self.HealthBarItem`)))
        (`/Engine/EditorBlueprintResources/StandardMacros.IsValid` _returnvalue_2
          (:`Is Valid`
            (bind _asw_health_bar_element (cast `/Game/Widget/W_HealthBarElement` _returnvalue_2)
              (:`then`
                (`KismetArrayLibrary.Array_Add` (`self.HealthBars`) (`/Game/Widget/W_HealthBarElement.HealthBar` _asw_health_bar_element)))
              (:`CastFailed`
                (bind _asw_health_bar_element_attacker (cast `/Game/Widget/W_HealthBarElementAttacker` _returnvalue_2))
                (`KismetArrayLibrary.Array_Add` (`self.HealthBars`) (`/Game/Widget/W_HealthBarElementAttacker.HealthBar` _asw_health_bar_element_attacker))))
            (`Widget.SetRenderScale` _returnvalue_2 (5.0 5.0))
            (`PanelWidget.AddChild` (`self.HealthbarContainer`) _returnvalue_2)))))
    (:`then_3`
      ;[1 1 1] Set Starthealth
      (if (or (`KismetSystemLibrary.IsServer`) (`KismetSystemLibrary.IsDedicatedServer`))
        (`self.AlterHealth` (`self.StartHealth`))))))

(event `CheckAndTriggerRegeneration`
  (bind _returnvalue (`GameplayStatics.GetWorldDeltaSeconds`))
  ;[1 1 1] Update TimeSinceLastHit
  (if (`self.ShouldRegenerate`)
    (bind _output_get (set `self.TimeSinceLastHit` (+ (`self.TimeSinceLastHit`) _returnvalue)))
    (if (> _output_get (`self.RegenerationDelayInSec`))
      (`self.AlterHealth` (* (`self.RegenerationRatePerSec`) _returnvalue)))))

(event `self.ReceiveTick`
  (params (DeltaSeconds :type "Float (single-precision)"))
  ;[1 1 1] Tick
  ;[1 1 1] Check And Trigger Regeneration
  ;;[1 1 1] As this actor does not have an owner, a call from the client will be DROPPED and this spams a message into the output log
  (if (or (`KismetSystemLibrary.IsServer`) (`KismetSystemLibrary.IsDedicatedServer`))
    (`self.CheckAndTriggerRegeneration`)))

(fn `CheckNumberOfHealthSegments`
  (locals (CheckedHealth :type "Float (double-precision)"))
  ;[1 1 1] Are there enough items in the array to get a valid reference for the loop?
  (if (>= (`KismetArrayLibrary.Array_Length` (`self.HealthPerSegment`)) (`self.AmountOfHealthSegments`))
    ;[1 1 1] For each HealthSegment
    (for _index (range 1 (+ (`self.AmountOfHealthSegments`) 1))
      (bind _output_get (set `local.CheckedHealth` (+ (`|GetArrayItem` (`self.HealthPerSegment`) (- _index 1)) (`local.CheckedHealth`))))
      (if (>= (- (`self.CurrentHealth`) _output_get) 0.0)
        (set `self.MaxHealthToRestore` 0.0)
        (else
          (bind _output_get_2 (set `self.AmountOfHealthSegments` _index))))
      (for _index_2 (range 1 (+ _output_get_2 1))
        (set `self.MaxHealthToRestore` (+ (`self.MaxHealthToRestore`) (`|GetArrayItem` (`self.HealthPerSegment`) (- _index_2 1))))))))

(fn `OnRep_CurrentHealth`
  (bind _activehud (`self.ActiveHUD`))
  (bind _output (`|GetArrayItem` (`self.HealthPerSegment`)))
  (`|ExecutionSequence`
    (:`then_0`
      ;[1 1 1] Update HealthPoints
      (`/Engine/EditorBlueprintResources/StandardMacros.IsValid` _activehud
        (:`Is Valid`
          (bind _asw_hero_hud (cast `/Game/Widget/W_HeroHUD` _activehud))
          (`TextBlock.SetText` (`/Game/Widget/W_HeroHUD.Health` _asw_hero_hud) (`KismetTextLibrary.Conv_DoubleToText` (`self.CurrentHealth`) "HalfToEven")))))
    (:`then_1`
      ;[1 1 1] Update Healthbars
      (if (and (> (`KismetArrayLibrary.Array_Length` (`self.HealthBars`)) 0) (> (`KismetArrayLibrary.Array_Length` (`self.HealthPerSegment`)) 0))
        (for (_array_element _array_index) (`self.HealthBars`)
          (`/Engine/EditorBlueprintResources/StandardMacros.IsValid` _array_element
            (:`Is Valid`
              (`ProgressBar.SetPercent` _array_element (/ (- (`self.CurrentHealth`) (* _array_index _output)) _output)))))))))

(fn `PerformCameraShake`
  (bind _asbp_attacker_base (cast `/Game/Blueprints/BP_Attacker_Base` (`self.GetOwner`)))
  (bind _asplayer_controller (cast `PlayerController` (`Pawn.GetController` _asbp_attacker_base)))
  (`PlayerController.ClientStartCameraShake` :`self` _asplayer_controller :`Shake` "/Game/Blueprints/HitCameraShake.HitCameraShake_C" :`Scale` 20.0))