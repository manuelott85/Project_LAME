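; BP_XPComponent tracks XP, level and upgrade points for attacker and defender characters.
; AlterXP checks per-level thresholds, carries surplus over and grants an upgrade point per level-up; past the array's end, the threshold is the last entry times a multiplier.
; On BeginPlay, the locally controlled owner caches its Hero or Villain HUD after a short delay.
; UpdateHUD refreshes that HUD's XP display on start, level-up and CurrentXP's OnRep.
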(event `UpdateHUD`
  (bind _xpneededperlevel (`self.XPNeededPerLevel`))
  (bind _currentlevel (`self.CurrentLevel`))
  (bind _xpneededperlevel_2 (`self.XPNeededPerLevel`))
  (bind _returnvalue (> (`KismetArrayLibrary.Array_Length` _xpneededperlevel_2) _currentlevel))
  (bind _returnvalue_2 (/ (`KismetMathLibrary.Conv_IntToDouble` (`self.CurrentXP`)) (`KismetMathLibrary.Conv_IntToDouble` (`|GetArrayItem` _xpneededperlevel_2 _currentlevel))))
  (bind _returnvalue_3 (/ (`KismetMathLibrary.Conv_IntToDouble` (`self.CurrentXP`)) (* (`KismetMathLibrary.Conv_IntToDouble` (`|GetArrayItem` _xpneededperlevel (`KismetArrayLibrary.Array_LastIndex` _xpneededperlevel))) (`self.XPNeededMultiplierAtCap`))))
  ;[1 1 1] UpdateHUD
  (bind _asw_villain_hud (cast `/Game/Widget/W_VillainHUD` (`self.ActiveHUD`))
    (:`then`
      (if _returnvalue
        (bind _progressbar_xp (`/Game/Widget/W_VillainHUD.ProgressBar_XP` _asw_villain_hud))
        (`ProgressBar.SetPercent` _progressbar_xp _returnvalue_2)
        (else
          (`ProgressBar.SetPercent` _progressbar_xp _returnvalue_3)))
      (`TextBlock.SetText` (`/Game/Widget/W_VillainHUD.Text_AmountUpgradePoints` _asw_villain_hud) (`KismetTextLibrary.Conv_IntToText` (`self.CurrentUpgradePoints`))))
    (:`CastFailed`
      (bind _asw_hero_hud (cast `/Game/Widget/W_HeroHUD` (`self.ActiveHUD`)))
      (if _returnvalue
        (bind _experiencebar (`/Game/Widget/W_HeroHUD.ExperienceBar` _asw_hero_hud))
        (`ProgressBar.SetPercent` _experiencebar _returnvalue_2)
        (`TextBlock.SetText` (`/Game/Widget/W_HeroHUD.PlayerLevel` _asw_hero_hud) (`KismetTextLibrary.Conv_IntToText` (+ (`self.CurrentLevel`) 1)))
        (else
          (`ProgressBar.SetPercent` _experiencebar _returnvalue_3)))
      (if (> (`self.CurrentUpgradePoints`) 0)
        (`UserWidget.PlayAnimation` _asw_hero_hud (`/Game/Widget/W_HeroHUD.LevelUpAnim` _asw_hero_hud) 0.0 1 "Forward" 1.0)))))

(event `self.ReceiveBeginPlay`
  (bind _returnvalue (`self.GetOwner`))
  ;[1 1 1] BeginPlay
  ;[1 1 1] Only the owning client should execute
  (if (== (`Controller.K2_GetPawn` (`GameplayStatics.GetPlayerController` 0)) (`self.GetOwner`))
    ;[1 1 1] Wait for the HUD reference
    (`KismetSystemLibrary.Delay` 0.2)
    (bind _asbp_attacker_base (cast `/Game/Blueprints/BP_Attacker_Base` _returnvalue)
      (:`then`
        (set `self.ActiveHUD` (`/Game/Blueprints/BP_Attacker_Base.ActiveHUD` _asbp_attacker_base)))
      (:`CastFailed`
        (bind _asbp_defender_base (cast `/Game/Blueprints/BP_Defender_Base` _returnvalue))
        (set `self.ActiveHUD` (`/Game/Blueprints/BP_Defender_Base.VillainHUD` _asbp_defender_base))))
    (`self.UpdateHUD`)))

(event `Alter XP`
  (params (Amount :type Integer))
  (bind _xpneededperlevel (`self.XPNeededPerLevel`))
  (bind _xpneededperlevel_2 (`self.XPNeededPerLevel`))
  (bind _currentlevel (`self.CurrentLevel`))
  (bind _returnvalue (+ Amount (`self.CurrentXP`)))
  (bind _output (`|GetArrayItem` _xpneededperlevel _currentlevel))
  (bind _returnvalue_2 (`KismetMathLibrary.FTrunc` (* (`KismetMathLibrary.Conv_IntToDouble` (`|GetArrayItem` _xpneededperlevel_2 (`KismetArrayLibrary.Array_LastIndex` _xpneededperlevel_2))) (`self.XPNeededMultiplierAtCap`))))
  ;[1 1 1] AlterXP
  ;;[1 1 1] Check, if a value is set for current level in array
  (if (> (`KismetArrayLibrary.Array_Length` _xpneededperlevel) _currentlevel)
    (if (> _output _returnvalue)
      (set `self.CurrentXP` _returnvalue)
      (else
        (set `self.CurrentXP` (- _returnvalue _output))
        (set `self.CurrentLevel` (+ (`self.CurrentLevel`) 1))
        (`self.AlterUpgradePoints` 1)
        (`self.UpdateHUD`)))
    (elif (> _returnvalue_2 _returnvalue)
      (set `self.CurrentXP` _returnvalue)
      (else
        (set `self.CurrentXP` (- _returnvalue _returnvalue_2))
        (set `self.CurrentLevel` (+ (`self.CurrentLevel`) 1))
        (`self.AlterUpgradePoints` 1)
        (`self.UpdateHUD`)))))

(event `AlterUpgradePoints`
  (params (Amount :type Integer))
  ;[1 1 1] Alter UpgradePoints
  (set `self.CurrentUpgradePoints` (+ Amount (`self.CurrentUpgradePoints`))))

(fn `OnRep_CurrentXP`
  (`self.UpdateHUD`))