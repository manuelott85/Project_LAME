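; Component that tracks the defender's drone upgrade levels for durability, agility, kamikaze and offense.
; Server events increment the matching level by one, with no cost or cap check here.
; Each level's RepNotify refreshes every top-level W_DroneUpgrade menu and calls ServerProcessDroneUpgrade on all living BP_Drone_Base actors, so existing drones pick up the change.
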(event `Server_UpgradeDurability`
  ;[1 1 1] Increase Levels by one
  (set `self.CurrentDurabilityLvl` (+ (`self.CurrentDurabilityLvl`) 1)))

(event `UpdateDroneUpgradeMenu`
  (bind _foundwidgets (`WidgetBlueprintLibrary.GetAllWidgetsOfClass` "/Game/Widget/W_DroneUpgrade.W_DroneUpgrade_C"))
  (for _array_element _foundwidgets
    (`/Game/Widget/W_DroneUpgrade.UpdateMenu` _array_element)))

(event `Server_UpgradeAgility`
  ;[1 1 1] Increase Levels by one
  (set `self.CurrentAgilityLvl` (+ (`self.CurrentAgilityLvl`) 1)))

(event `Server_UpgradeKamikazi`
  ;[1 1 1] Increase Levels by one
  (set `self.CurrentKamikaziLvl` (+ (`self.CurrentKamikaziLvl`) 1)))

(event `Server_UpgradeOffense`
  ;[1 1 1] Increase Levels by one
  (set `self.CurrentOffenseLvl` (+ (`self.CurrentOffenseLvl`) 1)))

(fn `OnRep_CurrentAgilityLvl`
  ;[1 1 1] Upgrade Defender UI
  (`self.UpdateDroneUpgradeMenu`)
  ;[1 1 1] Upgrade every drone, currently alive
  (bind _outactors (`GameplayStatics.GetAllActorsOfClass` "/Game/Blueprints/AI/BP_Drone_Base.BP_Drone_Base_C"))
  (if (> (`KismetArrayLibrary.Array_Length` _outactors) 0)
    (for _array_element _outactors
      (`/Game/Blueprints/AI/BP_Drone_Base.Server_ProcessDroneUpgrade` _array_element))))

(fn `OnRep_CurrentDurabilityLvl`
  ;[1 1 1] Upgrade Defender UI
  (`self.UpdateDroneUpgradeMenu`)
  ;[1 1 1] Upgrade every drone, currently alive
  (bind _outactors (`GameplayStatics.GetAllActorsOfClass` "/Game/Blueprints/AI/BP_Drone_Base.BP_Drone_Base_C"))
  (if (> (`KismetArrayLibrary.Array_Length` _outactors) 0)
    (for _array_element _outactors
      (`/Game/Blueprints/AI/BP_Drone_Base.Server_ProcessDroneUpgrade` _array_element))))

(fn `OnRep_CurrentKamikaziLvl`
  ;[1 1 1] Upgrade Defender UI
  (`self.UpdateDroneUpgradeMenu`)
  ;[1 1 1] Upgrade every drone, currently alive
  (bind _outactors (`GameplayStatics.GetAllActorsOfClass` "/Game/Blueprints/AI/BP_Drone_Base.BP_Drone_Base_C"))
  (if (> (`KismetArrayLibrary.Array_Length` _outactors) 0)
    (for _array_element _outactors
      (`/Game/Blueprints/AI/BP_Drone_Base.Server_ProcessDroneUpgrade` _array_element))))

(fn `OnRep_CurrentOffenseLvl`
  ;[1 1 1] Upgrade Defender UI
  (`self.UpdateDroneUpgradeMenu`)
  ;[1 1 1] Upgrade every drone, currently alive
  (bind _outactors (`GameplayStatics.GetAllActorsOfClass` "/Game/Blueprints/AI/BP_Drone_Base.BP_Drone_Base_C"))
  (if (> (`KismetArrayLibrary.Array_Length` _outactors) 0)
    (for _array_element _outactors
      (`/Game/Blueprints/AI/BP_Drone_Base.Server_ProcessDroneUpgrade` _array_element))))