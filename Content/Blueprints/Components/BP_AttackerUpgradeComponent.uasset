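; Upgrade component for BP_Attacker_Base that applies tiered Agility, Defense, Magnet and Offense upgrades to the owning attacker.
; UnlockAbility takes the next entry from the category's array, advances that level without bounds checks, then runs ProcessUpgrade.
; ProcessUpgrade turns percentages into multipliers to scale max energy or damage; firing delay becomes the reduction multiplier divided by the current delay.
; CheckUpgradeAvailable is an empty stub.
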(event `self.ReceiveBeginPlay`
  (bind _asbp_attacker_base (cast `/Game/Blueprints/BP_Attacker_Base` (`self.GetOwner`)))
  (set `self.PlayerCharacter` _asbp_attacker_base))

(event `UnlockAbility`
  (params (UpgradeCategory :type "/Game/Enum/Enum_UpgradeCategory Enum" :default "NewEnumerator0"))
  (switch `/Game/Enum/Enum_UpgradeCategory` UpgradeCategory
    (:`NewEnumerator0`
      (set `self.SelectedUpgrade` (`|GetArrayItem` (`self.AgilityUpgrades`) (`self.AgilityLevel`)))
      (`/Engine/EditorBlueprintResources/StandardMacros.IncrementInt` (`self.AgilityLevel`)
        (:`  `
          _)))
    (:`NewEnumerator1`
      (set `self.SelectedUpgrade` (`|GetArrayItem` (`self.DefenseUpgrades`) (`self.DefenseLevel`)))
      (`/Engine/EditorBlueprintResources/StandardMacros.IncrementInt` (`self.DefenseLevel`)
        (:`  `
          _)))
    (:`NewEnumerator2`
      (set `self.SelectedUpgrade` (`|GetArrayItem` (`self.MagnetUpgrades`) (`self.MagnetLevel`)))
      (`/Engine/EditorBlueprintResources/StandardMacros.IncrementInt` (`self.MagnetLevel`)
        (:`  `
          _)))
    (:`NewEnumerator3`
      (set `self.SelectedUpgrade` (`|GetArrayItem` (`self.OffenseUpgrades`) (`self.OffenseLevel`)))
      (`/Engine/EditorBlueprintResources/StandardMacros.IncrementInt` (`self.OffenseLevel`)
        (:`  `
          _))))
  (`self.ProcessUpgrade`))

(event `CheckUpgradeAvailable`)

(fn `CalculateMultiplier`
  (params (Reduce :type Boolean))
  (returns (Multiplier :type "Float (double-precision)"))
  (bind (_selectedupgrade_ability _selectedupgrade_changeinpercent) (break `/Game/Blueprints/BP_AttackerUpgrade` (`self.SelectedUpgrade`)))
  (bind (_selectedupgrade_ability_2 _selectedupgrade_changeinpercent_2) (break `/Game/Blueprints/BP_AttackerUpgrade` (`self.SelectedUpgrade`)))
  (if Reduce
    (return (- 1.0 (/ _selectedupgrade_changeinpercent_2 100.0)))
    (else
      (return (+ (/ _selectedupgrade_changeinpercent 100.0) 1.0)))))

(fn `ProcessUpgrade`
  (bind _playercharacter (`self.PlayerCharacter`))
  (bind _playercharacter_2 (`self.PlayerCharacter`))
  (bind _bp_energycomponent (`/Game/Blueprints/BP_Attacker_Base.BP_EnergyComponent` (`self.PlayerCharacter`)))
  (switch `/Game/Enum/Enum_AttackerUpgrades` (`.Ability_3_D2FB30A745C97D599EB01CB3B2AA4AFF` (break `/Game/Blueprints/BP_AttackerUpgrade` (`self.SelectedUpgrade`)))
    (:`NewEnumerator0`
      (bind _multiplier (`self.CalculateMultiplier` false))
      (set `/Game/Blueprints/Components/BP_EnergyComponent.MaxEnergy` (* (`/Game/Blueprints/Components/BP_EnergyComponent.MaxEnergy` _bp_energycomponent) _multiplier) _bp_energycomponent)
      (`/Game/Blueprints/Components/BP_EnergyComponent.AlterEnergy` _bp_energycomponent 0.0))
    (:`NewEnumerator1`
      (bind _multiplier_2 (`self.CalculateMultiplier` false))
      (set `/Game/Blueprints/BP_Attacker_Base.Damage` (* _multiplier_2 (`/Game/Blueprints/BP_Attacker_Base.Damage` _playercharacter_2)) _playercharacter_2))
    (:`NewEnumerator2`
      (bind _multiplier_3 (`self.CalculateMultiplier` true))
      (set `/Game/Blueprints/BP_Attacker_Base.FiringDelay` (/ _multiplier_3 (`/Game/Blueprints/BP_Attacker_Base.FiringDelay` _playercharacter)) _playercharacter))))