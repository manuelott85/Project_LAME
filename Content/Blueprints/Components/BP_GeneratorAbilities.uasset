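; Defender component that runs generator abilities (Blast, Shield, Call Drones) on the defender's LastHitActor.
; A server event switches on ability, charges the energy component via ManageEnergy (which doesn't block on shortfall) and handles Delay-based cooldowns.
; Blast deals radial damage, spawns projectiles and multicasts effects; Shield temporarily enables the generator's shield.
; Call Drones only spends energy and toggles Blast's cooldown flag; a helper respawns the generator widget actor.
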(event `Multi_debug`
  ;[1 1 1] Show BlastDebugSpheres
  (bind _asbp_defender_base (cast `/Game/Blueprints/BP_Defender_Base` (`self.GetOwner`)))
  (bind _returnvalue_location (`KismetMathLibrary.BreakTransform` (`Actor.GetTransform` (`/Game/Blueprints/BP_Defender_Base.LastHitActor` _asbp_defender_base))))
  (`KismetSystemLibrary.DrawDebugSphere` _returnvalue_location (`self.BlastDamageInnerRadius`) 12 (struct :`R` 1.0 :`B` 0.04112 :`A` 1.0) 10.0 20.0)
  (`KismetSystemLibrary.DrawDebugSphere` _returnvalue_location (`self.BlastDamageOuterRadius`) 12 (struct :`G` 0.109804 :`B` 1.0 :`A` 1.0) 10.0 20.0))

(event `Multi_PlayBlastEffects`
  (params (GeneratorRef :type "Actor Object Reference"))
  (bind (_returnvalue_location _returnvalue_rotation) (`KismetMathLibrary.BreakTransform` (`Actor.GetTransform` GeneratorRef)))
  ;[1 1 1] Blast Effects
  (`GameplayStatics.SpawnEmitterAtLocation` (`self.BlastExplosionFX`) _returnvalue_location _returnvalue_rotation (`self.BlastExplosionScale`))
  (`GameplayStatics.PlaySoundAtLocation` (`self.BlastSound`) _returnvalue_location (struct) 1.0 1.0 0.0 null null null))

(event `Mulit_BlastProjectileEffects`
  ;[1 1 1] Play ShootSound
  (`GameplayStatics.PlaySoundAtLocation` (`self.BlastProjectileSound`) (`Actor.K2_GetActorLocation` (`self.GetOwner`)) (struct) 1.0 1.0 0.0 null null null))

(event `Server_ExecuteAbility`
  (params (Ability :type "/Game/Enum/Enum_GeneratorAbilities Enum" :default "NewEnumerator0"))
  (bind _shieldduration (`self.ShieldDuration`))
  (switch `/Game/Enum/Enum_GeneratorAbilities` Ability
    (:`NewEnumerator0`
      ;[1 1 1] Only proceed if not on cooldown
      (if (`self.bBlastIsOnCooldown`)
        (`KismetSystemLibrary.PrintString` "Blast is on Cooldown")
        (else
          (`self.ManageEnergy` (`self.BlastEnergyCost`))
          ;[1 1 1] Blast Ability
          (bind _asbp_defender_base (cast `/Game/Blueprints/BP_Defender_Base` (`self.GetOwner`)))
          (bind _lasthitactor (`/Game/Blueprints/BP_Defender_Base.LastHitActor` _asbp_defender_base))
          (`/Engine/EditorBlueprintResources/StandardMacros.IsValid` _lasthitactor
            (:`Is Valid`
              (`self.Multi_PlayBlastEffects` _lasthitactor)
              (bind _outactors (`GameplayStatics.GetAllActorsOfClass` "/Game/Blueprints/AI/BP_Drone_Base.BP_Drone_Base_C"))
              (for _array_element _outactors
                (bind _array (`|MakeArray` _lasthitactor))
                (`KismetArrayLibrary.Array_Add` _array _array_element))
              (bind _returnvalue_location (`KismetMathLibrary.BreakTransform` (`Actor.GetTransform` _lasthitactor)))
              (`GameplayStatics.ApplyRadialDamageWithFalloff` (`self.BlastBaseDamage`) (`self.BlastMinimumDamage`) _returnvalue_location (`self.BlastDamageInnerRadius`) (`self.BlastDamageOuterRadius`) (`self.BlastDamageFalloff`) null _array _asbp_defender_base (`Pawn.GetController` _asbp_defender_base))
              (if (`self.BlastDebugVisuals`)
                (`self.Multi_debug`))
              ;[1 1 1] Spawn the Projectile
              (for _ (range 1 (+ (`self.BlastAmountOfProjectiles`) 1))
                (`|SpawnActorFromClass` "/Game/Blueprints/Projectiles/BP_GeneratorBlastProjectile.BP_GeneratorBlastProjectile_C" (`KismetMathLibrary.MakeTransform` (`Actor.K2_GetActorLocation` _lasthitactor) (`KismetMathLibrary.RandomRotator` false)) "AlwaysSpawn" "OverrideRootScale" null (`self.BlastProjectileDamage`) null)
                (`self.Mulit_BlastProjectileEffects`)
                ;[1 1 1] Cooldown handling
                (set `self.bBlastIsOnCooldown` true)
                (`KismetSystemLibrary.Delay` (`self.BlastCooldown`))
                (set `self.bBlastIsOnCooldown` false)))))))
    (:`NewEnumerator1`
      ;[1 1 1] Only proceed if not on cooldown
      (if (`self.bShieldIsOnCooldown`)
        (`KismetSystemLibrary.PrintString` "Shield is on Cooldown")
        (else
          (`self.ManageEnergy` (`self.ShieldEnergyCost`))
          ;[1 1 1] Shield Ability
          (bind _asbp_defender_base_2 (cast `/Game/Blueprints/BP_Defender_Base` (`self.GetOwner`)))
          (bind _lasthitactor_2 (`/Game/Blueprints/BP_Defender_Base.LastHitActor` _asbp_defender_base_2))
          (`/Engine/EditorBlueprintResources/StandardMacros.IsValid` _lasthitactor_2
            (:`Is Valid`
              (bind _asbp_generator (cast `/Game/Blueprints/BP_Generator` _lasthitactor_2))
              (`self.Server_activateShield` _asbp_generator)
              ;[1 1 1] Cooldown handling
              (if (> _shieldduration (`self.ShieldCooldown`))
                (set `self.ShieldCooldown` _shieldduration))
              (set `self.bShieldIsOnCooldown` true)
              (`KismetSystemLibrary.Delay` (`self.ShieldCooldown`))
              (set `self.bShieldIsOnCooldown` false))))))
    (:`NewEnumerator2`
      ;[1 1 1] Only proceed if not on cooldown
      (if (`self.bCallDronesIsOnCooldown`)
        (`KismetSystemLibrary.PrintString` "CallDrones is on Cooldown")
        (else
          (`self.ManageEnergy` (`self.CallEnergyCost`))
          ;[1 1 1] Cooldown handling
          (set `self.bBlastIsOnCooldown` true)
          (`KismetSystemLibrary.Delay` (`self.CallCooldown`))
          (set `self.bBlastIsOnCooldown` false))))))

(event `Server_activateShield`
  (params (Generator :type "/Game/Blueprints/BP_Generator Object Reference"))
  (bind _shield (`/Game/Blueprints/BP_Generator.Shield` Generator))
  (bind _shield_2 (`/Game/Blueprints/BP_Generator.Shield` Generator))
  ;[1 1 1] Activate Shield and manage lifetime
  (set `/Game/Blueprints/BP_Generator.bShieldActive` true Generator)
  (`SceneComponent.SetVisibility` _shield_2 true false)
  (`PrimitiveComponent.SetCollisionEnabled` _shield_2 "QueryAndPhysics")
  (`KismetSystemLibrary.RetriggerableDelay` (`self.ShieldDuration`))
  (set `/Game/Blueprints/BP_Generator.bShieldActive` false Generator)
  (`SceneComponent.SetVisibility` _shield false false)
  (`PrimitiveComponent.SetCollisionEnabled` _shield "NoCollision"))

(fn `CreateGeneratorWidget`
  (params (GeneratorReference :type "/Game/Blueprints/BP_Generator Object Reference"))
  ;[1 1 1] destroy any old ones before
  (bind _outactors (`GameplayStatics.GetAllActorsOfClass` "/Game/Blueprints/BP_GeneratorWidget.BP_GeneratorWidget_C"))
  (for _array_element _outactors
    (`Actor.K2_DestroyActor` _array_element))
  ;[1 1 1] Create the widget
  (`|SpawnActorFromClass` "/Game/Blueprints/BP_GeneratorWidget.BP_GeneratorWidget_C" (`KismetMathLibrary.MakeTransform` (+ (`Actor.K2_GetActorLocation` GeneratorReference) (`KismetMathLibrary.MakeVector` 0.0 0.0 (`self.WidgetSpawnHeight`))) (struct :`Pitch` 90.0 :`Yaw` 174.289398 :`Roll` 84.28952) (`self.WidgetScale`)) "AlwaysSpawn" "OverrideRootScale" null null))

(fn `ManageEnergy`
  (params (EnergyCost :type Integer) (DebugMessage :type String :default "Not enough energy left to use that ability"))
  ;[1 1 1] Energy Cost
  (bind _asbp_defender_base (cast `/Game/Blueprints/BP_Defender_Base` (`self.GetOwner`)))
  (bind _bp_energycomponent (`/Game/Blueprints/BP_Defender_Base.BP_EnergyComponent` _asbp_defender_base))
  (if (> (`/Game/Blueprints/Components/BP_EnergyComponent.CurrentEnergy` _bp_energycomponent) (`KismetMathLibrary.Conv_IntToDouble` EnergyCost))
    (`/Game/Blueprints/Components/BP_EnergyComponent.AlterEnergy` _bp_energycomponent (`KismetMathLibrary.Conv_IntToDouble` (* EnergyCost -1)))
    (else
      (`KismetSystemLibrary.PrintString` DebugMessage))))