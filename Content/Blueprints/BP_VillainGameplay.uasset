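; Villain player's controllable view: an orthographic camera with cursor, touch and widget input for spawning drones.
; Mouse clicks and touches trace into ProcessHit: hitting a drone spawner opens the spawn widget; otherwise an open drone info widget spawns its drone to investigate the hit location.
; Tick applies move and zoom values, with zoom changing ortho width rather than camera height.
; BeginPlay also creates a hidden upgrade menu.
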(event `self.ReceiveBeginPlay`
  ;[1 1 1] Enable mouse cursor and set cursor to crosshairs
  (bind _asplayer_controller (cast `PlayerController` (`self.GetController`)))
  (set `PlayerController.bShowMouseCursor` true _asplayer_controller)
  (set `PlayerController.CurrentMouseCursor` "Crosshairs" _asplayer_controller)
  (`self.SetOrthoCamHeight`)
  ;[1 1 1] Add the Upgrade Menu, but hide it
  (bind _returnvalue (`|CreateWidget` "/Game/Widget/W_VillainUpgradeMenu.W_VillainUpgradeMenu_C" _asplayer_controller))
  (bind _output_get (set `self.VillainUpgradeMenu` _returnvalue))
  (`Widget.SetVisibility` _output_get "Hidden")
  (`UserWidget.AddToViewport` _output_get 0))

(event `InputTouch`
  (params (Location :type "Vector Structure") (FingerIndex :type "ETouchIndex Enum"))
  (bind _widgetinteraction (`self.WidgetInteraction`))
  ;[1 1 1] Widget Interaction Input
  (:`Pressed`
    (`WidgetInteractionComponent.PressPointerKey` _widgetinteraction "LeftMouseButton" :!label _label))
  (:`Released`
    (`WidgetInteractionComponent.ReleasePointerKey` _widgetinteraction "LeftMouseButton" :!label _label_2)))

(event `InputTouch`
  (params (Location :type "Vector Structure") (FingerIndex :type "ETouchIndex Enum"))
  ;[1 1 1] Raycast on Touch and send result to Process Hit
  (:`Pressed`
    (bind _hitresult (`self.PerformLinecastTouch` Location FingerIndex))
    (`self.Process Hit` _hitresult)))

(event `Key|LeftMouseButton`
  (params (Key :type "Key Structure"))
  ;[1 1 1] Widget Interaction Input
  (:`Pressed`
    (goto _label))
  (:`Released`
    (goto _label_2)))

(event `InputAction|Shoot`
  (params (Key :type "Key Structure"))
  ;[1 1 1] Raycast on Mouse Click and send result to Process Hit
  (:`Pressed`
    (bind _asplayer_controller (cast `PlayerController` (`self.GetController`)))
    (`self.Process Hit` (`PlayerController.GetHitResultUnderCursorByChannel` _asplayer_controller "TraceTypeQuery1" false))))

(event `self.ReceiveTick`
  (params (DeltaSeconds :type "Float (single-precision)"))
  (bind _camera (`self.Camera`))
  (`|ExecutionSequence`
    (:`then_0`
      ;[1 1 1] ZoomInput Processing
      (if (`self.shouldZoom`)
        (set `self.CameraHeight` (`KismetMathLibrary.FClamp` (+ (* (* (* (`self.currentZoomValue`) DeltaSeconds) -1.0) (`self.CamZoomSpeed`)) (`self.CameraHeight`)) (`self.MinCamHeight`) (`self.MaxCamHeight`)))
        (`self.SetOrthoCamHeight`)))
    (:`then_1`
      ;[1 1 1] Camera Move Input Processing
      (if (`self.shouldMove`)
        (`SceneComponent.K2_SetWorldLocation` _camera (+ (`SceneComponent.K2_GetComponentLocation` _camera) (* (* (`self.currentMoveVector`) DeltaSeconds) (`self.CamMoveSpeed`))) false false)))))

(event `Process Hit`
  (params (`Hit Result` :type "HitResult Structure"))
  ;[1 1 1] Process the HitResult
  (set `self.ValidProcessFound` false)
  (`|ExecutionSequence`
    (:`then_0`
      (`self.Case DroneSpawner` `Hit Result`))
    (:`then_1`
      (if (not (`self.ValidProcessFound`))
        (`self.Case W_DroneInfo is open` `Hit Result`)))))

(event `Case DroneSpawner`
  (params (`Hit Result` :type "HitResult Structure"))
  (bind _bp_spawningcomponent (`self.BP_SpawningComponent`))
  ;[1 1 1] Check if Drone Spawner was hit
  (bind _asbp_drone_spawner (cast `/Game/Blueprints/BP_DroneSpawner` (`.HitActor` (`GameplayStatics.BreakHitResult` `Hit Result`))))
  (set `/Game/Blueprints/BP_SpawningComponent.CurrentSpawnerPosition` (`SceneComponent.K2_GetComponentLocation` (`/Game/Blueprints/BP_DroneSpawner.Plane` _asbp_drone_spawner)) _bp_spawningcomponent)
  (`/Game/Blueprints/BP_SpawningComponent.CreateSpawningWidget` _bp_spawningcomponent)
  (set `self.ValidProcessFound` true))

(event `Case W_DroneInfo is open`
  (params (HitResult :type "HitResult Structure"))
  (bind _foundwidgets (`WidgetBlueprintLibrary.GetAllWidgetsOfClass` "/Game/Widget/W_SpawnDroneInformation.W_SpawnDroneInformation_C"))
  (if (> (`KismetArrayLibrary.Array_Length` _foundwidgets) 0)
    (bind _output (`|GetArrayItem` _foundwidgets))
    (`/Engine/EditorBlueprintResources/StandardMacros.IsValid` _output
      (:`Is Valid`
        (`/Game/Blueprints/BP_SpawningComponent.SpawnDrone` (`self.BP_SpawningComponent`) (`/Game/Widget/W_SpawnDroneInformation.DroneToSpawn` _output) (`.Location` (`GameplayStatics.BreakHitResult` HitResult)))
        (`Widget.RemoveFromParent` _output)))))

(fn `PerformLinecastTouch`
  (params (InVec :type "Vector Structure") (InputPin :type "ETouchIndex Enum" :default "Touch1"))
  (returns (HitResult :type "HitResult Structure"))
  (bind _asplayer_controller (cast `PlayerController` (`self.GetController`)))
  (`PlayerController.SetMouseLocation` _asplayer_controller (`KismetMathLibrary.FTrunc` (.x InVec)) (`KismetMathLibrary.FTrunc` (.y InVec)))
  (return (`PlayerController.GetHitResultUnderFingerByChannel` _asplayer_controller InputPin "TraceTypeQuery1" true)))

(fn `SetOrthoCamHeight`
  ;[1 1 1] Camera Heigth Orthographic
  (`CameraComponent.SetOrthoWidth` (`self.Camera`) (`self.CameraHeight`)))

(fn `UserConstructionScript`)