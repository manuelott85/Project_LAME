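; Health component that tracks an actor's health, restarting the level when the player character dies and destroying other actors at zero health.
; Damage events feed negated amounts into AlterHealth, which clamps the total and also applies starting health at BeginPlay.
; An OnRep function for CurrentHealth updates the local player's HUD text.
; That HUD reference comes from the character's energy component, leaving the component's own widget creation unused.
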(event `self.ReceiveBeginPlay`
  (`|ExecutionSequence`
    (:`then_0`
      ;[1 1 1] Get the HeroHUD
      (bind _asbp_fps_character (cast `/Game/Blueprints/BP_FPS_Character` (`self.GetOwner`)))
      (set `self.HeroeHUD` (`/Game/Blueprints/BP_EnergyComponent.ActiveHUD` (`/Game/Blueprints/BP_FPS_Character.BP_EnergyComponent` _asbp_fps_character))))
    (:`then_1`
      ;[1 1 1] Set Starthealth
      (`self.AlterHealth` (`self.StartHealth`)))))

(event `AlterHealth`
  (params (AmountToAlter :type "Float (double-precision)"))
  (bind _returnvalue (`GameplayStatics.GetGameMode`))
  ;[1 1 1] Alter Health
  (set `self.CurrentHealth` (`KismetMathLibrary.FClamp` (+ AmountToAlter (`self.CurrentHealth`)) 0.0 (`self.MaxHealth`)))
  ;[1 1 1] Destroy the actor if not the player
  (if (<= (`self.CurrentHealth`) 0.0)
    (cast `/Game/Blueprints/BP_FPS_Character` (`self.GetOwner`)
      (:`then`
        ;[1 1 1] Restart current level
        (`/Engine/EditorBlueprintResources/StandardMacros.IsValid` _returnvalue
          (:`Is Valid`
            (bind _asbp_game_mode (cast `/Game/Blueprints/BP_GameMode` _returnvalue))
            (`/Game/Blueprints/BP_GameMode.RestartLevel` _asbp_game_mode))))
      (:`CastFailed`
        (`Actor.K2_DestroyActor` (`self.GetOwner`))
        (`KismetSystemLibrary.PrintString` "destroyed")))))

(event `Remote: Event any Damage`
  (params (Damage :type "Float (double-precision)") (DamageType :type "DamageType Object Reference") (InstigatedBy :type "Controller Object Reference") (DamageCauser :type "Actor Object Reference"))
  ;[1 1 1] Handle Damage
  (`|ExecutionSequence`
    (:`then_0`
      (`self.AlterHealth` (* Damage -1.0)))))

(fn `OnRep_CurrentHealth`
  (if (== (`Pawn.GetController` (`Actor.Instigator` (`self.GetOwner`))) (`GameplayStatics.GetPlayerController` 0))
    (bind _asw_hero_hud (cast `/Game/Widget/W_HeroHUD` (`self.HeroeHUD`)))
    (`TextBlock.SetText` (`/Game/Widget/W_HeroHUD.Health` _asw_hero_hud) (`KismetTextLibrary.Conv_DoubleToText` (`self.CurrentHealth`) "HalfToEven"))))