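; Base pawn for the defender (villain) player, who commands drones through an orthographic camera with mouse or touch.
; BeginPlay builds the HUD and hidden upgrade menus, while Tick applies camera zoom (ortho width) and movement.
; Click and touch raycasts feed ProcessHit, which tries cases in order until ValidProcessFound is set.
; Cases open mainframe spawn or generator menus, send drones to clicked locations, or collect energy pickups via a server event.
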(event `self.ReceiveBeginPlay`
  (`|ExecutionSequence`
    (:`then_0`
      ;[1 1 1] Enable mouse cursor and set cursor to crosshairs
      (bind _asplayer_controller (cast `PlayerController` (`self.GetController`)))
      (set `PlayerController.bShowMouseCursor` true _asplayer_controller)
      (set `PlayerController.CurrentMouseCursor` "Crosshairs" _asplayer_controller))
    (:`then_1`
      (`self.SetOrthoCamHeight`))
    (:`then_2`
      ;[1 1 1] Create the HUD
      (bind _asbp_player_controller (cast `/Game/Blueprints/BP_PlayerController` (`self.GetController`)))
      (bind _returnvalue (`|CreateWidget` "/Game/Widget/W_VillainHUD.W_VillainHUD_C" _asbp_player_controller))
      (bind _output_get (set `self.VillainHUD` _returnvalue))
      (`UserWidget.AddToViewport` _output_get 0)
      (set `/Game/Blueprints/Components/BP_SpawningComponent.ActiveHUD` (`self.VillainHUD`) (`self.BP_SpawningComponent`))
      (set `/Game/Blueprints/Components/BP_XPComponent.ActiveHUD` (`self.VillainHUD`) (`self.BP_XPComponent`)))
    (:`then_3`
      ;[1 1 1] Add the Upgrade Menus, but hide them
      (bind _asbp_player_controller_2 (cast `/Game/Blueprints/BP_PlayerController` (`self.GetController`)))
      (bind _returnvalue_2 (`|CreateWidget` "/Game/Widget/W_GeneratorUpgrade.W_GeneratorUpgrade_C" _asbp_player_controller_2))
      (bind _output_get_2 (set `self.VillainUpgradeMenu` _returnvalue_2))
      (`Widget.SetVisibility` _output_get_2 "Hidden")
      (`UserWidget.AddToViewport` _output_get_2 0)
      (bind _returnvalue_3 (`|CreateWidget` "/Game/Widget/W_DroneUpgrade.W_DroneUpgrade_C" _asbp_player_controller_2))
      (bind _output_get_3 (set `self.VillainDroneUpgradeMenu` _returnvalue_3))
      (`Widget.SetVisibility` _output_get_3 "Hidden")
      (`UserWidget.AddToViewport` _output_get_3 0))))

(event `InputTouch`
  (params (Location :type "Vector Structure") (FingerIndex :type "ETouchIndex Enum"))
  (bind _widgetinteraction (`self.WidgetInteraction`))
  ;[1 1 1] Widget Interaction Input
  (:`Pressed`
    (`WidgetInteractionComponent.PressPointerKey` _widgetinteraction "LeftMouseButton" :!label _label))
  (:`Released`
    (`WidgetInteractionComponent.ReleasePointerKey` _widgetinteraction "LeftMouseButton" :!label _label_2)))

(event `InputTouch`
  (params (Location :type "Vector Structure") (FingerIndex :type "ETouchIndex Enum"))
  ;[1 1 1] Raycast on Touch and send result to Process Hit
  (:`Pressed`
    (bind _hitresult (`self.PerformLinecastTouch` Location FingerIndex))
    (`self.Process Hit` _hitresult)))

(event `Key|LeftMouseButton`
  (params (Key :type "Key Structure"))
  ;[1 1 1] Widget Interaction Input
  (:`Pressed`
    (goto _label))
  (:`Released`
    (goto _label_2)))

(event `InputAction|Shoot`
  (params (Key :type "Key Structure"))
  ;[1 1 1] Raycast on Mouse Click and send result to Process Hit
  (:`Pressed`
    (bind _asplayer_controller (cast `PlayerController` (`self.GetController`)))
    (`self.Process Hit` (`PlayerController.GetHitResultUnderCursorByChannel` _asplayer_controller "TraceTypeQuery1" false))))

(event `self.ReceiveTick`
  (params (DeltaSeconds :type "Float (single-precision)"))
  (bind _camera (`self.Camera`))
  (`|ExecutionSequence`
    (:`then_0`
      ;[1 1 1] ZoomInput Processing
      (if (`self.shouldZoom`)
        (set `self.CameraHeight` (`KismetMathLibrary.FClamp` (+ (* (* (* (`self.currentZoomValue`) DeltaSeconds) -1.0) (`self.CamZoomSpeed`)) (`self.CameraHeight`)) (`self.MinCamHeight`) (`self.MaxCamHeight`)))
        (`self.SetOrthoCamHeight`)))
    (:`then_1`
      ;[1 1 1] Camera Move Input Processing
      (if (`self.shouldMove`)
        (`SceneComponent.K2_SetWorldLocation` _camera (+ (`SceneComponent.K2_GetComponentLocation` _camera) (* (* (`self.currentMoveVector`) DeltaSeconds) (`self.CamMoveSpeed`))) false false)))))

(event `Server_UpdateLastHitActor`
  (params (ActorReference :type "Actor Object Reference"))
  ;[1 1 1] Update LastHitActor
  (`/Engine/EditorBlueprintResources/StandardMacros.IsValid` ActorReference
    (:`Is Valid`
      (set `self.LastHitActor` ActorReference))))

(event `Case Mainframe`
  (params (`Hit Result` :type "HitResult Structure"))
  ;[1 1 1] Check if mainframe was hit and open the spawn menu
  (bind _asbp_mainframe (cast `/Game/Blueprints/Towers/BP_Mainframe` (`.HitActor` (`GameplayStatics.BreakHitResult` `Hit Result`))))
  (if (> (`/Game/Blueprints/Components/BP_HealthComponent.CurrentHealth` (`/Game/Blueprints/Towers/BP_Mainframe.BP_HealthComponent` _asbp_mainframe)) 0.0)
    (set `/Game/Blueprints/Components/BP_SpawningComponent.CurrentSpawnerPosition` (`SceneComponent.K2_GetComponentLocation` (`/Game/Blueprints/Towers/BP_Mainframe.SpawnPoint` _asbp_mainframe)) (`self.BP_SpawningComponent`))
    (bind _returnvalue (`|CreateWidget` "/Game/Widget/W_SpawnDroneInformation.W_SpawnDroneInformation_C" null (`self.DroneToSpawn`)))
    (`UserWidget.AddToViewport` _returnvalue 0)
    (set `self.ValidProcessFound` true)
    (else
      (`KismetSystemLibrary.PrintString` "Error: Spawner does not have healthpoints left" true true (struct :`R` 1.0 :`A` 1.0) 5.0))))

(event `Process Hit`
  (params (`Hit Result` :type "HitResult Structure"))
  ;[1 1 1] Process the HitResult
  (set `self.ValidProcessFound` false)
  (`|ExecutionSequence`
    (:`then_0`
      (`self.Case Mainframe` `Hit Result`))
    (:`then_1`
      (if (not (`self.ValidProcessFound`))
        (`self.Case W_DroneInfo is open` `Hit Result`)))
    (:`then_2`
      (if (not (`self.ValidProcessFound`))
        (`self.Case DefenderPickUp` `Hit Result`)))
    (:`then_3`
      (if (not (`self.ValidProcessFound`))
        (`self.Case DefenderPickUp` `Hit Result`)))
    (:`then_4`
      (if (not (`self.ValidProcessFound`))
        (`self.Case_Generator` `Hit Result`)))))

(event `Case W_DroneInfo is open`
  (params (HitResult :type "HitResult Structure"))
  (bind _bp_spawningcomponent (`self.BP_SpawningComponent`))
  ;[1 1 1] Check if the defender already had a drone selected; spawn this drone
  (bind _foundwidgets (`WidgetBlueprintLibrary.GetAllWidgetsOfClass` "/Game/Widget/W_SpawnDroneInformation.W_SpawnDroneInformation_C"))
  (if (> (`KismetArrayLibrary.Array_Length` _foundwidgets) 0)
    (bind _output (`|GetArrayItem` _foundwidgets))
    (`/Engine/EditorBlueprintResources/StandardMacros.IsValid` _output
      (:`Is Valid`
        (if (< (`/Game/Blueprints/Components/BP_SpawningComponent.CurrentNumberOfDrones` _bp_spawningcomponent) (`/Game/Blueprints/Components/BP_SpawningComponent.MaxNumberOfDrones` _bp_spawningcomponent))
          (`/Game/Blueprints/Components/BP_SpawningComponent.SpawnDrone` (`self.BP_SpawningComponent`) (`self.DroneToSpawn`) (`.Location` (`GameplayStatics.BreakHitResult` HitResult)))
          (`Widget.RemoveFromParent` _output)
          (set `self.ValidProcessFound` true)
          (else
            (`KismetSystemLibrary.PrintString` "ERROR: Maximum number of drones reached" true false (struct :`R` 1.0 :`B` 0.014791 :`A` 1.0) 10.0)))))))

(event `Case DefenderPickUp`
  (params (HitResult :type "HitResult Structure"))
  ;[1 1 1] Check if a pickup for the defender was selected
  (bind _asbp_defender_pickup_base (cast `/Game/Blueprints/PickUps/BP_DefenderPickup_Base` (`.HitActor` (`GameplayStatics.BreakHitResult` HitResult))))
  (`/Game/Blueprints/PickUps/BP_DefenderPickup_Base.PlayClientsideEffects` _asbp_defender_pickup_base)
  (set `self.ValidProcessFound` true)
  (`self.Server_PickupEnergy` (`/Game/Blueprints/PickUps/BP_DefenderPickup_Base.EnergyContained` _asbp_defender_pickup_base) _asbp_defender_pickup_base))

(event `Server_PickupEnergy`
  (params (Energy :type "Float (double-precision)") (PickUpRef :type "/Game/Blueprints/PickUps/BP_DefenderPickup_Base Object Reference"))
  (bind _bp_energycomponent (`self.BP_EnergyComponent`))
  ;[1 1 1] Add/substract Energy if needed
  (if (< (`/Game/Blueprints/Components/BP_EnergyComponent.CurrentEnergy` _bp_energycomponent) (`/Game/Blueprints/Components/BP_EnergyComponent.MaxEnergy` _bp_energycomponent))
    (`/Game/Blueprints/Components/BP_EnergyComponent.AlterEnergy` (`self.BP_EnergyComponent`) Energy)
    (`self.K2_DestroyActor` PickUpRef)
    (else
      (`KismetSystemLibrary.PrintString` "BP_VillainGP: Your energy is at maximum" true true (struct :`R` 1.0 :`G` 0.878469 :`A` 1.0) 4.0))))

(event `Case_Generator`
  (params (HitResult :type "HitResult Structure"))
  ;[1 1 1] Check if generator was hit and open the menu
  (bind _asbp_generator (cast `/Game/Blueprints/BP_Generator` (`.HitActor` (`GameplayStatics.BreakHitResult` HitResult))))
  (`self.Server_UpdateLastHitActor` _asbp_generator)
  (if (> (`/Game/Blueprints/Components/BP_HealthComponent.CurrentHealth` (`/Game/Blueprints/BP_Generator.BP_HealthComponent` _asbp_generator)) 0.0)
    (`/Game/Blueprints/Components/BP_GeneratorAbilities.CreateGeneratorWidget` (`self.BP_GeneratorAbilities`) _asbp_generator)
    (set `self.ValidProcessFound` true)
    (else
      (`KismetSystemLibrary.PrintString` "Error: Spawner does not have healthpoints left" true true (struct :`R` 1.0 :`A` 1.0) 5.0))))

(fn `PerformLinecastTouch`
  (params (InVec :type "Vector Structure") (InputPin :type "ETouchIndex Enum" :default "Touch1"))
  (returns (HitResult :type "HitResult Structure"))
  (bind _asplayer_controller (cast `PlayerController` (`self.GetController`)))
  (`PlayerController.SetMouseLocation` _asplayer_controller (`KismetMathLibrary.FTrunc` (.x InVec)) (`KismetMathLibrary.FTrunc` (.y InVec)))
  (return (`PlayerController.GetHitResultUnderFingerByChannel` _asplayer_controller InputPin "TraceTypeQuery1" true)))

(fn `SetOrthoCamHeight`
  ;[1 1 1] Camera Heigth Orthographic
  (`CameraComponent.SetOrthoWidth` (`self.Camera`) (`self.CameraHeight`)))

(fn `UserConstructionScript`)