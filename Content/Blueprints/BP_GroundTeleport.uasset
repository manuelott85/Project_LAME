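; BP_GroundTeleport is a trigger volume that sends characters who enter it back to a nearby spawn point and damages them.
; On BeginPlay it caches all actors of a configurable spawn point class.
; On box overlap, the server finds the spawn point closest to the overlapping BP_FPS_CharacterBase using squared distances.
; It then moves the character there and applies a configurable amount of damage.
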(event `self.ReceiveBeginPlay`
  (bind _outactors (`GameplayStatics.GetAllActorsOfClass` (`self.ClassOfTheSpawnpoints`)))
  (set `self.PlayerStarts` _outactors))

(event `self.Box.OnComponentBeginOverlap`
  (params (OverlappedComponent :type "PrimitiveComponent Object Reference") (OtherActor :type "Actor Object Reference") (OtherComp :type "PrimitiveComponent Object Reference") (OtherBodyIndex :type Integer) (bFromSweep :type Boolean) (SweepResult :type "HitResult Structure (by ref)"))
  (bind _playerstarts (`self.PlayerStarts`))
  (`/Engine/EditorBlueprintResources/ActorMacros.Switch Has Authority`
    (:`Authority`
      (bind _asbp_fps_character_base (cast `/Game/Blueprints/BP_FPS_CharacterBase` OtherActor))
      ;[1 1 1] Get the closest spawn point
      (if (> (`KismetArrayLibrary.Array_Length` _playerstarts) 0)
        (set `self.closestPlayerstart` (`|GetArrayItem` _playerstarts))
        (for _array_element _playerstarts
          (bind _returnvalue (`self.K2_GetActorLocation` _asbp_fps_character_base))
          (if (< (`KismetMathLibrary.VSizeSquared` (- (`self.K2_GetActorLocation` _array_element) _returnvalue)) (`KismetMathLibrary.VSizeSquared` (- _returnvalue (`self.K2_GetActorLocation` (`self.closestPlayerstart`)))))
            (bind _output_get (set `self.closestPlayerstart` _array_element))))
        ;[1 1 1] teleport and do damage
        (`self.K2_SetActorLocation` _asbp_fps_character_base (`self.K2_GetActorLocation` _output_get) false false)
        (`GameplayStatics.ApplyDamage` _asbp_fps_character_base (`self.AmountOfDamage`))))))

(fn `UserConstructionScript`)