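; Game mode for an asymmetric multiplayer match that assigns roles and spawns pawns on the server.
; On login it ensures one BP_FPS_Character, then one villain BP_ObstaclePlacement, then makes everyone else FPS, possessing and activating input.
; FPS players cycle through PlayerStarts, while the villain consumes and destroys a BP_VillainSpawn.
; BeginPlay spawns a set number of Team2 AI at the LastUsedAISpawn point, an index never advanced here.
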(event `self.K2_PostLogin`
  (params (NewPlayer :type "PlayerController Object Reference"))
  (`/Engine/EditorBlueprintResources/ActorMacros.Switch Has Authority`
    (:`Authority`
      (`|ExecutionSequence`
        (:`then_0`
          ;[1 1 1] Add recently joined player to the controller list
          (`KismetArrayLibrary.Array_Add` (`self.ConnectedPlayerController`) NewPlayer)
          (set `self.PlayerGotActor` false))
        (:`then_1`
          ;[1 1 1] Get all playerspawns, if the array has not been created yet
          (if (== (`KismetArrayLibrary.Array_Length` (`self.PlayerSpawns`)) 0)
            (bind _outactors (`GameplayStatics.GetAllActorsOfClass` "/Script/Engine.PlayerStart"))
            (set `self.PlayerSpawns` _outactors)))
        (:`then_2`
          (`|ExecutionSequence`
            (:`then_0`
              ;[1 1 1] If there is not at least one regular player, spawn one
              (bind _outactors_2 (`GameplayStatics.GetAllActorsOfClass` "/Game/Blueprints/BP_FPS_Character.BP_FPS_Character_C"))
              (if (== (`KismetArrayLibrary.Array_Length` _outactors_2) 0)
                (`self.SpawnFPSPlayer` NewPlayer)
                (set `self.PlayerGotActor` true)))
            (:`then_1`
              ;[1 1 1] If there is not at least one villain player, spawn one
              (if (not (`self.PlayerGotActor`))
                (bind _outactors_3 (`GameplayStatics.GetAllActorsOfClass` "/Game/Blueprints/BP_ObstaclePlacement.BP_ObstaclePlacement_C"))
                (if (== (`KismetArrayLibrary.Array_Length` _outactors_3) 0)
                  (`self.SpawnVillain` NewPlayer)
                  (set `self.PlayerGotActor` true))))
            (:`then_2`
              ;[1 1 1] Spawn a FPS Player anyway
              (if (not (`self.PlayerGotActor`))
                (`self.SpawnFPSPlayer` NewPlayer)))))))))

(event `self.ReceiveBeginPlay`
  (`/Engine/EditorBlueprintResources/ActorMacros.Switch Has Authority`
    (:`Authority`
      (`|ExecutionSequence`
        (:`then_0`
          ;[1 1 1] Get all AIspawns, if the array has not been created yet
          (if (== (`KismetArrayLibrary.Array_Length` (`self.AISpawns`)) 0)
            (bind _outactors (`GameplayStatics.GetAllActorsOfClass` "/Game/Blueprints/AI/BP_AISpawn.BP_AISpawn_C"))
            (set `self.AISpawns` _outactors)))
        (:`then_1`
          ;[1 1 1] Spawn the AI
          (for _ (range (`self.NumberOfAIToSpawnAtLevelStart`))
            (`|SpawnActorFromClass` "/Game/Blueprints/AI/BP_AICharacter_Team2.BP_AICharacter_Team2_C" (`SceneComponent.K2_GetComponentToWorld` (`Actor.RootComponent` (`|GetArrayItem` (`self.AISpawns`) (`self.LastUsedAISpawn`)))) "AdjustIfPossibleButAlwaysSpawn" "OverrideRootScale" null null)))))))

(fn `IncrementPlayerSpawnIndex`
  (bind _returnvalue (+ (`self.LastUsedPlayerSpawn`) 1))
  (if (< _returnvalue (`KismetArrayLibrary.Array_Length` (`self.PlayerSpawns`)))
    (set `self.LastUsedPlayerSpawn` _returnvalue)
    (else
      (set `self.LastUsedPlayerSpawn` 0))))

(fn `SpawnFPSPlayer`
  (params (`New Player` :type "PlayerController Object Reference"))
  (bind _returnvalue (`|SpawnActorFromClass` "/Game/Blueprints/BP_FPS_Character.BP_FPS_Character_C" (`SceneComponent.K2_GetComponentToWorld` (`Actor.RootComponent` (`|GetArrayItem` (`self.PlayerSpawns`) (`self.LastUsedPlayerSpawn`)))) "AdjustIfPossibleButAlwaysSpawn" "OverrideRootScale" null null))
  (`self.IncrementPlayerSpawnIndex`)
  (`Controller.Possess` `New Player` _returnvalue)
  (bind _asbp_player_controller (cast `/Game/Blueprints/BP_PlayerController` `New Player`))
  (`/Game/Blueprints/BP_PlayerController.ActivateInput` _asbp_player_controller))

(fn `SpawnVillain`
  (params (`New Player` :type "PlayerController Object Reference"))
  (locals (UsedSpawnPosition :type "/Game/Blueprints/BP_VillainSpawn Object Reference"))
  (bind _outactors (`GameplayStatics.GetAllActorsOfClass` "/Game/Blueprints/BP_VillainSpawn.BP_VillainSpawn_C"))
  (bind _output (`|GetArrayItem` _outactors))
  (set `local.UsedSpawnPosition` _output)
  (bind _returnvalue (`|SpawnActorFromClass` "/Game/Blueprints/BP_ObstaclePlacement.BP_ObstaclePlacement_C" (`SceneComponent.K2_GetComponentToWorld` (`Actor.RootComponent` _output)) "AdjustIfPossibleButAlwaysSpawn" "OverrideRootScale" null null))
  (`Controller.Possess` `New Player` _returnvalue)
  (bind _asbp_player_controller (cast `/Game/Blueprints/BP_PlayerController` `New Player`))
  (`/Game/Blueprints/BP_PlayerController.ActivateInput` _asbp_player_controller)
  (`self.K2_DestroyActor` (`local.UsedSpawnPosition`)))

(fn `UserConstructionScript`)