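; BP_BillboardAddition is a Paper2D sprite actor that hovers above another actor as a billboard marker.
; BeginPlay applies the configured sprite asset and world scale to its sprite component.
; Each Tick, while the target actor is valid, it moves to that actor's location plus a vertical height offset, without formal attachment.
; The graph does no camera-facing rotation.
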(event `self.ReceiveBeginPlay`
  (bind _papersprite (`self.PaperSprite`))
  (`PaperSpriteComponent.SetSprite` _papersprite (`self.SpriteAsset`))
  (`SceneComponent.SetWorldScale3D` _papersprite (`self.Scale`)))

(event `self.ReceiveTick`
  (params (DeltaSeconds :type "Float (single-precision)"))
  (bind _actortoattach (`self.ActorToAttach`))
  (`/Engine/EditorBlueprintResources/StandardMacros.IsValid` _actortoattach
    (:`Is Valid`
      (`self.K2_SetActorLocation` (+ (`self.K2_GetActorLocation` _actortoattach) (`KismetMathLibrary.MakeVector` 0.0 0.0 (`self.BillboardHeight`)))))))

(fn `UserConstructionScript`)