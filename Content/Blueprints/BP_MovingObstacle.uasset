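; BP_MovingObstacle is an obstacle whose static mesh oscillates back and forth along its local Y axis.
; Each tick it offsets the mesh by Direction, which acts as a signed speed, scaled by delta time, teleporting without sweep and zeroing X and Z.
; Direction flips sign whenever the mesh's relative distance from the origin exceeds MaxDelta.
; BeginPlay stores the world start position, which the graph never reads.
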(event `self.ReceiveBeginPlay`
  (set `self.StartPos` (`SceneComponent.K2_GetComponentLocation` (`self.StaticMesh`))))

(event `self.ReceiveTick`
  (params (DeltaSeconds :type "Float (single-precision)"))
  (bind _relativelocation (`SceneComponent.RelativeLocation` (`self.StaticMesh`)))
  (if (not (<= (`KismetMathLibrary.VSize` _relativelocation) (`self.MaxDelta`)))
    (set `self.Direction` (* (`self.Direction`) -1)))
  (`SceneComponent.K2_SetRelativeLocation` (`self.StaticMesh`) (`KismetMathLibrary.MakeVector` 0.0 (+ (.y _relativelocation) (* (`self.Direction`) DeltaSeconds))) false true))

(fn `UserConstructionScript`)