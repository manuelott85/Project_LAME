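; BP_Mainframe is a tower actor with a health bar and a shield that blocks damage while any BP_Generator has health left.
; The server caches generators at BeginPlay, polls their health every tick and replicates shield changes through an OnRep that toggles the mesh's visibility.
; Damage reaches BPHealthComponent only when unshielded and not from AI projectiles.
; The health bar faces the local camera, and the billboard sprite shows only for Defender players.
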(event `self.ReceiveTick`
  (params (DeltaSeconds :type "Float (single-precision)"))
  (bind _returnvalue (`GameplayStatics.GetPlayerCameraManager` 0))
  (bind _healthrotator (`self.HealthRotator`))
  ;[1 1 1] Tick
  ;[1 1 1] Rotate Healthbar
  (`/Engine/EditorBlueprintResources/StandardMacros.IsValid` _returnvalue
    (:`Is Valid`
      (`SceneComponent.K2_SetWorldRotation` _healthrotator (`KismetMathLibrary.FindLookAtRotation` (`SceneComponent.K2_GetComponentLocation` _healthrotator) (`PlayerCameraManager.GetCameraLocation` _returnvalue)) false false)
      ;[1 1 1] Update Healthbar
      (cast `/Game/Widget/W_Healthbar` (`WidgetComponent.GetUserWidgetObject` (`self.HealthWidget`)))
      ;[1 1 1] As this actor does not have an owner, a call from the client will be DROPPED and this spams a message into the output log
      (if (or (`KismetSystemLibrary.IsServer`) (`KismetSystemLibrary.IsDedicatedServer`))
        ;[1 1 1] Update MainframeShield
        (`self.Server_CheckShield`)))))

(event `self.ReceiveAnyDamage`
  (params (Damage :type "Float (single-precision)") (DamageType :type "DamageType Object Reference") (InstigatedBy :type "Controller Object Reference") (DamageCauser :type "Actor Object Reference"))
  ;[1 1 1] Handle Damage
  ;;[1 1 1] Exclude friendly fire
  (cast `/Game/Blueprints/Projectiles/BP_AIProjectile_Base` DamageCauser
    (:`CastFailed`
      (if (not (`self.bShieldActive`))
        (`/Game/Blueprints/Components/BP_HealthComponent.Remote: Event any Damage` (`self.BP_HealthComponent`) Damage DamageType InstigatedBy DamageCauser)))))

(event `self.ReceiveBeginPlay`
  (bind _returnvalue (`GameplayStatics.GetPlayerController` 0))
  (bind _papersprite (`self.PaperSprite`))
  ;[1 1 1] BeginPlay
  (`|ExecutionSequence`
    (:`then_0`
      ;[1 1 1] Get all DroneSpawner as a reference to determine later if the shield should be active
      (if (or (`KismetSystemLibrary.IsServer`) (`KismetSystemLibrary.IsDedicatedServer`))
        (bind _outactors (`GameplayStatics.GetAllActorsOfClass` "/Game/Blueprints/BP_Generator.BP_Generator_C"))
        (for _array_element _outactors
          (`KismetArrayLibrary.Array_Add` (`self.DroneSpawnerReference`) _array_element))))
    (:`then_1`
      ;[1 1 1] Set Visability of the Billboard
      (`/Engine/EditorBlueprintResources/StandardMacros.IsValid` _returnvalue
        (:`Is Valid`
          (cast `/Game/Blueprints/BP_Defender_Base` (`Controller.K2_GetPawn` _returnvalue)
            (:`then`
              (`SceneComponent.K2_SetWorldRotation` _papersprite (struct :`Roll` -90.0) false false))
            (:`CastFailed`
              (`SceneComponent.SetVisibility` _papersprite false false))))))))

(event `Server_CheckShield`
  ;[1 1 1] Check if shield should be active; Need to be overworked, cause of the onTickEvent calling it to often
  (set `self.bShieldActiveTemp` false)
  (for _array_element (`self.DroneSpawnerReference`)
    (if (> (`/Game/Blueprints/Components/BP_HealthComponent.CurrentHealth` (`/Game/Blueprints/BP_Generator.BP_HealthComponent` _array_element)) 0.0)
      (set `self.bShieldActiveTemp` true)))
  ;[1 1 1] Only change the OnRepNotify variable, if there was a change
  (if (!= (`self.bShieldActiveTemp`) (`self.bShieldActive`))
    (set `self.bShieldActive` (`self.bShieldActiveTemp`))))

(fn `OnRep_bShieldActive`
  (bind _shield (`self.Shield`))
  (if (`self.bShieldActive`)
    (`SceneComponent.SetVisibility` _shield true true)
    (else
      (`SceneComponent.SetVisibility` _shield false true))))

(fn `UserConstructionScript`)