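; Game mode for an asymmetric multiplayer game that spawns joining players as either an FPS character or a villain.
; On PostLogin, the server records the controller, caches all PlayerStarts, spawns a pawn at the current one, possesses it and activates input.
; The spawn index also picks the role: index zero gives the FPS character, any other the villain.
; IncrementPlayerSpawnIndex cycles that index, wrapping to zero.
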(event `self.K2_PostLogin`
  (params (NewPlayer :type "PlayerController Object Reference"))
  (bind _lastusedplayerspawn (`self.LastUsedPlayerSpawn`))
  (bind _returnvalue (`SceneComponent.K2_GetComponentToWorld` (`Actor.RootComponent` (`|GetArrayItem` (`self.PlayerSpawns`) _lastusedplayerspawn))))
  (`/Engine/EditorBlueprintResources/ActorMacros.Switch Has Authority`
    (:`Authority`
      (`|ExecutionSequence`
        (:`then_0`
          ;[1 1 1] Add recently joined player to the controller list
          (`KismetArrayLibrary.Array_Add` (`self.ConnectedPlayerController`) NewPlayer))
        (:`then_1`
          ;[1 1 1] Get all playerspawns, if the array has not been created yet
          (if (== (`KismetArrayLibrary.Array_Length` (`self.PlayerSpawns`)) 0)
            (bind _outactors (`GameplayStatics.GetAllActorsOfClass` "/Script/Engine.PlayerStart"))
            (set `self.PlayerSpawns` _outactors)))
        (:`then_2`
          ;[1 1 1] Spawn an actor for the player and possess it
          (if (< _lastusedplayerspawn 1)
            (bind _returnvalue_2 (`|SpawnActorFromClass` "/Game/Blueprints/BP_FPS_Character.BP_FPS_Character_C" _returnvalue "AdjustIfPossibleButAlwaysSpawn" "OverrideRootScale" null null))
            (`self.IncrementPlayerSpawnIndex`)
            (`Controller.Possess` NewPlayer _returnvalue_2)
            (bind _asbp_player_controller (cast `/Game/Blueprints/BP_PlayerController` NewPlayer))
            (`/Game/Blueprints/BP_PlayerController.ActivateInput` _asbp_player_controller)
            (else
              (bind _returnvalue_3 (`|SpawnActorFromClass` "/Game/Blueprints/BP_VillainGameplay.BP_VillainGameplay_C" _returnvalue "Undefined" "OverrideRootScale" null null))
              (`self.IncrementPlayerSpawnIndex`)
              (`Controller.Possess` NewPlayer _returnvalue_3)
              (bind _asbp_player_controller_2 (cast `/Game/Blueprints/BP_PlayerController` NewPlayer))
              (`/Game/Blueprints/BP_PlayerController.ActivateInput` _asbp_player_controller_2))))))))

(fn `IncrementPlayerSpawnIndex`
  (bind _returnvalue (+ (`self.LastUsedPlayerSpawn`) 1))
  (if (< _returnvalue (`KismetArrayLibrary.Array_Length` (`self.PlayerSpawns`)))
    (set `self.LastUsedPlayerSpawn` _returnvalue)
    (else
      (set `self.LastUsedPlayerSpawn` 0))))

(fn `UserConstructionScript`)