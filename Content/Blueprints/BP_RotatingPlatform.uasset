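; BP_RotatingPlatform is a platform actor that spins continuously around its vertical axis.
; On BeginPlay it places the static mesh at a DistanceToParent offset relative to its parent.
; Each Tick it adds RotationSpeed scaled by delta time to the Scene component's yaw, setting pitch and roll to zero.
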(event `self.ReceiveBeginPlay`
  (`SceneComponent.K2_SetRelativeLocation` (`self.StaticMesh`) (`self.DistanceToParent`) false false))

(event `self.ReceiveTick`
  (params (DeltaSeconds :type "Float (single-precision)"))
  (bind (_relativerotation_roll _relativerotation_pitch _relativerotation_yaw) (`KismetMathLibrary.BreakRotator` (`SceneComponent.RelativeRotation` (`self.Scene`))))
  (`SceneComponent.K2_SetRelativeRotation` (`self.Scene`) (`KismetMathLibrary.MakeRotator` 0.0 0.0 (+ (* DeltaSeconds (`self.RotationSpeed`)) _relativerotation_yaw)) false false))

(fn `UserConstructionScript`)