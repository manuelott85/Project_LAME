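; Actor component that tracks a player's XP, level and upgrade points and shows XP progress and points on the HUD.
; AlterXP carries surplus XP over on level-up, granting one upgrade point and at most one level per call.
; Thresholds come from a per-level array, then stay at the last entry times a cap multiplier.
; CurrentXP's RepNotify refreshes the HUD, as does a delayed BeginPlay for the locally controlled pawn.
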(event `UpdateHUD`
  (bind _activehud (`self.ActiveHUD`))
  (bind _xpneededperlvl (`self.XPNeededPerLvl`))
  (bind _currentlvl (`self.CurrentLvl`))
  (bind _xpneededperlvl_2 (`self.XPNeededPerLvl`))
  (bind _progressbar_xp (`/Game/Widget/W_VillainHUD.ProgressBar_XP` _activehud))
  ;[1 1 1] UpdateHUD
  (`/Engine/EditorBlueprintResources/StandardMacros.IsValid` _activehud
    (:`Is Valid`
      (if (> (`KismetArrayLibrary.Array_Length` _xpneededperlvl_2) _currentlvl)
        (`ProgressBar.SetPercent` _progressbar_xp (/ (`KismetMathLibrary.Conv_IntToDouble` (`self.CurrentXP`)) (`KismetMathLibrary.Conv_IntToDouble` (`|GetArrayItem` _xpneededperlvl_2 _currentlvl))))
        (else
          (`ProgressBar.SetPercent` _progressbar_xp (/ (`KismetMathLibrary.Conv_IntToDouble` (`self.CurrentXP`)) (* (`KismetMathLibrary.Conv_IntToDouble` (`|GetArrayItem` _xpneededperlvl (`KismetArrayLibrary.Array_LastIndex` _xpneededperlvl))) (`self.XpNeededMultiplierAtCap`))))))
      (`TextBlock.SetText` (`/Game/Widget/W_VillainHUD.Text_AmountUpgradePoints` _activehud) (`KismetTextLibrary.Conv_IntToText` (`self.CurrentUpgradePoints`))))))

(event `self.ReceiveBeginPlay`
  ;[1 1 1] BeginPlay
  ;[1 1 1] Only the owning client should execute
  (if (== (`Controller.K2_GetPawn` (`GameplayStatics.GetPlayerController` 0)) (`self.GetOwner` self))
    ;[1 1 1] Wait for the HUD reference
    (`KismetSystemLibrary.Delay` 0.2)
    (`self.UpdateHUD`)))

(event `Alter XP`
  (params (Amount :type Integer))
  (bind _xpneededperlvl (`self.XPNeededPerLvl`))
  (bind _xpneededperlvl_2 (`self.XPNeededPerLvl`))
  (bind _currentlvl (`self.CurrentLvl`))
  (bind _returnvalue (+ Amount (`self.CurrentXP`)))
  (bind _output (`|GetArrayItem` _xpneededperlvl _currentlvl))
  (bind _returnvalue_2 (`KismetMathLibrary.FTrunc` (* (`KismetMathLibrary.Conv_IntToDouble` (`|GetArrayItem` _xpneededperlvl_2 (`KismetArrayLibrary.Array_LastIndex` _xpneededperlvl_2))) (`self.XpNeededMultiplierAtCap`))))
  ;[1 1 1] AlterXP
  ;;[1 1 1] Check, if a value is set for current level in array
  (if (> (`KismetArrayLibrary.Array_Length` _xpneededperlvl) _currentlvl)
    (if (> _output _returnvalue)
      (set `self.CurrentXP` _returnvalue)
      (else
        (set `self.CurrentXP` (- _returnvalue _output))
        (set `self.CurrentLvl` (+ (`self.CurrentLvl`) 1))
        (`self.AlterUpgradePoints` 1)))
    (elif (> _returnvalue_2 _returnvalue)
      (set `self.CurrentXP` _returnvalue)
      (else
        (set `self.CurrentXP` (- _returnvalue _returnvalue_2))
        (set `self.CurrentLvl` (+ (`self.CurrentLvl`) 1))
        (`self.AlterUpgradePoints` 1)))))

(event `AlterUpgradePoints`
  (params (Amount :type Integer))
  (set `self.CurrentUpgradePoints` (+ Amount (`self.CurrentUpgradePoints`))))

(fn `OnRep_CurrentXP`
  (`self.UpdateHUD`))