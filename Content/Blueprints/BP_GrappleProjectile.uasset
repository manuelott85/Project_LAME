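; BP_GrappleProjectile is the visual projectile of a grapple, flying toward a target location.
; Each tick it moves its Sphere component toward TargetLocation at constant speed with VInterpToConstant, without sweeping for collision.
; Once within a small radius it plays a concrete impact sound once, guarded by a flag, then destroys itself after a short delay.
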(event `self.ReceiveTick`
  (params (DeltaSeconds :type "Float (single-precision)"))
  (bind _targetlocation (`self.TargetLocation`))
  (bind _returnvalue (`SceneComponent.K2_GetComponentLocation` (`self.Sphere`)))
  (if (> (`KismetMathLibrary.VSize` (- _returnvalue _targetlocation)) 50.0)
    (`SceneComponent.K2_SetWorldLocation` (`self.Sphere`) (`KismetMathLibrary.VInterpTo_Constant` _returnvalue _targetlocation DeltaSeconds 5000.0) false false)
    (elif (not (`self.SoundTriggered`))
      (`GameplayStatics.PlaySoundAtLocation` "/Game/Sounds/Grappeling_Impact_Concrete_Cue.Grappeling_Impact_Concrete_Cue" _returnvalue (struct) 1.0 1.0 0.0 null null null)
      (set `self.SoundTriggered` true)
      (`KismetSystemLibrary.Delay` 0.2)
      (`self.K2_DestroyActor`))))

(fn `UserConstructionScript`)