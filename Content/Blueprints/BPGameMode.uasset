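; Game mode that spawns and possesses an FPS character for each player who joins, running with server authority.
; On PostLogin it records the controller, caches the level's PlayerStarts on first use, and spawns the character at the current start, adjusting for collisions but always spawning.
; A wrapping index rotates through the starts round-robin.
; After possession it activates input on the custom player controller.
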(event `self.K2_PostLogin`
  (params (NewPlayer :type "PlayerController Object Reference"))
  (`/Engine/EditorBlueprintResources/ActorMacros.Switch Has Authority`
    (:`Authority`
      (`|ExecutionSequence`
        (:`then_0`
          ;[1 1 1] Add recently joined player to the controller list
          (`KismetArrayLibrary.Array_Add` (`self.ConnectedPlayerController`) NewPlayer))
        (:`then_1`
          ;[1 1 1] Get all playerspawns, if the array has not been created yet
          (if (== (`KismetArrayLibrary.Array_Length` (`self.PlayerSpawns`)) 0)
            (bind _outactors (`GameplayStatics.GetAllActorsOfClass` "/Script/Engine.PlayerStart"))
            (set `self.PlayerSpawns` _outactors)))
        (:`then_2`
          ;[1 1 1] Spawn an actor for the player and possess it
          (bind _returnvalue (`|SpawnActorFromClass` "/Game/Blueprints/BP_FPS_Character.BP_FPS_Character_C" (`SceneComponent.K2_GetComponentToWorld` (`Actor.RootComponent` (`|GetArrayItem` (`self.PlayerSpawns`) (`self.LastUsedPlayerSpawn`)))) "AdjustIfPossibleButAlwaysSpawn" "OverrideRootScale" null null))
          (`self.IncrementPlayerSpawnIndex`)
          (`Controller.Possess` NewPlayer _returnvalue)
          (bind _asbpplayer_controller (cast `/Game/Blueprints/BPPlayerController` NewPlayer))
          (`/Game/Blueprints/BPPlayerController.ActivateInput` _asbpplayer_controller))))))

(fn `IncrementPlayerSpawnIndex`
  (bind _returnvalue (+ (`self.LastUsedPlayerSpawn`) 1))
  (if (< _returnvalue (`KismetArrayLibrary.Array_Length` (`self.PlayerSpawns`)))
    (set `self.LastUsedPlayerSpawn` _returnvalue)
    (else
      (set `self.LastUsedPlayerSpawn` 0))))

(fn `UserConstructionScript`)