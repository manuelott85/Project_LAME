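; Grappling-hook "magnet" component that pulls the owning BP_FPS_Character toward a traced surface.
; ActivateMagnetV2 spends a charge, aims above static mesh tops to clear ledges and spawns BP_GrappleProjectile; StartMovement begins the pull.
; Tick follows the target via a stored offset, using swept constant-speed interpolation or legacy flying input per EnableNewGrappleMode, recharges charges and updates W_HeroHUD.
; DisableMagnet restores falling, keeping momentum if short of target, and destroys projectiles.
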(event `self.ReceiveBeginPlay`
  (set `self.CurrentCharges` (`self.MaximumCharges`))
  (`self.UpdateUI`))

(event `self.ReceiveTick`
  (params (DeltaSeconds :type "Float (single-precision)"))
  (`|ExecutionSequence`
    (:`then_0`
      (if (`self.MagnetActive`)
        (bind _asbp_fps_character (cast `/Game/Blueprints/BP_FPS_Character` (`self.GetOwner`)))
        (if (`/Game/Blueprints/BP_FPS_Character.EnableNewGrappleMode` _asbp_fps_character)
          (`self.MoveToTargetV2` DeltaSeconds)
          (else
            (`self.MoveToTarget` DeltaSeconds)))))
    (:`then_1`
      (`self.UpdateCooldown` DeltaSeconds)
      (`self.UpdateUI`))))

(event `StartMovement`
  (set `self.MagnetActive` true)
  (bind _asbp_fps_character (cast `/Game/Blueprints/BP_FPS_Character` (`self.GetOwner`)))
  (set `/Game/Blueprints/BP_FPS_Character.DoubleJump` false _asbp_fps_character)
  (`AudioComponent.Play` (`/Game/Blueprints/BP_FPS_Character.Grappeling_pulling_Cue` _asbp_fps_character) 0.0))

(fn `ActivateMagnet`
  (params (StartPosition :type "Vector Structure") (Direction :type "Vector Structure"))
  (locals (Debug :type Boolean :default false) (ObjectLocation :type "Vector Structure"))
  (bind (_outhit _returnvalue) (`KismetSystemLibrary.LineTraceSingle` :`Start` StartPosition :`End` (+ StartPosition (* Direction (`self.Range`))) :`TraceChannel` "TraceTypeQuery1" :`DrawDebugType` "ForOneFrame" :`DrawTime` 1000.0))
  (if _returnvalue
    (bind (_bblockinghit _binitialoverlap _time _distance _location _impactpoint _normal _impactnormal _physmat _hitactor _hitcomponent) (`GameplayStatics.BreakHitResult` _outhit))
    (if (`KismetSystemLibrary.IsValid` _hitactor)
      (set `self.Target` _hitactor)
      (set `local.ObjectLocation` (`Actor.K2_GetActorLocation` _hitactor))
      (else
        (set `self.Target` _hitcomponent)
        (set `local.ObjectLocation` (`SceneComponent.K2_GetComponentLocation` _hitcomponent))))
    (if (`local.Debug`)
      (`KismetSystemLibrary.DrawDebugSphere` StartPosition 50.0 4 (struct :`R` 0.035435 :`G` 1.0 :`A` 1.0) 500.0 3.0)
      (`KismetSystemLibrary.DrawDebugSphere` _location 50.0 4 (struct :`R` 1.0 :`B` 0.265872 :`A` 1.0) 500.0 3.0)
      (`KismetSystemLibrary.PrintText` (`KismetTextLibrary.Conv_VectorToText` _location)))
    (bind _output_get (set `self.ImpactLocationOffset` (- (`local.ObjectLocation`) _location)))
    (if (`local.Debug`)
      (`KismetSystemLibrary.PrintText` (`KismetTextLibrary.Conv_VectorToText` _output_get)))
    (set `self.MagnetActive` true)
    (`GameplayStatics.PlaySoundAtLocation` "/Game/Sounds/Grappeling_firing.Grappeling_firing" (`Actor.K2_GetActorLocation` (`self.GetOwner`)) (struct) 1.0 1.0 0.0 null null null)
    (bind _asbp_fps_character (cast `/Game/Blueprints/BP_FPS_Character` (`self.GetOwner`)))
    (`AudioComponent.Play` (`/Game/Blueprints/BP_FPS_Character.Grappeling_pulling_Cue` _asbp_fps_character) 0.0)))

(fn `ActivateMagnetV2`
  (params (StartPosition :type "Vector Structure") (Direction :type "Vector Structure"))
  (locals (Debug :type Boolean :default true) (TargetLocation :type "Vector Structure") (GrappleGunLocation :type "Vector Structure"))
  (set `local.GrappleGunLocation` StartPosition)
  (bind (_outhit _returnvalue) (`KismetSystemLibrary.LineTraceSingle` :`Start` StartPosition :`End` (+ StartPosition (* Direction (`self.Range`))) :`TraceChannel` "TraceTypeQuery1" :`DrawDebugType` "ForOneFrame" :`DrawTime` 1000.0))
  (if _returnvalue
    (bind _sufficientcharges (`self.CheckCharges`))
    (if _sufficientcharges
      (bind (_bblockinghit _binitialoverlap _time _distance _location _impactpoint _normal _impactnormal _physmat _hitactor _hitcomponent) (`GameplayStatics.BreakHitResult` _outhit))
      (`KismetSystemLibrary.PrintString` (`KismetSystemLibrary.GetDisplayName` _hitcomponent))
      (bind _asstatic_mesh_component (cast `StaticMeshComponent` _hitcomponent)
        (:`then`
          (bind _returnvalue_2 (`self.FindHighestPointInMesh` _asstatic_mesh_component))
          (set `self.Target` _hitcomponent)
          (set `local.TargetLocation` (`KismetMathLibrary.MakeVector` (.x _impactpoint) (.y _impactpoint) _returnvalue_2)))
        (:`CastFailed`
          (bind _asmodel_component (cast `ModelComponent` _hitcomponent))
          (set `self.Target` _asmodel_component)
          (set `local.TargetLocation` _impactpoint)))
      (bind _asbp_fps_character (cast `/Game/Blueprints/BP_FPS_Character` (`self.GetOwner`)))
      (bind _returnvalue_3 (+ (`local.TargetLocation`) (`KismetMathLibrary.MakeVector` 0.0 0.0 (`CapsuleComponent.GetScaledCapsuleHalfHeight` (`Character.CapsuleComponent` _asbp_fps_character)))))
      (`KismetSystemLibrary.DrawDebugSphere` _returnvalue_3 1.0 4 (struct :`G` 1.0 :`B` 0.306961 :`A` 1.0) 20.0 5.0)
      (bind _output_get (set `self.ImpactLocationOffset` (- (`SceneComponent.K2_GetComponentLocation` _hitcomponent) _returnvalue_3)))
      (if (`local.Debug`)
        (`KismetSystemLibrary.PrintText` (`KismetTextLibrary.Conv_VectorToText` _output_get)))
      (`self.PlaySoundFX` (`local.TargetLocation`))
      (bind _returnvalue_4 (`|SpawnActorFromClass` "/Game/Blueprints/BP_GrappleProjectile.BP_GrappleProjectile_C" (`KismetMathLibrary.MakeTransform` (`local.GrappleGunLocation`) (`KismetMathLibrary.FindLookAtRotation` (`local.GrappleGunLocation`) (`local.TargetLocation`))) "Undefined" "OverrideRootScale" (`self.GetOwner`) null))
      (set `/Game/Blueprints/BP_GrappleProjectile.TargetLocation` (`local.TargetLocation`) _returnvalue_4))))

(fn `CalculateTargetLocation`
  (returns (HitLocation :type "Vector Structure"))
  (bind _target (`self.Target`))
  (bind _asactor (cast `Actor` _target)
    (:`then`
      (return (- (`Actor.K2_GetActorLocation` _asactor) (`self.ImpactLocationOffset`))))
    (:`CastFailed`
      (bind _asprimitive_component (cast `PrimitiveComponent` _target))
      (return (- (`SceneComponent.K2_GetComponentLocation` _asprimitive_component) (`self.ImpactLocationOffset`))))))

(fn `CheckCharges`
  (returns (SufficientCharges :type Boolean))
  (if (>= (`self.CurrentCharges`) 1)
    (`/Engine/EditorBlueprintResources/StandardMacros.DecrementInt` (`self.CurrentCharges`)
      (:`  `
        (if (<= (`self.CurrentCooldown`) 0.0)
          (set `self.CurrentCooldown` (`self.ChargeCooldown`)))
        (return true)))
    (else
      (`KismetSystemLibrary.PrintString` "Insufficient Magnet Charges")
      (return false))))

(fn `CheckDistance`
  (params (TargetLocation :type "Vector Structure"))
  (returns (LocationReached :type Boolean))
  (bind _returnvalue (`Actor.K2_GetActorLocation` (`self.GetOwner`)))
  (`KismetSystemLibrary.DrawDebugSphere` _returnvalue 1.0 4 (struct :`R` 1.0 :`G` 0.021407 :`A` 1.0) 20.0 5.0)
  (`KismetSystemLibrary.DrawDebugSphere` TargetLocation 1.0 4 (struct :`G` 0.356638 :`B` 1.0 :`A` 1.0) 20.0 5.0)
  (return (and (>= (.z _returnvalue) (.z TargetLocation)) (<= (`KismetMathLibrary.VSize` (- TargetLocation _returnvalue)) (`self.DistanceTolerance`)))))

(fn `DisableMagnet`
  (locals (PlayerCharacter :type "/Game/Blueprints/BP_FPS_Character Object Reference"))
  (bind _playercharacter (`local.PlayerCharacter`))
  (bind _charactermovement (`Character.CharacterMovement` (`local.PlayerCharacter`)))
  (set `self.MagnetActive` false)
  (bind _asbp_fps_character (cast `/Game/Blueprints/BP_FPS_Character` (`self.GetOwner`)))
  (set `local.PlayerCharacter` _asbp_fps_character)
  (bind _hitlocation (`self.CalculateTargetLocation`))
  (bind _locationreached (`self.CheckDistance` _hitlocation))
  (if _locationreached
    (`MovementComponent.StopMovementImmediately` _charactermovement)
    (else
      (set `MovementComponent.Velocity` (* (`KismetMathLibrary.Normal` (- _hitlocation (`SceneComponent.K2_GetComponentLocation` (`Character.Mesh` (`local.PlayerCharacter`))))) (/ (* (`self.GrappleSpeed`) 300.0) (`self.DecelerationSpeed`))) _charactermovement)))
  (`CharacterMovementComponent.SetMovementMode` _charactermovement "MOVE_Falling" 0)
  (`AudioComponent.Stop` (`/Game/Blueprints/BP_FPS_Character.Grappeling_pulling_Cue` _playercharacter))
  (bind _outactors (`GameplayStatics.GetAllActorsOfClass` "/Game/Blueprints/BP_GrappleProjectile.BP_GrappleProjectile_C"))
  (for _array_element _outactors
    (`Actor.K2_DestroyActor` _array_element))
  (`GameplayStatics.PlaySoundAtLocation` "/Game/Sounds/Grappeling_Reconnecting_Cue.Grappeling_Reconnecting_Cue" (`SceneComponent.K2_GetComponentLocation` (`Character.Mesh` _playercharacter)) (struct) 1.0 1.0 0.0 null null null))

(fn `FindHighestPointInMesh`
  (params (StaticMesh :type "StaticMeshComponent Object Reference"))
  (returns (ReturnValue :type "Float (double-precision)"))
  (bind (_returnvalue_x _returnvalue_y _returnvalue_z) (`KismetMathLibrary.BreakVector` (`SceneComponent.K2_GetComponentLocation` StaticMesh)))
  (bind (_returnvalue_x_2 _returnvalue_y_2 _returnvalue_z_2) (`KismetMathLibrary.BreakVector` (`SceneComponent.K2_GetComponentScale` StaticMesh)))
  (return (+ _returnvalue_z (* (.z (`.Max` (`StaticMeshComponent.GetLocalBounds` StaticMesh))) _returnvalue_z_2))))

(fn `MoveToTarget`
  (params (DeltaSeconds :type "Float (double-precision)"))
  (locals (HitLocation :type "Vector Structure") (Debug :type Boolean :default false) (ElapsedTime :type "Float (double-precision)"))
  (bind _hitlocation (`local.HitLocation`))
  (bind (_hitlocation_x _hitlocation_y _hitlocation_z) (`KismetMathLibrary.BreakVector` (`local.HitLocation`)))
  (bind _hitlocation_2 (`local.HitLocation`))
  (bind _hitlocation_3 (`self.CalculateTargetLocation`))
  (bind _output_get (set `local.HitLocation` _hitlocation_3))
  (bind _locationreached (`self.CheckDistance` _output_get))
  (if _locationreached
    (if (`self.LooseVelocityOnLocationReached`)
      ;[1 1 1] Stop moving when reaching target location
      (bind _asbp_fps_character (cast `/Game/Blueprints/BP_FPS_Character` (`self.GetOwner`)))
      (set `MovementComponent.Velocity` (0.0 0.0 0.0) (`Character.CharacterMovement` _asbp_fps_character)))
    (else
      (if (`local.Debug`)
        (`KismetSystemLibrary.DrawDebugSphere` _hitlocation 200.0 4 (struct :`G` 0.140895 :`B` 1.0 :`A` 1.0) 1000.0 5.0)
        (`KismetSystemLibrary.PrintText` (`KismetTextLibrary.Conv_VectorToText` _hitlocation)))
      (bind _asbp_fps_character_2 (cast `/Game/Blueprints/BP_FPS_Character` (`self.GetOwner`)))
      (bind _charactermovement (`Character.CharacterMovement` _asbp_fps_character_2))
      (if (`|EnumInequality` (`CharacterMovementComponent.MovementMode` _charactermovement) "MOVE_Flying")
        (`CharacterMovementComponent.SetMovementMode` _charactermovement "MOVE_Flying" 0))
      (set `CharacterMovementComponent.MaxAcceleration` (`self.MaxTravelSpeed`) _charactermovement)
      (bind _returnvalue (`Actor.K2_GetActorLocation` _asbp_fps_character_2))
      (`Pawn.AddMovementInput` _asbp_fps_character_2 (- _hitlocation_2 _returnvalue) 1.0 false)
      (`KismetSystemLibrary.DrawDebugLine` _hitlocation_2 _returnvalue (struct :`G` 0.490464 :`B` 0.647569 :`A` 1.0) 0.0 2.0)
      (bind (_returnvalue_x _returnvalue_y _returnvalue_z) (`KismetMathLibrary.BreakVector` (`Actor.K2_GetActorLocation` _asbp_fps_character_2)))
      (bind _velocity (`MovementComponent.Velocity` _charactermovement))
      (if (and (>= _returnvalue_z _hitlocation_z) (> (.z _velocity) 0.0))
        (set `MovementComponent.Velocity` (* _velocity (1.0 1.0 0.0)) _charactermovement)))))

(fn `MoveToTargetV2`
  (params (DeltaSeconds :type "Float (double-precision)"))
  (locals (HitLocation :type "Vector Structure") (Debug :type Boolean :default false) (ElapsedTime :type "Float (double-precision)") (PlayerCharacter :type "/Game/Blueprints/BP_FPS_Character Object Reference"))
  (bind _playercharacter (`local.PlayerCharacter`))
  (bind _hitlocation (`local.HitLocation`))
  (set `local.ElapsedTime` DeltaSeconds)
  (bind _hitlocation_2 (`self.CalculateTargetLocation`))
  (bind _output_get (set `local.HitLocation` _hitlocation_2))
  (bind _locationreached (`self.CheckDistance` _output_get))
  (if _locationreached
    ;[1 1 1] Disable grapple when reaching target
    (`self.DisableMagnet`)
    (else
      (if (`local.Debug`)
        (`KismetSystemLibrary.DrawDebugSphere` _hitlocation 200.0 4 (struct :`G` 0.140895 :`B` 1.0 :`A` 1.0) 1000.0 5.0)
        (`KismetSystemLibrary.PrintText` (`KismetTextLibrary.Conv_VectorToText` _hitlocation)))
      (bind _asbp_fps_character (cast `/Game/Blueprints/BP_FPS_Character` (`self.GetOwner`)))
      (bind _output_get_2 (set `local.PlayerCharacter` _asbp_fps_character))
      (bind _charactermovement (`Character.CharacterMovement` _output_get_2))
      (if (`|EnumInequality` (`CharacterMovementComponent.MovementMode` _charactermovement) "MOVE_Flying")
        (`CharacterMovementComponent.SetMovementMode` _charactermovement "MOVE_Flying" 0))
      (bind _sweephitresult (`SceneComponent.K2_SetWorldLocation` (`Actor.RootComponent` _output_get_2) (`KismetMathLibrary.VInterpTo_Constant` (`Actor.K2_GetActorLocation` _output_get_2) (`local.HitLocation`) (`local.ElapsedTime`) (* (`self.GrappleSpeed`) 300.0)) true false))
      (if (`GameplayStatics.BreakHitResult` _sweephitresult)
        (`CharacterMovementComponent.SetMovementMode` (`Character.CharacterMovement` _playercharacter) "MOVE_Walking" 0)
        (`Character.Jump` _playercharacter)))))

(fn `PlaySoundFX`
  (params (Location :type "Vector Structure"))
  (`GameplayStatics.PlaySoundAtLocation` "/Game/Sounds/Grappeling_firing.Grappeling_firing" (`Actor.K2_GetActorLocation` (`self.GetOwner`)) (struct) 1.0 1.0 0.0 null null null))

(fn `UpdateCooldown`
  (params (ElapsedTime :type "Float (double-precision)"))
  (if (and (<= (`self.CurrentCooldown`) 0.0) (< (`self.CurrentCharges`) (`self.MaximumCharges`)))
    (`/Engine/EditorBlueprintResources/StandardMacros.IncrementInt` (`self.CurrentCharges`)
      (:`  `
        (set `self.CurrentCooldown` (`self.ChargeCooldown`))))
    (else
      (set `self.CurrentCooldown` (- (`self.CurrentCooldown`) ElapsedTime)))))

(fn `UpdateUI`
  (bind _foundwidgets (`WidgetBlueprintLibrary.GetAllWidgetsOfClass` "/Game/Widget/W_HeroHUD.W_HeroHUD_C"))
  (for _array_element _foundwidgets
    (`TextBlock.SetText` (`/Game/Widget/W_HeroHUD.GrappleUses` _array_element) (`KismetTextLibrary.Conv_IntToText` (`self.CurrentCharges`)))
    (if (> (`self.CurrentCooldown`) 0.0)
      (bind _cooldownbar (`/Game/Widget/W_HeroHUD.CooldownBar` _array_element))
      (`ProgressBar.SetPercent` _cooldownbar (/ (- (`self.ChargeCooldown`) (`self.CurrentCooldown`)) (`self.ChargeCooldown`)))
      (else
        (`ProgressBar.SetPercent` _cooldownbar 1.0)))))