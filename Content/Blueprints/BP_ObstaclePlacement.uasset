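; Player-controlled pawn that lets a player place replicated obstacles, currently delivery drone actors, by touch or mouse click.
; BeginPlay shows a crosshair cursor and sets the camera's orthographic width from CameraHeight, while a perspective height alternative sits unconnected.
; Touch and Shoot input trace the Visibility channel under the finger or cursor into ProcessTouch.
; ProcessTouch prints the hit actor's name and sends the location to a server event that spawns the drone.
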(event `self.ReceiveBeginPlay`
  ;[1 1 1] Enable mouse cursor and set cursor to crosshairs
  (bind _asplayer_controller (cast `PlayerController` (`self.GetController`)))
  (set `PlayerController.bShowMouseCursor` true _asplayer_controller)
  (set `PlayerController.CurrentMouseCursor` "Crosshairs" _asplayer_controller)
  ;[1 1 1] Camera Heigth Orthographic
  (`CameraComponent.SetOrthoWidth` (`self.Camera`) (`self.CameraHeight`)))

(event `InputTouch`
  (params (Location :type "Vector Structure") (FingerIndex :type "ETouchIndex Enum"))
  ;[1 1 1] Raycast on Touch and send location to server
  (:`Pressed`
    (bind _asplayer_controller (cast `PlayerController` (`self.GetController`)))
    (`PlayerController.SetMouseLocation` _asplayer_controller (`KismetMathLibrary.FTrunc` (.x Location)) (`KismetMathLibrary.FTrunc` (.y Location)))
    (`self.Process Touch` (`PlayerController.GetHitResultUnderFingerByChannel` _asplayer_controller FingerIndex "TraceTypeQuery1" true))))

(event `Process Touch`
  (params (`Hit Result` :type "HitResult Structure"))
  (bind (_bblockinghit _binitialoverlap _time _distance _location _impactpoint _normal _impactnormal _physmat _hitactor) (`GameplayStatics.BreakHitResult` `Hit Result`))
  ;[1 1 1] Process the HitResult
  (`KismetSystemLibrary.PrintText` (`KismetTextLibrary.Conv_StringToText` (`KismetSystemLibrary.GetDisplayName` _hitactor)))
  (`self.RunOnServer_CreateObstacle` _location))

(event `InputAction|Shoot`
  (params (Key :type "Key Structure"))
  ;[1 1 1] Raycast on Mouse and send location to server
  (:`Pressed`
    (bind _asplayer_controller (cast `PlayerController` (`self.GetController`)))
    (`self.Process Touch` (`PlayerController.GetHitResultUnderCursorByChannel` _asplayer_controller "TraceTypeQuery1" false))))

(event `RunOnServer_CreateObstacle`
  (params (SpawnLocation :type "Vector Structure"))
  ;[1 1 1] Spawn Obstacle on transmitted location
  (bind _returnvalue (`|SpawnActorFromClass` "/Game/Blueprints/AI/EnergyDelivery/BP_DeliveryDrone_Mark1.BP_DeliveryDrone_Mark1_C" (`KismetMathLibrary.MakeTransform` SpawnLocation) "AlwaysSpawn" "OverrideRootScale" null null))
  (`self.SetReplicates` _returnvalue true)
  (`self.SetReplicateMovement` _returnvalue true))

(fn `UserConstructionScript`)