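; Behavior tree task that picks a random navigable point around the controlled pawn using the DoN Navigation manager.
; Radius feeds both the search distance and the maximum Z angular displacement.
; A valid result is written to the LocationToConvert blackboard key and the task succeeds; otherwise it fails.
; A check rejecting points beyond MaximumTravelDist is present but disconnected, so it never runs.
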(event `self.ReceiveExecuteAI`
  (params (OwnerController :type "AIController Object Reference") (ControlledPawn :type "Pawn Object Reference"))
  (bind _radius (`self.Radius`))
  (bind (_bfoundvalidresult _returnvalue) (`DonNavigationManager.FindRandomPointAroundOriginInNavWorld` (`DonNavigationHelper.DonNavigationManager`) ControlledPawn (0.0 0.0 0.0) _radius -1.0 _radius 5))
  (if _bfoundvalidresult
    (`BTFunctionLibrary.SetBlackboardValueAsVector` (`self.LocationToConvert`) _returnvalue)
    (`self.FinishExecute` true)
    (else
      (`self.FinishExecute` false))))