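; Behavior Tree decorator that, despite its TargetIsVisible name, checks whether the AI's own actor is facing a target, with no trace or sight test.
; It reads both actors from blackboard keys and compares the self actor's rotation to the look-at rotation toward the target.
; It passes while the rotations differ beyond a small tolerance, and fails when they match or either actor is missing.
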(fn `PerformConditionCheckAI`
  (params (OwnerController :type "AIController Object Reference") (ControlledPawn :type "Pawn Object Reference"))
  (returns (ReturnValue :type Boolean))
  (bind _returnvalue (`AIBlueprintHelperLibrary.GetBlackboard` OwnerController))
  (bind _asactor (cast `Actor` (`BlackboardComponent.GetValueAsObject` _returnvalue (`self.ActorToLookFor`)))
    (:`then`
      (bind _asactor_2 (cast `Actor` (`BlackboardComponent.GetValueAsObject` _returnvalue (`self.SelfActor`)))
        (:`then`
          (if (== (`Actor.K2_GetActorRotation` _asactor_2) (`KismetMathLibrary.FindLookAtRotation` (`Actor.K2_GetActorLocation` _asactor_2) (`Actor.K2_GetActorLocation` _asactor)) :`ErrorTolerance` 2.0)
            (return false)
            (else
              (return true))))
        (:`CastFailed`
          _)))
    (:`CastFailed`
      _))
  (return false))