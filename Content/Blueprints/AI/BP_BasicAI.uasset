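; BP_BasicAI is an AI-controlled actor that runs the BT_BasicAI behavior tree on BeginPlay and can fire projectiles.
; StartFire spawns a damage-carrying BP_AIProjectile from the Sphere component, offset by GunOffset along its rotation, adjusting for collisions or skipping the spawn.
; StopFire only prints a debug message, and the firing sound node is left unconnected.
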(event `self.ReceiveBeginPlay`
  (`AIController.RunBehaviorTree` (`AIBlueprintHelperLibrary.GetAIController` self) "/Game/Blueprints/AI/BT_BasicAI.BT_BasicAI"))

(fn `StartFire`
  (bind _returnvalue (`SceneComponent.K2_GetComponentRotation` (`self.Sphere`)))
  (`KismetSystemLibrary.PrintString` "I start to fire")
  (`|SpawnActorFromClass` "/Game/Blueprints/AI/BP_AIProjectile.BP_AIProjectile_C" (`KismetMathLibrary.MakeTransform` (+ (`SceneComponent.K2_GetComponentLocation` (`self.Sphere`)) (`KismetMathLibrary.GreaterGreater_VectorRotator` (`self.GunOffset`) _returnvalue)) _returnvalue) "AdjustIfPossibleButDontSpawnIfColliding" "OverrideRootScale" null 10.0 null) ; Spawn projectile
)

(fn `StopFire`
  (`KismetSystemLibrary.PrintString` "I stop to fire"))

(fn `UserConstructionScript`)