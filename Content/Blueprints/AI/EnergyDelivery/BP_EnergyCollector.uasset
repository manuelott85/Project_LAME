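; BP_EnergyCollector is an energy drop-off actor where delivery drones turn their cargo into energy for the villain.
; On the server, a BP_DeliveryDrone_Base overlapping its DeliveryTrigger adds a fixed amount to the energy component of the first BP_VillainGameplay found in the world.
; The drone is then destroyed.
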(event `self.DeliveryTrigger.OnComponentBeginOverlap`
  (params (OverlappedComponent :type "PrimitiveComponent Object Reference") (OtherActor :type "Actor Object Reference") (OtherComp :type "PrimitiveComponent Object Reference") (OtherBodyIndex :type Integer) (bFromSweep :type Boolean) (SweepResult :type "HitResult Structure (by ref)"))
  ;[1 1 1] Check for valid delivery drone type & Server Only
  (`/Engine/EditorBlueprintResources/ActorMacros.Switch Has Authority`
    (:`Authority`
      (if (`.bSuccess` (cast `/Game/Blueprints/AI/EnergyDelivery/BP_DeliveryDrone_Base` OtherActor :!pure true))
        (`|ExecutionSequence`
          (:`then_0`
            ;[1 1 1] Add Energy to the villain
            (bind _outactors (`GameplayStatics.GetAllActorsOfClass` "/Game/Blueprints/BP_VillainGameplay.BP_VillainGameplay_C"))
            (`/Game/Blueprints/BP_EnergyComponent.AlterEnergy` (`/Game/Blueprints/BP_VillainGameplay.BP_EnergyComponent` (`|GetArrayItem` _outactors)) 10.0))
          (:`then_1`
            ;[1 1 1] Remove Drone after delivery
            (`self.K2_DestroyActor` OtherActor)))))))

(fn `UserConstructionScript`)