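; BP_EnergyField is an energy field actor that recharges carrier drones entering its DeliveryTrigger volume.
; On overlap, the server checks that the other actor is a BP_CarrierDrone_Base with a valid BPEnergyComponent.
; It then passes that component's MaxEnergy to AlterEnergy, adding a full charge's worth of energy in a single call.
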(event `self.DeliveryTrigger.OnComponentBeginOverlap`
  (params (OverlappedComponent :type "PrimitiveComponent Object Reference") (OtherActor :type "Actor Object Reference") (OtherComp :type "PrimitiveComponent Object Reference") (OtherBodyIndex :type Integer) (bFromSweep :type Boolean) (SweepResult :type "HitResult Structure (by ref)"))
  (bind (_asbp_carrier_drone_base _bsuccess) (cast `/Game/Blueprints/AI/EnergyDelivery/BP_CarrierDrone_Base` OtherActor :!pure true))
  (bind _bp_energycomponent (`/Game/Blueprints/AI/BP_Drone_Base.BP_EnergyComponent` _asbp_carrier_drone_base))
  ;[1 1 1] Check for valid delivery drone type & Server Only
  (`/Engine/EditorBlueprintResources/ActorMacros.Switch Has Authority`
    (:`Authority`
      (if _bsuccess
        ;[1 1 1] Add Energy to the carrier
        (`/Engine/EditorBlueprintResources/StandardMacros.IsValid` _bp_energycomponent
          (:`Is Valid`
            (`/Game/Blueprints/Components/BP_EnergyComponent.AlterEnergy` _bp_energycomponent (`/Game/Blueprints/Components/BP_EnergyComponent.MaxEnergy` _bp_energycomponent))))))))

(fn `UserConstructionScript`)