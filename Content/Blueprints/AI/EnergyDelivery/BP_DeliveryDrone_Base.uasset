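; BP_DeliveryDrone_Base is the base Blueprint for an AI delivery drone in the energy delivery system.
; On BeginPlay the authority runs the BT_DeliveryDrone behavior tree through the drone's AI controller, while remote instances make the Billboard component visible.
; Any damage received is forwarded to BPHealthComponent, which handles it.
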(event `self.ReceiveBeginPlay`
  (`|ExecutionSequence`
    (:`then_0`
      ;[1 1 1] Run behavior tree on server only
      (`/Engine/EditorBlueprintResources/ActorMacros.Switch Has Authority`
        (:`Authority`
          (`AIController.RunBehaviorTree` (`AIBlueprintHelperLibrary.GetAIController` self) "/Game/Blueprints/AI/EnergyDelivery/BT_DeliveryDrone.BT_DeliveryDrone"))))
    (:`then_1`
      (`/Engine/EditorBlueprintResources/ActorMacros.Switch Has Authority`
        (:`Remote`
          (`SceneComponent.SetVisibility` (`self.Billboard`) true false))))))

(event `self.ReceiveAnyDamage`
  (params (Damage :type "Float (single-precision)") (DamageType :type "DamageType Object Reference") (InstigatedBy :type "Controller Object Reference") (DamageCauser :type "Actor Object Reference"))
  (`/Game/Blueprints/BP_HealthComponent.Remote: Event any Damage` (`self.BP_HealthComponent`) Damage DamageType InstigatedBy DamageCauser))

(fn `UserConstructionScript`)