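; BP_CarrierDrone_Base is the base Blueprint for an AI carrier drone used in energy delivery.
; On BeginPlay, the server runs the BT_CarrierDrone behavior tree through the drone's AI controller.
; When destroyed, the authority asks its HomeCollector to spawn a replacement carrier, a respawn marked as testing only.
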(event `self.ReceiveDestroyed`
  (bind _homecollector (`self.HomeCollector`))
  ;[1 1 1] Respawn the Drone for testing purpose only
  (`/Engine/EditorBlueprintResources/ActorMacros.Switch Has Authority`
    (:`Authority`
      (`/Engine/EditorBlueprintResources/StandardMacros.IsValid` _homecollector
        (:`Is Valid`
          (`/Game/Blueprints/AI/EnergyDelivery/BP_EnergyCollector.SpawnCarrier` _homecollector))))))

(event `self.ReceiveBeginPlay`
  (`parent.ReceiveBeginPlay`)
  ;[1 1 1] Run behavior tree on server only
  (if (or (`KismetSystemLibrary.IsServer`) (`KismetSystemLibrary.IsDedicatedServer`))
    (`AIController.RunBehaviorTree` (`AIBlueprintHelperLibrary.GetAIController` self) "/Game/Blueprints/AI/EnergyDelivery/BT_CarrierDrone.BT_CarrierDrone")))

(fn `UserConstructionScript`)