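; Behavior tree task that finds the actor of a configurable class nearest to the controlled pawn and stores it on the Blackboard.
; On execute, it gets all actors of that class and linearly compares straight-line distances to keep the closest.
; It writes the result to the chosen key and succeeds, or writes an empty value to that key and fails when none are found.
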(event `self.ReceiveExecuteAI`
  (params (OwnerController :type "AIController Object Reference") (ControlledPawn :type "Pawn Object Reference"))
  (bind _returnvalue (`Actor.K2_GetActorLocation` ControlledPawn))
  (bind _outactors (`GameplayStatics.GetAllActorsOfClass` (`self.ActorToLookFor`)))
  (bind _output (`|GetArrayItem` _outactors))
  (`/Engine/EditorBlueprintResources/StandardMacros.IsValid` _output
    (:`Is Valid`
      (set `self.ClosestEnergyField` _output)
      (bind _returnvalue_2 (`KismetArrayLibrary.Array_Length` _outactors))
      (if (> _returnvalue_2 1)
        (for _index (range 1 _returnvalue_2)
          (bind _output_2 (`|GetArrayItem` _outactors _index))
          ;[1 1 1] Loop through each found actor, compare the distances, and if shorter: set as closest actor
          (if (< (`KismetMathLibrary.VSize` (- (`Actor.K2_GetActorLocation` _output_2) _returnvalue)) (`KismetMathLibrary.VSize` (- (`Actor.K2_GetActorLocation` (`self.ClosestEnergyField`)) _returnvalue)))
            (set `self.ClosestEnergyField` _output_2))))
      ;[1 1 1] Communicate the closest actor to the BlackBoard
      (`BTFunctionLibrary.SetBlackboardValueAsObject` (`self.BBKeyToStoreActorResult`) (`self.ClosestEnergyField`))
      (`self.FinishExecute` true))
    (:`Is Not Valid`
      ;[1 1 1] If there is no actor, abort the operation
      (`BTFunctionLibrary.SetBlackboardValueAsObject` (`self.BBKeyToStoreActorResult`))
      (`self.FinishExecute` false))))