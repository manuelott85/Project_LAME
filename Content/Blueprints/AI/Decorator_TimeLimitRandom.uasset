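; Behavior tree decorator that acts as a time limit with random variance, failing its condition once the time runs out.
; On execution start it records the time and rolls a symmetric random offset within RandomOffset.
; Each tick sets TimeIsOver when elapsed time exceeds TimeLimit plus that offset, and the condition check returns its inverse.
; The flag resets when execution finishes or the observer deactivates.
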(event `self.ReceiveExecutionStartAI`
  (params (OwnerController :type "AIController Object Reference") (ControlledPawn :type "Pawn Object Reference"))
  (bind _randomoffset (`self.RandomOffset`))
  (set `self.StartTime` (`GameplayStatics.GetTimeSeconds`))
  (set `self.CalculatedRandomOffset` (`KismetMathLibrary.RandomFloatInRange` (* _randomoffset -1.0) _randomoffset)))

(event `self.ReceiveTickAI`
  (params (OwnerController :type "AIController Object Reference") (ControlledPawn :type "Pawn Object Reference") (DeltaSeconds :type "Float (single-precision)"))
  (set `self.TimeIsOver` (> (`GameplayStatics.GetTimeSeconds`) (+ (`self.StartTime`) (`self.TimeLimit`) (`self.CalculatedRandomOffset`)))))

(event `self.ReceiveObserverDeactivatedAI`
  (params (OwnerController :type "AIController Object Reference") (ControlledPawn :type "Pawn Object Reference"))
  (set `self.TimeIsOver` false :!label _label))

(event `self.ReceiveExecutionFinishAI`
  (params (OwnerController :type "AIController Object Reference") (ControlledPawn :type "Pawn Object Reference") (NodeResult :type "EBTNodeResult Enum" :default "Succeeded"))
  (goto _label))

(fn `PerformConditionCheckAI`
  (params (OwnerController :type "AIController Object Reference") (ControlledPawn :type "Pawn Object Reference"))
  (returns (ReturnValue :type Boolean))
  (if (`self.TimeIsOver`)
    (return false)
    (else
      (return true))))