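; Base AI drone pawn with smoothed, pitch- and roll-clamped movement, blackboard-driven turning toward a TargetActor and an empty Fire function.
; Damage goes to a health component, shown on a health bar widget that faces the camera each tick.
; Spawning plays a sound, optionally randomizes yaw and adds a billboard when the local player controls a Defender.
; Destruction removes the billboard and, on authority, decrements the Defender's drone count except for carrier drones.
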(event `self.AddMovementInputCustom`
  (params (WorldDirection :type "Vector Structure") (ScaleValue :type "Float (single-precision)"))
  ;[1 1 1] Move the Pawn
  (`self.K2_SetActorRotation` (`KismetMathLibrary.RInterpTo` (`self.K2_GetActorRotation`) (`KismetMathLibrary.MakeRotator` (`KismetMathLibrary.FClamp` (.roll (`KismetMathLibrary.MakeRotFromX` WorldDirection)) -30.0 30.0) (`KismetMathLibrary.FClamp` (.pitch (`KismetMathLibrary.MakeRotFromX` WorldDirection)) -30.0 30.0) (.yaw (`KismetMathLibrary.MakeRotFromX` WorldDirection))) (`GameplayStatics.GetWorldDeltaSeconds`) 5.0))
  (`self.AddMovementInput` WorldDirection (* ScaleValue (`self.Bot Speed Scale`))))

(event `self.ReceiveTick`
  (params (DeltaSeconds :type "Float (single-precision)"))
  (bind _returnvalue (`GameplayStatics.GetPlayerCameraManager` 0))
  ;[1 1 1] Tick
  ;[1 1 1] Rotate Healthbar
  (`/Engine/EditorBlueprintResources/StandardMacros.IsValid` _returnvalue
    (:`Is Valid`
      (`SceneComponent.K2_SetWorldRotation` (`self.HealthWidget`) (`KismetMathLibrary.FindLookAtRotation` (`SceneComponent.K2_GetComponentLocation` (`self.HealthWidget`)) (`PlayerCameraManager.GetCameraLocation` _returnvalue)) false false)
      ;[1 1 1] Update Healthbar
      (bind _asw_healthbar (cast `/Game/Widget/W_Healthbar` (`WidgetComponent.GetUserWidgetObject` (`self.HealthWidget`))))
      (`TextBlock.SetText` (`/Game/Widget/W_Healthbar.Text_Healthpoints` _asw_healthbar) (`KismetTextLibrary.Conv_DoubleToText` (`/Game/Blueprints/Components/BP_HealthComponent.CurrentHealth` (`self.BP_HealthComponent`)) "HalfToEven")))))

(event `self.ReceiveBeginPlay`
  (bind (_returnvalue_roll _returnvalue_pitch) (`KismetMathLibrary.BreakRotator` (`self.K2_GetActorRotation`)))
  (bind _audio (`self.Audio`))
  ;[1 1 1] BeginPlay
  (`|ExecutionSequence`
    (:`then_0`
      ;[1 1 1] Create the billboard
      (bind _asbp_player_controller (cast `/Game/Blueprints/BP_PlayerController` (`GameplayStatics.GetPlayerController` 0)))
      (cast `/Game/Blueprints/BP_Defender_Base` (`Controller.K2_GetPawn` _asbp_player_controller))
      (bind _returnvalue (`|SpawnActorFromClass` "/Game/Blueprints/BP_BillboardAddition.BP_BillboardAddition_C" (`KismetMathLibrary.MakeTransform` (`self.K2_GetActorLocation` self)) "Undefined" "OverrideRootScale" null self (`self.BillboardSprite`) (`self.BillboardScale`) null))
      (set `self.BillboardReference` _returnvalue))
    (:`then_1`
      ;[1 1 1] Randomize view vector at startup
      (if (`self.RandomizeRotationAtSpawn`)
        (`self.K2_SetActorRotation` (`KismetMathLibrary.MakeRotator` _returnvalue_roll _returnvalue_pitch (`KismetMathLibrary.RandomFloatInRange` 0.0 360.0)))))
    (:`then_2`
      ;[1 1 1] Play Sound
      (`AudioComponent.SetSound` _audio (`self.Drone spawned`))
      (`AudioComponent.Play` _audio 0.0))))

(event `self.ReceiveAnyDamage`
  (params (Damage :type "Float (single-precision)") (DamageType :type "DamageType Object Reference") (InstigatedBy :type "Controller Object Reference") (DamageCauser :type "Actor Object Reference"))
  ;[1 1 1] Handle Damage
  (`/Game/Blueprints/Components/BP_HealthComponent.Remote: Event any Damage` (`self.BP_HealthComponent`) Damage DamageType InstigatedBy DamageCauser))

(event `self.ReceiveDestroyed`
  (bind _billboardreference (`self.BillboardReference`))
  ;[1 1 1] Destroyed
  (`|ExecutionSequence`
    (:`then_0`
      (`/Engine/EditorBlueprintResources/ActorMacros.Switch Has Authority`
        (:`Authority`
          ;[1 1 1] Exclude carrier from the math
          (cast `/Game/Blueprints/AI/EnergyDelivery/BP_CarrierDrone_Base` self
            (:`CastFailed`
              ;[1 1 1] Reduce current number of drones for the villain player
              (bind _outactors (`GameplayStatics.GetAllActorsOfClass` "/Game/Blueprints/BP_Defender_Base.BP_Defender_Base_C"))
              (if (> (`KismetArrayLibrary.Array_Length` _outactors) 0)
                (`/Game/Blueprints/Components/BP_SpawningComponent.AlterCurNumDrones` (`/Game/Blueprints/BP_Defender_Base.BP_SpawningComponent` (`|GetArrayItem` _outactors)) -1)))))))
    (:`then_1`
      ;[1 1 1] Remove the billboard
      (`/Engine/EditorBlueprintResources/StandardMacros.IsValid` _billboardreference
        (:`Is Valid`
          (`self.K2_DestroyActor` _billboardreference))))))

(fn `Fire`)

(fn `RotateTowardsActor`
  (locals (TargetRotation :type "Rotator Structure") (StartRotation :type "Rotator Structure"))
  (`|ExecutionSequence`
    (:`then_0`
      ;[1 1 1] Get BB TargetActor as Actor
      (bind _asactor (cast `Actor` (`BlackboardComponent.GetValueAsObject` (`AIController.Blackboard` (`AIBlueprintHelperLibrary.GetAIController` self)) "TargetActor")))
      (set `self.TargetActor` _asactor))
    (:`then_1`
      ;[1 1 1] Get a rotation vector towards the target
      (`/Engine/EditorBlueprintResources/StandardMacros.IsValid` (`self.TargetActor`)
        (:`Is Valid`
          (set `local.TargetRotation` (`KismetMathLibrary.FindLookAtRotation` (`self.K2_GetActorLocation`) (`self.K2_GetActorLocation` (`self.TargetActor`))))
          (set `local.StartRotation` (`self.K2_GetActorRotation`))
          ;[1 1 1] Rotate towards the target
          (`self.K2_SetActorRotation` (`KismetMathLibrary.RInterpTo` (`local.StartRotation`) (`local.TargetRotation`) (`GameplayStatics.GetWorldDeltaSeconds`) (`self.TurnSpeed`))))))))

(fn `UserConstructionScript`)