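; Behavior tree task that makes the controlled AI pawn fire its weapon.
; A cast chain picks the firing method: BP_BasicAI and BP_AICharacter_Team2 fire a short timed burst through StartFire and StopFire, while BP_SentineDrone_Base calls a single Fire.
; Each supported pawn finishes the task successfully, and any other pawn type calls FinishAbort instead of reporting failure.
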(event `self.ReceiveExecuteAI`
  (params (OwnerController :type "AIController Object Reference") (ControlledPawn :type "Pawn Object Reference"))
  (bind _asbp_basic_ai (cast `/Game/Blueprints/AI/BP_BasicAI` ControlledPawn)
    (:`then`
      (`/Game/Blueprints/AI/BP_BasicAI.StartFire` _asbp_basic_ai)
      (`KismetSystemLibrary.Delay` 0.4)
      (`/Game/Blueprints/AI/BP_BasicAI.StopFire` _asbp_basic_ai)
      (`self.FinishExecute` true))
    (:`CastFailed`
      (bind _asbp_aicharacter_team_2 (cast `/Game/Blueprints/AI/BP_AICharacter_Team2` ControlledPawn)
        (:`then`
          (`/Game/Blueprints/AI/BP_AICharacter_Team2.StartFire` _asbp_aicharacter_team_2)
          (`KismetSystemLibrary.Delay` 0.4)
          (`/Game/Blueprints/AI/BP_AICharacter_Team2.StopFire` _asbp_aicharacter_team_2)
          (`self.FinishExecute` true))
        (:`CastFailed`
          (bind _asbp_sentine_drone_base (cast `/Game/Blueprints/AI/SentinelDrone/BP_SentineDrone_Base` ControlledPawn)
            (:`then`
              (`/Game/Blueprints/AI/SentinelDrone/BP_SentineDrone_Base.Fire` _asbp_sentine_drone_base)
              (`self.FinishExecute` true))
            (:`CastFailed`
              (`self.FinishAbort`))))))))