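; Behavior tree task that prints the distance between the AI-controlled pawn and its target actor, apparently for debugging.
; On AI execute, it reads the TargetActor blackboard value by hardcoded key name, casts it to Actor and prints the distance between the two locations in green.
; A failed cast prints nothing, and neither path calls Finish Execute, so the task never reports completion.
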(event `self.ReceiveExecuteAI`
  (params (OwnerController :type "AIController Object Reference") (ControlledPawn :type "Pawn Object Reference"))
  (bind _asactor (cast `Actor` (`BlackboardComponent.GetValueAsObject` (`AIBlueprintHelperLibrary.GetBlackboard` ControlledPawn) "TargetActor")))
  (`KismetSystemLibrary.PrintString` (`KismetStringLibrary.Concat_StrStr` "distance: " (`KismetStringLibrary.Conv_DoubleToString` (`KismetMathLibrary.VSize` (- (`Actor.K2_GetActorLocation` _asactor) (`Actor.K2_GetActorLocation` ControlledPawn))))) true true (struct :`R` 0.035046 :`G` 1.0 :`A` 1.0)))