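; Base AI turret drone that runs its behavior tree on the server, plays a spawn sound and shoots at attackers.
; Fire reads TargetActor from the Blackboard, checks that the drone faces it, then line-traces on the Camera channel for an attacker to judge cover.
; When the cover flag is clear, it spawns a damage-carrying projectile at the muzzle, aimed at an attacker's first-person camera with random spread, and plays a shot sound.
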(event `self.ReceiveBeginPlay`
  (bind _audio (`self.Audio`))
  (`parent.ReceiveBeginPlay`)
  (`|ExecutionSequence`
    (:`then_0`
      ;[1 1 1] Run behavior tree on server only
      (`/Engine/EditorBlueprintResources/ActorMacros.Switch Has Authority`
        (:`Authority`
          (`AIController.RunBehaviorTree` (`AIBlueprintHelperLibrary.GetAIController` self) "/Game/Blueprints/AI/Turret/BT_Turret.BT_Turret"))))
    (:`then_1`
      (`AudioComponent.SetSound` _audio (`self.Drone spawned`))
      (`AudioComponent.Play` _audio 0.0))))

(event `self.Fire`
  (bind _returnvalue (`KismetMathLibrary.RandomFloatInRange` -5.0 5.0))
  (bind _targetactor (`self.TargetActor`))
  (bind _returnvalue_location (`KismetMathLibrary.BreakTransform` (`SceneComponent.K2_GetComponentToWorld` (`self.MuzzleToSpawnTheProjectile`))))
  (`parent.Fire`)
  (`|ExecutionSequence`
    (:`then_0`
      ;[1 1 1] Get BB TargetActor as Actor
      (bind _asactor (cast `Actor` (`BlackboardComponent.GetValueAsObject` (`AIController.Blackboard` (`AIBlueprintHelperLibrary.GetAIController` self)) "TargetActor")))
      (set `self.TargetActor` _asactor))
    (:`then_1`
      ;[1 1 1] Only shoot if the drone looks at its target
      (`/Engine/EditorBlueprintResources/StandardMacros.IsValid` (`self.TargetActor`)
        (:`Is Valid`
          (set `self.LooksAtTarget` (== (`self.K2_GetActorRotation`) (`KismetMathLibrary.FindLookAtRotation` (`self.K2_GetActorLocation`) (`self.K2_GetActorLocation` (`self.TargetActor`))) :`ErrorTolerance` 2.0)))))
    (:`then_2`
      ;[1 1 1] Check if the target is actualy visible
      (if (`self.LooksAtTarget`)
        (bind _outhit (`KismetSystemLibrary.LineTraceSingle` (`SceneComponent.K2_GetComponentLocation` (`self.Capsule`)) (* (- (`self.K2_GetActorLocation` (`self.TargetActor`)) (`SceneComponent.K2_GetComponentLocation` (`self.Capsule`))) 2500.0) "TraceTypeQuery2"))
        (cast `/Game/Blueprints/BP_Attacker_Base` (`.HitActor` (`GameplayStatics.BreakHitResult` _outhit))
          (:`then`
            (set `self.TargetIsNotInCover` true))
          (:`CastFailed`
            (set `self.TargetIsNotInCover` false)))))
    (:`then_3`
      ;[1 1 1] Spawn the Projectile
      (if (`self.TargetIsNotInCover`)
        (bind _asbp_attacker_base (cast `/Game/Blueprints/BP_Attacker_Base` _targetactor)
          (:`then`
            (set `self.TargetActorLocation` (- (`SceneComponent.K2_GetComponentLocation` (`/Game/Blueprints/BP_Attacker_Base.FirstPersonCamera` _asbp_attacker_base)) (`KismetMathLibrary.MakeVector` _returnvalue _returnvalue _returnvalue))))
          (:`CastFailed`
            (set `self.TargetActorLocation` (`self.K2_GetActorLocation` _targetactor))))
        (`|SpawnActorFromClass` "/Game/Blueprints/Projectiles/BP_AIProjectile_Base.BP_AIProjectile_Base_C" (`KismetMathLibrary.MakeTransform` _returnvalue_location (`KismetMathLibrary.FindLookAtRotation` _returnvalue_location (`self.TargetActorLocation`)) (0.1 0.1 0.1)) "AlwaysSpawn" "OverrideRootScale" null (`self.Damage`) null)
        ;[1 1 1] Play ShootSound
        (`GameplayStatics.PlaySoundAtLocation` (`self.ShootSound`) (`self.K2_GetActorLocation`) (struct) 1.0 1.0 0.0 null null null)))))

(fn `UserConstructionScript`
  (`parent.UserConstructionScript`))