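; Base sentinel drone AI that turns toward and fires on a blackboard target, forwarding damage to its health component.
; The server runs its behavior tree and randomizes starting yaw, while remote clients show a billboard meant for the Villain player.
; RotateTowardsActor interpolates toward the target; Fire checks aim and line-traces for an attacker, setting FollowTarget when none is hit.
; Shots are only debug lines, and the firing sound is unwired.
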(event `self.ReceiveAnyDamage`
  (params (Damage :type "Float (single-precision)") (DamageType :type "DamageType Object Reference") (InstigatedBy :type "Controller Object Reference") (DamageCauser :type "Actor Object Reference"))
  ;[1 1 1] Process incomming Damage
  (`/Game/Blueprints/Components/BP_HealthComponent.Remote: Event any Damage` (`self.BP_HealthComponent`) Damage DamageType InstigatedBy DamageCauser))

(event `self.ReceiveBeginPlay`
  (bind (_returnvalue_roll _returnvalue_pitch) (`KismetMathLibrary.BreakRotator` (`self.K2_GetActorRotation`)))
  (`/Engine/EditorBlueprintResources/ActorMacros.Switch Has Authority`
    (:`Authority`
      (`|ExecutionSequence`
        (:`then_0`
          ;[1 1 1] Run behavior tree on server only
          (`AIController.RunBehaviorTree` (`AIBlueprintHelperLibrary.GetAIController` self) "/Game/Blueprints/AI/SentinelDrone/BT_SentinelDrone.BT_SentinelDrone"))
        (:`then_1`
          ;[1 1 1] Randomize view vector at startup
          (`self.K2_SetActorRotation` (`KismetMathLibrary.MakeRotator` _returnvalue_roll _returnvalue_pitch (`KismetMathLibrary.RandomFloatInRange` 0.0 360.0))))))
    (:`Remote`
      ;[1 1 1] Show Billboard to Villainplayer only
      (`SceneComponent.SetVisibility` (`self.Billboard`) true false))))

(fn `Fire`
  (locals (TargetActor :type "Actor Object Reference"))
  (`|ExecutionSequence`
    (:`then_0`
      ;[1 1 1] Get BB TargetActor as Actor
      (bind _asactor (cast `Actor` (`BlackboardComponent.GetValueAsObject` (`AIController.Blackboard` (`AIBlueprintHelperLibrary.GetAIController` self)) "TargetActor")))
      (set `local.TargetActor` _asactor))
    (:`then_1`
      ;[1 1 1] Only shoot if the drone looks at its target
      (`/Engine/EditorBlueprintResources/StandardMacros.IsValid` (`local.TargetActor`)
        (:`Is Valid`
          (if (== (`self.K2_GetActorRotation`) (`KismetMathLibrary.FindLookAtRotation` (`self.K2_GetActorLocation`) (`self.K2_GetActorLocation` (`local.TargetActor`))) :`ErrorTolerance` 2.0)
            ;[1 1 1] Check if the target is actualy visible
            (bind _outhit (`KismetSystemLibrary.LineTraceSingle` (`SceneComponent.K2_GetComponentLocation` (`self.CapsuleComponent`)) (* (- (`self.K2_GetActorLocation` (`local.TargetActor`)) (`SceneComponent.K2_GetComponentLocation` (`self.CapsuleComponent`))) 2500.0) "TraceTypeQuery2"))
            (cast `/Game/Blueprints/BP_Attacker_Base` (`.HitActor` (`GameplayStatics.BreakHitResult` _outhit))
              (:`then`
                ;[1 1 1] Debug Shoot Visuals
                (`KismetSystemLibrary.DrawDebugLine` (`SceneComponent.K2_GetComponentLocation` (`self.Mesh`)) (`self.K2_GetActorLocation` (`local.TargetActor`)) (`self.ShootColor`) 0.2 10.0))
              (:`CastFailed`
                ;[1 1 1] Ask to follow the target
                (`BlackboardComponent.SetValueAsBool` (`AIBlueprintHelperLibrary.GetBlackboard` self) "FollowTarget" true)))))))))

(fn `RotateTowardsActor`
  (locals (TargetActor :type "Actor Object Reference") (TargetRotation :type "Rotator Structure") (StartRotation :type "Rotator Structure"))
  (`|ExecutionSequence`
    (:`then_0`
      ;[1 1 1] Get BB TargetActor as Actor
      (bind _asactor (cast `Actor` (`BlackboardComponent.GetValueAsObject` (`AIController.Blackboard` (`AIBlueprintHelperLibrary.GetAIController` self)) "TargetActor")))
      (set `local.TargetActor` _asactor))
    (:`then_1`
      ;[1 1 1] Get a rotation vector towards the target
      (`/Engine/EditorBlueprintResources/StandardMacros.IsValid` (`local.TargetActor`)
        (:`Is Valid`
          (set `local.TargetRotation` (`KismetMathLibrary.FindLookAtRotation` (`self.K2_GetActorLocation`) (`self.K2_GetActorLocation` (`local.TargetActor`))))
          (set `local.StartRotation` (`self.K2_GetActorRotation`))
          ;[1 1 1] Rotate towards the target
          (`self.K2_SetActorRotation` (`KismetMathLibrary.RInterpTo` (`local.StartRotation`) (`local.TargetRotation`) (`GameplayStatics.GetWorldDeltaSeconds`) (`self.TurnSpeed`))))))))

(fn `UserConstructionScript`)