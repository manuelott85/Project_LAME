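; AI drone character for Team 2 that runs the BT_SentinelDrone behavior tree on the server and spawns with a random yaw.
; Each tick, a dynamic material shifts its sphere from yellow toward red while it lingers within a minimum travel distance, and toward green when it moves beyond it.
; StartFire only draws a debug line to the blackboard TargetActor and plays a sound; StopFire is empty.
; Any damage destroys the drone.
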(event `self.ReceiveBeginPlay`
  (bind (_returnvalue_roll _returnvalue_pitch) (`KismetMathLibrary.BreakRotator` (`self.K2_GetActorRotation`)))
  (bind _sphere (`self.Sphere`))
  (`|ExecutionSequence`
    (:`then_0`
      ;[1 1 1] Run behavior tree on server only
      (`/Engine/EditorBlueprintResources/ActorMacros.Switch Has Authority`
        (:`Authority`
          (`AIController.RunBehaviorTree` (`AIBlueprintHelperLibrary.GetAIController` self) "/Game/Blueprints/AI/SentinelDrone/BT_SentinelDrone.BT_SentinelDrone"))))
    (:`then_1`
      ;[1 1 1] Randomize view vector at startup
      (`self.K2_SetActorRotation` (`KismetMathLibrary.MakeRotator` _returnvalue_roll _returnvalue_pitch (`KismetMathLibrary.RandomFloatInRange` 0.0 360.0))))
    (:`then_2`
      ;[1 1 1] Instanciate Material and initialize
      (set `self.location` (`self.K2_GetActorLocation`))
      (bind _returnvalue (`PrimitiveComponent.CreateDynamicMaterialInstance` _sphere 0 (`PrimitiveComponent.GetMaterial` _sphere 0) "None"))
      (bind _output_get (set `self.DynMat` _returnvalue))
      (`MaterialInstanceDynamic.SetVectorParameterValue` _output_get "BodyColor" (make `LinearColor` 1.0 1.0 0.0 1.0)))))

(event `self.ReceiveTick`
  (params (DeltaSeconds :type "Float (single-precision)"))
  (bind _dynmat (`self.DynMat`))
  (bind _dynmat_2 (`self.DynMat`))
  (bind _increasevalue (`self.IncreaseValue`))
  (bind _decreasevalue (`self.DecreaseValue`))
  (if (< (`KismetMathLibrary.VSize` (- (`self.K2_GetActorLocation`) (`self.location`))) (`self.MinTravelDist`))
    ;[1 1 1] Decrease Color towards red
    (bind _returnvalue (`MaterialInstanceDynamic.K2_GetVectorParameterValue` _dynmat "BodyColor"))
    (if (< (break `LinearColor` _returnvalue) 1.0)
      (bind _returnvalue_2 (`KismetMathLibrary.FClamp` (+ (break `LinearColor` _returnvalue) _decreasevalue)))
      (`MaterialInstanceDynamic.SetVectorParameterValue` _dynmat "BodyColor" (make `LinearColor` _returnvalue_2 1.0 0.0 1.0))
      (set `self.currentColor` (make `LinearColor` _returnvalue_2 1.0 0.0 1.0))
      (else
        (bind _returnvalue_3 (`KismetMathLibrary.FClamp` (- (`.G` (break `LinearColor` _returnvalue)) _decreasevalue)))
        (`MaterialInstanceDynamic.SetVectorParameterValue` _dynmat "BodyColor" (make `LinearColor` 1.0 _returnvalue_3 0.0 1.0))
        (set `self.currentColor` (make `LinearColor` 1.0 _returnvalue_3 0.0 1.0))))
    (else
      ;[1 1 1] Increas color towards green
      (set `self.location` (`self.K2_GetActorLocation`))
      (bind _returnvalue_4 (`MaterialInstanceDynamic.K2_GetVectorParameterValue` _dynmat_2 "BodyColor"))
      (if (< (`.G` (break `LinearColor` _returnvalue_4)) 1.0)
        (bind _returnvalue_5 (`KismetMathLibrary.FClamp` (+ (`.G` (break `LinearColor` _returnvalue_4)) _increasevalue)))
        (`MaterialInstanceDynamic.SetVectorParameterValue` _dynmat_2 "BodyColor" (make `LinearColor` 1.0 _returnvalue_5 0.0 1.0))
        (set `self.currentColor` (make `LinearColor` 1.0 _returnvalue_5 0.0 1.0))
        (else
          (bind _returnvalue_6 (`KismetMathLibrary.FClamp` (- (break `LinearColor` _returnvalue_4) _increasevalue)))
          (`MaterialInstanceDynamic.SetVectorParameterValue` _dynmat_2 "BodyColor" (make `LinearColor` _returnvalue_6 1.0 0.0 1.0))
          (set `self.currentColor` (make `LinearColor` _returnvalue_6 1.0 0.0 1.0)))))))

(event `self.ReceiveAnyDamage`
  (params (Damage :type "Float (single-precision)") (DamageType :type "DamageType Object Reference") (InstigatedBy :type "Controller Object Reference") (DamageCauser :type "Actor Object Reference"))
  ;[1 1 1] Example Damage
  (`KismetSystemLibrary.PrintString` "Damage Recieved" true true (struct :`R` 1.0 :`G` 0.062383 :`A` 1.0))
  (`self.K2_DestroyActor`))

(fn `StartFire`
  (`KismetSystemLibrary.PrintString` "I start to fire")
  (bind _asactor (cast `Actor` (`BlackboardComponent.GetValueAsObject` (`AIController.Blackboard` (`AIBlueprintHelperLibrary.GetAIController` self)) "TargetActor")))
  (`KismetSystemLibrary.DrawDebugLine` (`SceneComponent.K2_GetComponentLocation` (`self.Mesh`)) (`self.K2_GetActorLocation` _asactor) (`self.ShootColor`) 0.2 10.0)
  (`GameplayStatics.PlaySoundAtLocation` "/Game/_FirstPerson/Audio/FirstPersonTemplateWeaponFire02.FirstPersonTemplateWeaponFire02" (`self.K2_GetActorLocation`) (struct) 1.0 1.0 0.0 null null null) ; Play firing sound
)

(fn `StopFire`)

(fn `UserConstructionScript`)