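; Base melee drone AI that acts as a suicide bomber, exploding on its target.
; On BeginPlay the server runs BT_MeeleDrone and writes AttackRange to its Blackboard, and a spawn sound plays.
; Fire traces toward the Blackboard TargetActor, and on hitting an attacker deals falloff radial damage, draws a debug sphere and destroys the drone.
; PlayAudio maps state names to drone sounds.
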(event `self.ReceiveBeginPlay`
  (bind _audio (`self.Audio`))
  (`parent.ReceiveBeginPlay`)
  (`|ExecutionSequence`
    (:`then_0`
      ;[1 1 1] Run behavior tree on server only
      (`/Engine/EditorBlueprintResources/ActorMacros.Switch Has Authority`
        (:`Authority`
          (`AIController.RunBehaviorTree` (`AIBlueprintHelperLibrary.GetAIController` self) "/Game/Blueprints/AI/MeeleDrone/BT_MeeleDrone.BT_MeeleDrone")
          ;[1 1 1] Make AttackRange available in the Blackboard
          (`BlackboardComponent.SetValueAsFloat` (`AIBlueprintHelperLibrary.GetBlackboard` self) "AttackRange" (`self.AttackRange`)))))
    (:`then_1`
      (`AudioComponent.SetSound` _audio (`self.Drone spawned`))
      (`AudioComponent.Play` _audio 0.0))))

(event `self.Fire`
  (bind _returnvalue (`self.K2_GetActorLocation`))
  (bind _damagemaxradius (`self.DamageMaxRadius`))
  (`parent.Fire`)
  (`|ExecutionSequence`
    (:`then_0`
      ;[1 1 1] Get BB TargetActor as Actor
      (bind _asactor (cast `Actor` (`BlackboardComponent.GetValueAsObject` (`AIController.Blackboard` (`AIBlueprintHelperLibrary.GetAIController` self)) "TargetActor")))
      (set `self.TargetActor_0` _asactor))
    (:`then_1`
      ;[1 1 1] Check if the target is actualy visible
      (bind _outhit (`KismetSystemLibrary.LineTraceSingle` (`SceneComponent.K2_GetComponentLocation` (`self.Capsule`)) (* (- (`self.K2_GetActorLocation` (`self.TargetActor_0`)) (`SceneComponent.K2_GetComponentLocation` (`self.Capsule`))) 2500.0) "TraceTypeQuery2"))
      (cast `/Game/Blueprints/BP_Attacker_Base` (`.HitActor` (`GameplayStatics.BreakHitResult` _outhit))
        (:`then`
          (set `self.TargetIsNotInCover` true))
        (:`CastFailed`
          (set `self.TargetIsNotInCover` false))))
    (:`then_2`
      (if (`self.TargetIsNotInCover`)
        (cast `/Game/Blueprints/BP_Attacker_Base` (`self.TargetActor_0`))
        (`GameplayStatics.ApplyRadialDamageWithFalloff` :`BaseDamage` (`self.Damage`) :`MinimumDamage` (`self.MinDamage`) :`Origin` _returnvalue :`DamageInnerRadius` (`self.RadiusFullDamage`) :`DamageOuterRadius` _damagemaxradius :`DamageFalloff` (`self.DamageFalloff`) :`DamageCauser` self :`InstigatedByController` (`self.GetController` self))
        (`KismetSystemLibrary.DrawDebugSphere` _returnvalue _damagemaxradius 12 (struct :`R` 1.0 :`G` 0.006907 :`A` 1.0) 30.0 1.0)
        ;[1 1 1] Play ShootSound
        (`GameplayStatics.PlaySoundAtLocation` (`self.ShootSound`) (`self.K2_GetActorLocation`) (struct) 1.0 1.0 0.0 null null null)
        (`self.K2_DestroyActor`)))))

(fn `PlayAudio`
  (params (FileName :type "/Game/Blueprints/AI/Enum_Sound Enum" :default "NewEnumerator0"))
  (bind _audio (`self.Audio`))
  (`|ExecutionSequence`
    (:`then_0`
      (switch `/Game/Blueprints/AI/Enum_Sound` FileName
        (:`NewEnumerator0`
          (set `self.SoundToPlay` (`self.Engage Target`)))
        (:`NewEnumerator1`
          (set `self.SoundToPlay` (`self.Searching for Target`)))
        (:`NewEnumerator2`
          (set `self.SoundToPlay` (`self.GunSound`)))
        (:`NewEnumerator3`
          (set `self.SoundToPlay` (`self.Drone spawned`)))
        (:`NewEnumerator4`
          (set `self.SoundToPlay` (`self.Target Spotted`)))
        (:`NewEnumerator5`
          (set `self.SoundToPlay` (`self.Target Lost`)))
        (:`NewEnumerator6`
          (set `self.SoundToPlay` (`self.Target Neutralized`)))))
    (:`then_1`
      (`AudioComponent.SetSound` _audio (`self.SoundToPlay`))
      (`AudioComponent.Play` _audio 0.0))))

(fn `UserConstructionScript`)