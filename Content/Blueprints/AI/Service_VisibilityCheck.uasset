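; Behavior Tree service that checks whether the controlled pawn has line of sight to an actor stored in the Blackboard.
; Each AI tick runs a Camera-channel line trace from the pawn, ignoring itself, with the end set to the pawn-to-target vector scaled up, without adding the start location.
; It writes true to a Blackboard bool if the target is hit first, otherwise false, including when the target is invalid.
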(event `self.ReceiveTickAI`
  (params (OwnerController :type "AIController Object Reference") (ControlledPawn :type "Pawn Object Reference") (DeltaSeconds :type "Float (single-precision)"))
  (bind _returnvalue (`Actor.K2_GetActorLocation` ControlledPawn))
  (bind _booltostoreresult (`self.BoolToStoreResult`))
  (bind _returnvalue_2 (`BTFunctionLibrary.GetBlackboardValueAsActor` (`self.ActorToLookFor`)))
  (`/Engine/EditorBlueprintResources/StandardMacros.IsValid` _returnvalue_2
    (:`Is Valid`
      ;[1 1 1] Check if the target is actualy visible
      (bind _outhit (`KismetSystemLibrary.LineTraceSingle` _returnvalue (* (- (`Actor.K2_GetActorLocation` _returnvalue_2) _returnvalue) 2500.0) "TraceTypeQuery2" false (`|MakeArray` ControlledPawn :!type "Actor Object Reference") "None" true (struct :`R` 1.0 :`G` 0.763045 :`A` 1.0)))
      (if (== (`BTFunctionLibrary.GetBlackboardValueAsActor` (`self.ActorToLookFor`)) (`.HitActor` (`GameplayStatics.BreakHitResult` _outhit)))
        (`BTFunctionLibrary.SetBlackboardValueAsBool` _booltostoreresult true)
        (else
          (`BTFunctionLibrary.SetBlackboardValueAsBool` _booltostoreresult))))
    (:`Is Not Valid`
      (`BTFunctionLibrary.SetBlackboardValueAsBool` (`self.BoolToStoreResult`)))))