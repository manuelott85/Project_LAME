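; Behavior tree task that makes a BP_Drone_Base pawn look around by sweeping its yaw.
; On execute it sets arc limits around the starting yaw, failing if the pawn is not a drone.
; Each tick advances an alpha by TurnSpeed and eases rotation between the limits.
; When alpha wraps, both limits are negated to mirror the sweep, and the task never finishes successfully itself.
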(event `self.ReceiveExecuteAI`
  (params (OwnerController :type "AIController Object Reference") (ControlledPawn :type "Pawn Object Reference"))
  (bind _asbp_drone_base (cast `/Game/Blueprints/AI/BP_Drone_Base` ControlledPawn)
    (:`then`
      (bind _output_get (set `self.DroneActor` _asbp_drone_base))
      (set `self.StartRotation` (`Actor.K2_GetActorRotation` _output_get))
      (set `self.MinTargetRotation` (`KismetMathLibrary.MakeRotator` 0.0 0.0 (+ (.yaw (`self.StartRotation`)) (`self.HalfArcFromCenter`))))
      (bind _output_get_2 (set `self.MaxTargetRotation` (`KismetMathLibrary.MakeRotator` 0.0 0.0 (- (.yaw (`self.StartRotation`)) (`self.HalfArcFromCenter`)))))
      (set `self.CurrentTargetRotation` _output_get_2))
    (:`CastFailed`
      (`self.FinishExecute` false))))

(event `self.ReceiveTickAI`
  (params (OwnerController :type "AIController Object Reference") (ControlledPawn :type "Pawn Object Reference") (DeltaSeconds :type "Float (single-precision)"))
  (bind _returnvalue (+ (`self.EaseAlpha`) (* (`GameplayStatics.GetWorldDeltaSeconds`) (/ (`/Game/Blueprints/AI/BP_Drone_Base.TurnSpeed` (`self.DroneActor`)) 4.0))))
  ;[1 1 1] ensure that alpha stays between 0 and 1
  (if (> _returnvalue 1.0)
    (set `self.EaseAlpha` 0.0)
    ;[1 1 1] Mirror movement
    (set `self.MinTargetRotation` (* (`self.MinTargetRotation`) -1))
    (set `self.MaxTargetRotation` (* (`self.MaxTargetRotation`) -1))
    (else
      (set `self.EaseAlpha` _returnvalue)))
  ;[1 1 1] Apply Hover
  (`Actor.K2_SetActorRotation` (`self.DroneActor`) (`|EaseFunction` "EaseInOut" _returnvalue (`self.MinTargetRotation`) (`self.MaxTargetRotation`) false 1.65) false))