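; Behavior tree task that replaces a blackboard vector with a valid location in the DoN Navigation world.
; It asks the DoN navigation manager for a random navigable point within a short radius of that vector, using the controlled pawn as navigation actor.
; A found point overwrites the same key and the task succeeds; otherwise it fails.
; The random query is evaluated separately for the check and the write.
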(event `self.ReceiveExecuteAI`
  (params (OwnerController :type "AIController Object Reference") (ControlledPawn :type "Pawn Object Reference"))
  (bind (_bfoundvalidresult _returnvalue) (`DonNavigationManager.FindRandomPointAroundOriginInNavWorld` (`DonNavigationHelper.DonNavigationManager`) ControlledPawn (`BTFunctionLibrary.GetBlackboardValueAsVector` (`self.LocationToConvert`)) 40.0 -1.0 15.0 5))
  (if _bfoundvalidresult
    (`BTFunctionLibrary.SetBlackboardValueAsVector` (`self.LocationToConvert`) _returnvalue)
    (`self.FinishExecute` true)
    (else
      (`self.FinishExecute` false))))