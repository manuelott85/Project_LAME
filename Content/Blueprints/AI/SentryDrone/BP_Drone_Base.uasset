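; Base Blueprint for an AI sentry drone pawn, handling movement, turning and damage hand-off.
; Custom movement input eases rotation toward the travel direction with clamped pitch and roll, then applies speed-scaled movement.
; RotateTowardsActor reads TargetActor from the AI controller's Blackboard and interpolates toward it at TurnSpeed.
; BeginPlay shows a billboard and randomizes starting yaw, while damage is forwarded to BPHealthComponent.
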(event `self.AddMovementInputCustom`
  (params (WorldDirection :type "Vector Structure") (ScaleValue :type "Float (single-precision)"))
  ;[1 1 1] Move the Pawn
  (`self.K2_SetActorRotation` (`KismetMathLibrary.RInterpTo` (`self.K2_GetActorRotation`) (`KismetMathLibrary.MakeRotator` (`KismetMathLibrary.FClamp` (.roll (`KismetMathLibrary.MakeRotFromX` WorldDirection)) -30.0 30.0) (`KismetMathLibrary.FClamp` (.pitch (`KismetMathLibrary.MakeRotFromX` WorldDirection)) -30.0 30.0) (.yaw (`KismetMathLibrary.MakeRotFromX` WorldDirection))) (`GameplayStatics.GetWorldDeltaSeconds`) 5.0))
  (`self.AddMovementInput` WorldDirection (* ScaleValue (`self.Bot Speed Scale`))))

(event `self.ReceiveBeginPlay`
  (bind (_returnvalue_roll _returnvalue_pitch) (`KismetMathLibrary.BreakRotator` (`self.K2_GetActorRotation`)))
  (`|ExecutionSequence`
    (:`then_0`
      ;[1 1 1] Show Billboard to Villainplayer only
      (`/Engine/EditorBlueprintResources/ActorMacros.Switch Has Authority`
        (:`Authority`
          _)
        (:`Remote`
          _))
      (`SceneComponent.SetVisibility` (`self.Billboard`) true false))
    (:`then_1`
      ;[1 1 1] Randomize view vector at startup
      (`self.K2_SetActorRotation` (`KismetMathLibrary.MakeRotator` _returnvalue_roll _returnvalue_pitch (`KismetMathLibrary.RandomFloatInRange` 0.0 360.0))))))

(event `self.ReceiveAnyDamage`
  (params (Damage :type "Float (single-precision)") (DamageType :type "DamageType Object Reference") (InstigatedBy :type "Controller Object Reference") (DamageCauser :type "Actor Object Reference"))
  ;[1 1 1] Handle Damage
  (`/Game/Blueprints/BP_HealthComponent.Remote: Event any Damage` (`self.BP_HealthComponent`) Damage DamageType InstigatedBy DamageCauser))

(fn `RotateTowardsActor`
  (locals (TargetActor :type "Actor Object Reference") (TargetRotation :type "Rotator Structure") (StartRotation :type "Rotator Structure"))
  (`|ExecutionSequence`
    (:`then_0`
      ;[1 1 1] Get BB TargetActor as Actor
      (bind _asactor (cast `Actor` (`BlackboardComponent.GetValueAsObject` (`AIController.Blackboard` (`AIBlueprintHelperLibrary.GetAIController` self)) "TargetActor")))
      (set `local.TargetActor` _asactor))
    (:`then_1`
      ;[1 1 1] Get a rotation vector towards the target
      (`/Engine/EditorBlueprintResources/StandardMacros.IsValid` (`local.TargetActor`)
        (:`Is Valid`
          (set `local.TargetRotation` (`KismetMathLibrary.FindLookAtRotation` (`self.K2_GetActorLocation`) (`self.K2_GetActorLocation` (`local.TargetActor`))))
          (set `local.StartRotation` (`self.K2_GetActorRotation`))
          ;[1 1 1] Rotate towards the target
          (`self.K2_SetActorRotation` (`KismetMathLibrary.RInterpTo` (`local.StartRotation`) (`local.TargetRotation`) (`GameplayStatics.GetWorldDeltaSeconds`) (`self.TurnSpeed`))))))))

(fn `UserConstructionScript`)