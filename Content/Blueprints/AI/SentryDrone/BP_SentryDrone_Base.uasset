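; Base sentry drone AI for the defender side that shoots or blasts attackers.
; On the server it runs BT_SentryDrone, feeds the Blackboard combat values and a DonNavigation-validated investigate location, and scales damage and fire rate from the defender's offense upgrade.
; Fire checks facing and cover by trace, then spawns a projectile at the attacker's head with random spread.
; Melee applies radial falloff damage, with sounds and blast effects sent through Multi events.
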(event `Server_UpdateDamageValue`
  ;[1 1 1] Update Damage Values according to Agility Lvl of the Defender
  (bind _outactors (`GameplayStatics.GetAllActorsOfClass` "/Game/Blueprints/BP_Defender_Base.BP_Defender_Base_C"))
  (if (> (`KismetArrayLibrary.Array_Length` _outactors) 0)
    (bind _currentoffenselvl (`/Game/Blueprints/Components/BP_DroneUpgradeComponent.CurrentOffenseLvl` (`/Game/Blueprints/BP_Defender_Base.BP_DroneUpgradeComponent` (`|GetArrayItem` _outactors))))
    (if (< _currentoffenselvl 1)
      (set `self.Damage` (`self.DamageOffenseLvl0`))
      (else
        (set `self.Damage` (`self.DamageOffenseLvl1`))))
    (if (< _currentoffenselvl 2)
      (set `self.RoundsPerMinute` (`self.RoundsPerMinuteOffensiveLvl0`))
      (else
        (set `self.RoundsPerMinute` (`self.RoundsPerMinuteOffensiveLvl1`))))))

(event `Server_UpdateBBValues`
  (bind _returnvalue (`AIBlueprintHelperLibrary.GetBlackboard` self))
  ;[1 1 1] Make MinDistance available in the Blackboard
  (`/Engine/EditorBlueprintResources/StandardMacros.IsValid` _returnvalue
    (:`Is Valid`
      (`BlackboardComponent.SetValueAsFloat` _returnvalue "MinDistance" (`self.MinDistance`))
      ;[1 1 1] Make AttackRange available in the Blackboard
      (`BlackboardComponent.SetValueAsFloat` _returnvalue "AttackRange" (`self.AttackRange`))
      ;[1 1 1] Make bCanAttackMeele available in the Blackboard
      (`BlackboardComponent.SetValueAsBool` _returnvalue "bCanAttackMeele" (`self.bCanAttackMeele`)))))

(event `self.ReceiveBeginPlay`
  (bind _audio (`self.Audio`))
  (bind _investigatelocation (`self.InvestigateLocation`))
  ;[1 1 1] BeginPlay
  (`parent.ReceiveBeginPlay`)
  (`|ExecutionSequence`
    (:`then_0`
      ;[1 1 1] Run behavior tree on server only
      (`/Engine/EditorBlueprintResources/ActorMacros.Switch Has Authority`
        (:`Authority`
          (`AIController.RunBehaviorTree` (`AIBlueprintHelperLibrary.GetAIController` self) "/Game/Blueprints/AI/SentryDrone/BT_SentryDrone.BT_SentryDrone")
          (`self.Server_UpdateBBValues`)
          (`self.Server_UpdateDamageValue`)
          ;[1 1 1] Make InvestigateLocation available in the Blackboard
          (bind _asbp_game_state (cast `/Game/Blueprints/BP_GameState` (`GameplayStatics.GetGameState`))
            (:`then`
              (bind _donnavigationmanager (`/Game/Blueprints/BP_GameState.DonNavigationManager` _asbp_game_state))
              (`/Engine/EditorBlueprintResources/StandardMacros.IsValid` _donnavigationmanager
                (:`Is Valid`
                  ;;[1 1 1] Check if we can reach the destination
                  (if (`DonNavigationManager.IsLocationWithinNavigableWorld` _donnavigationmanager _investigatelocation)
                    (`BlackboardComponent.SetValueAsVector` (`AIBlueprintHelperLibrary.GetBlackboard` self) "InvestigateLocation" (`self.InvestigateLocation`))
                    (else
                      (bind (_bfoundvalidresult _returnvalue) (`DonNavigationManager.FindRandomPointAroundOriginInNavWorld` _donnavigationmanager null _investigatelocation 50.0 -1.0 50.0 5))
                      ;;[1 1 1] Try to find a possible location nearby
                      (if _bfoundvalidresult
                        (`BlackboardComponent.SetValueAsVector` (`AIBlueprintHelperLibrary.GetBlackboard` self) "InvestigateLocation" _returnvalue)
                        (else
                          ;;[1 1 1] Deactivate the investigate location by setting Z to its maximum
                          (`BlackboardComponent.SetValueAsBool` (`AIBlueprintHelperLibrary.GetBlackboard` self) "InvestigateLocationOnceVisited" true)
                          (`KismetSystemLibrary.PrintString` "BP_SentryDroneBase: No valid location found!"))))))))
            (:`CastFailed`
              (`KismetSystemLibrary.PrintString` "BP_SentryDroneBase: No Navigation Manager found!" true true (struct :`R` 1.0 :`B` 0.016369 :`A` 1.0) 60.0))))))
    (:`then_1`
      (`AudioComponent.SetSound` _audio (`self.Drone spawned`))
      (`AudioComponent.Play` _audio 0.0))))

(event `self.Fire`
  (bind _returnvalue (`KismetMathLibrary.RandomFloatInRange` -5.0 5.0))
  (bind _targetactor (`self.TargetActor`))
  (bind _returnvalue_location (`KismetMathLibrary.BreakTransform` (`SceneComponent.K2_GetComponentToWorld` (`self.MuzzleToSpawnTheProjectile`))))
  ;[1 1 1] Fire
  (`parent.Fire`)
  (`KismetSystemLibrary.Delay` (/ 60.0 (`self.RoundsPerMinute`)))
  (`|ExecutionSequence`
    (:`then_0`
      (`self.GetBBTargetActor`))
    (:`then_1`
      ;[1 1 1] Only shoot if the drone looks at its target
      (`/Engine/EditorBlueprintResources/StandardMacros.IsValid` (`self.TargetActor`)
        (:`Is Valid`
          (set `self.LooksAtTarget` (== (`self.K2_GetActorRotation`) (`KismetMathLibrary.FindLookAtRotation` (`self.K2_GetActorLocation`) (`self.K2_GetActorLocation` (`self.TargetActor`))) :`ErrorTolerance` 2.0)))))
    (:`then_2`
      ;[1 1 1] Check if the target is actualy visible
      (if (`self.LooksAtTarget`)
        (bind _outhit (`KismetSystemLibrary.LineTraceSingle` (`SceneComponent.K2_GetComponentLocation` (`self.Capsule`)) (* (- (`self.K2_GetActorLocation` (`self.TargetActor`)) (`SceneComponent.K2_GetComponentLocation` (`self.Capsule`))) 2500.0) "TraceTypeQuery2"))
        (cast `/Game/Blueprints/BP_Attacker_Base` (`.HitActor` (`GameplayStatics.BreakHitResult` _outhit))
          (:`then`
            (set `self.TargetIsNotInCover` true))
          (:`CastFailed`
            (set `self.TargetIsNotInCover` false)))))
    (:`then_3`
      ;[1 1 1] Spawn the Projectile
      (if (`self.TargetIsNotInCover`)
        (`/Engine/EditorBlueprintResources/StandardMacros.IsValid` _targetactor
          (:`Is Valid`
            (bind _asbp_attacker_base (cast `/Game/Blueprints/BP_Attacker_Base` _targetactor)
              (:`then`
                (set `self.TargetActorLocation` (- (`SceneComponent.K2_GetComponentLocation` (`/Game/Blueprints/BP_Attacker_Base.FirstPersonCamera` _asbp_attacker_base)) (`KismetMathLibrary.MakeVector` _returnvalue _returnvalue _returnvalue))))
              (:`CastFailed`
                (set `self.TargetActorLocation` (`self.K2_GetActorLocation` _targetactor))))
            (`|SpawnActorFromClass` "/Game/Blueprints/Projectiles/BP_AIProjectile_Base.BP_AIProjectile_Base_C" (`KismetMathLibrary.MakeTransform` _returnvalue_location (`KismetMathLibrary.FindLookAtRotation` _returnvalue_location (`self.TargetActorLocation`)) (0.1 0.1 0.1)) "AlwaysSpawn" "OverrideRootScale" null (`self.Damage`) null)
            (`self.Multi_ShootEffects`)))))))

(event `Multi_ShowDebugMeleeRange`
  (params (Origin :type "Vector Structure") (InnerRadius :type "Float (double-precision)") (OuterRadius :type "Float (double-precision)"))
  ;[1 1 1] Show Debug Sphere for Blast Radia
  (if (`self.bShowBlastDebugSpheres`)
    (`KismetSystemLibrary.DrawDebugSphere` Origin InnerRadius 12 (struct :`R` 1.0 :`B` 0.04112 :`A` 1.0) 10.0 20.0)
    (`KismetSystemLibrary.DrawDebugSphere` Origin OuterRadius 12 (struct :`G` 0.109804 :`B` 1.0 :`A` 1.0) 10.0 20.0)))

(event `self.Melee`
  (bind _returnvalue (`self.K2_GetActorLocation`))
  (bind _blastinnerradius (`self.BlastInnerRadius`))
  (bind _blastouterradius (`self.BlastOuterRadius`))
  ;[1 1 1] Melee
  (`parent.Melee`)
  ;[1 1 1] Delay equivalent to the BlastsPerMinute
  (`KismetSystemLibrary.Delay` (/ (`self.BlastsPerMinute`) 60.0))
  (`|ExecutionSequence`
    (:`then_0`
      (`self.GetBBTargetActor`))
    (:`then_1`
      ;[1 1 1] Create the Blast
      (cast `/Game/Blueprints/BP_Attacker_Base` (`self.TargetActor`))
      (`GameplayStatics.ApplyRadialDamageWithFalloff` :`BaseDamage` (`self.BlastMaxDamage`) :`MinimumDamage` (`self.BlastMinDamage`) :`Origin` _returnvalue :`DamageInnerRadius` _blastinnerradius :`DamageOuterRadius` _blastouterradius :`DamageFalloff` (`self.BlastDamageFalloff`) :`DamageCauser` self :`InstigatedByController` (`self.GetController` self))
      (`self.Multi_ShowDebugMeleeRange` _returnvalue _blastinnerradius _blastouterradius)
      (`self.Multi_BlastEffects`))))

(event `Multi_BlastEffects`
  (bind _returnvalue (`self.K2_GetActorLocation`))
  ;[1 1 1] Blast Effects
  (`GameplayStatics.PlaySoundAtLocation` (`self.BlastSound`) _returnvalue (struct) 1.0 1.0 0.0 null null null)
  (`GameplayStatics.SpawnEmitterAtLocation` (`self.BlastFX`) _returnvalue))

(event `Multi_ShootEffects`
  ;[1 1 1] Shoot effects
  (`GameplayStatics.PlaySoundAtLocation` (`self.ShootSound`) (`self.K2_GetActorLocation`) (struct) 1.0 1.0 0.0 null null null))

(fn `GetBBTargetActor`
  ;[1 1 1] Get BB TargetActor as Actor
  (bind _asactor (cast `Actor` (`BlackboardComponent.GetValueAsObject` (`AIController.Blackboard` (`AIBlueprintHelperLibrary.GetAIController` self)) "TargetActor")))
  (set `self.TargetActor` _asactor))

(fn `PlayAudio`
  (params (FileName :type "/Game/Blueprints/AI/Enum_Sound Enum" :default "NewEnumerator0"))
  (bind _audio (`self.Audio`))
  (`|ExecutionSequence`
    (:`then_0`
      (switch `/Game/Blueprints/AI/Enum_Sound` FileName
        (:`NewEnumerator0`
          (set `self.SoundToPlay` (`self.Engage Target`)))
        (:`NewEnumerator1`
          (set `self.SoundToPlay` (`self.Searching for Target`)))
        (:`NewEnumerator2`
          (set `self.SoundToPlay` (`self.GunSound`)))
        (:`NewEnumerator3`
          (set `self.SoundToPlay` (`self.Drone spawned`)))
        (:`NewEnumerator4`
          (set `self.SoundToPlay` (`self.Target Spotted`)))
        (:`NewEnumerator5`
          (set `self.SoundToPlay` (`self.Target Lost`)))
        (:`NewEnumerator6`
          (set `self.SoundToPlay` (`self.Target Neutralized`)))))
    (:`then_1`
      (`AudioComponent.SetSound` _audio (`self.SoundToPlay`))
      (`AudioComponent.Play` _audio 0.0))))

(fn `UserConstructionScript`)