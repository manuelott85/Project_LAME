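; Base pickup that grants energy and/or health to BP_Attacker_Base actors, then respawns.
; On the authority, an overlap with the attacker's root component passes positive amounts to its energy and health components and plays a pickup sound.
; BeginPlay and Respawn share one cycle that hides the box and disables its collision, waits RespawnTime, then restores it with a sound, so pickups start inactive.
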(event `self.ReceiveBeginPlay`
  ;[1 1 1] Deactivate the Pickup
  (`PrimitiveComponent.SetCollisionEnabled` (`self.Box`) "NoCollision" :!label _label)
  (`SceneComponent.SetVisibility` (`self.Box`) false true)
  ;[1 1 1] Wait for the respawn timer
  (`KismetSystemLibrary.Delay` (`self.RespawnTime`))
  ;[1 1 1] Activate the Pickup again
  (`SceneComponent.SetVisibility` (`self.Box`) true true)
  (`PrimitiveComponent.SetCollisionEnabled` (`self.Box`) "QueryOnly")
  ;[1 1 1] Play a Sound
  (`GameplayStatics.PlaySoundAtLocation` (`self.SoundPlayedAfterRespawning`) (`self.K2_GetActorLocation`) (struct) 1.0 1.0 0.0 null null null))

(event `Respawn`
  (goto _label))

(event `self.Box.OnComponentBeginOverlap`
  (params (OverlappedComponent :type "PrimitiveComponent Object Reference") (OtherActor :type "Actor Object Reference") (OtherComp :type "PrimitiveComponent Object Reference") (OtherBodyIndex :type Integer) (bFromSweep :type Boolean) (SweepResult :type "HitResult Structure (by ref)"))
  (`/Engine/EditorBlueprintResources/ActorMacros.Switch Has Authority`
    (:`Authority`
      (bind _asbp_attacker_base (cast `/Game/Blueprints/BP_Attacker_Base` OtherActor))
      ;[1 1 1] Only proceed if the main collision was hit (root)
      (if (== (`Actor.RootComponent` _asbp_attacker_base) OtherComp)
        (`|ExecutionSequence`
          (:`then_0`
            ;[1 1 1] Add/substract Energy if needed
            (if (> (`self.EnergyContained`) 0.0)
              (bind _bp_energycomponent (`/Game/Blueprints/BP_Attacker_Base.BP_EnergyComponent` _asbp_attacker_base))
              (`/Engine/EditorBlueprintResources/StandardMacros.IsValid` _bp_energycomponent
                (:`Is Valid`
                  (`/Game/Blueprints/Components/BP_EnergyComponent.AlterEnergy` _bp_energycomponent (`self.EnergyContained`))))))
          (:`then_1`
            ;[1 1 1] Add/substract Health if needed
            (if (> (`self.HealthContained`) 0.0)
              (bind _bp_healthcomponent (`/Game/Blueprints/BP_Attacker_Base.BP_HealthComponent` _asbp_attacker_base))
              (`/Engine/EditorBlueprintResources/StandardMacros.IsValid` _bp_healthcomponent
                (:`Is Valid`
                  (`/Game/Blueprints/Components/BP_HealthComponent.AlterHealth` _bp_healthcomponent (`self.HealthContained`))))))
          (:`then_2`
            ;[1 1 1] Play a sound and respawn the pickup
            (`GameplayStatics.PlaySoundAtLocation` (`self.SoundPlayedByPickingUp`) (`self.K2_GetActorLocation`) (struct) 1.0 1.0 0.0 null null null)
            (`self.Respawn`)))))))

(fn `UserConstructionScript`)