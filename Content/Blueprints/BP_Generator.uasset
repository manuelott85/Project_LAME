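; BP_Generator is a damageable generator actor that spawns pickups at random offsets around itself.
; The server spawns respawning pickups at BeginPlay, and accumulated damage past a threshold spawns a one-off pickup while health remains.
; Damage reaches the health component unless the shield is active or an AI projectile caused it.
; The health bar faces the camera each tick, the billboard shows only for defender pawns, and the health text update is unwired.
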(event `self.ReceiveTick`
  (params (DeltaSeconds :type "Float (single-precision)"))
  (bind _returnvalue (`GameplayStatics.GetPlayerCameraManager` 0))
  (bind _healthrotator (`self.HealthRotator`))
  ;[1 1 1] Tick
  ;[1 1 1] Rotate Healthbar
  (`/Engine/EditorBlueprintResources/StandardMacros.IsValid` _returnvalue
    (:`Is Valid`
      (`SceneComponent.K2_SetWorldRotation` _healthrotator (`KismetMathLibrary.FindLookAtRotation` (`SceneComponent.K2_GetComponentLocation` _healthrotator) (`PlayerCameraManager.GetCameraLocation` _returnvalue)) false false))))

(event `self.ReceiveBeginPlay`
  (bind _returnvalue (`GameplayStatics.GetPlayerController` 0))
  (bind _papersprite (`self.PaperSprite`))
  ;[1 1 1] BeginPlay
  (`|ExecutionSequence`
    (:`then_0`
      ;[1 1 1] Server only
      (if (or (`KismetSystemLibrary.IsServer`) (`KismetSystemLibrary.IsDedicatedServer`))
        ;[1 1 1] ForEach Pickup
        (for _ (range (`self.PickupAmount`))
          (`self.Server_SpawnPickup` true (`self.PickUpTypePermanent`)))))
    (:`then_1`
      ;[1 1 1] Set Visability of the Billboard
      (`/Engine/EditorBlueprintResources/StandardMacros.IsValid` _returnvalue
        (:`Is Valid`
          (cast `/Game/Blueprints/BP_Defender_Base` (`Controller.K2_GetPawn` _returnvalue)
            (:`then`
              (`SceneComponent.K2_SetWorldRotation` _papersprite (struct :`Roll` -90.0) false false))
            (:`CastFailed`
              (`SceneComponent.SetVisibility` _papersprite false false))))))))

(event `Server_SpawnPickup`
  (params (bShouldRespawn :type Boolean) (PickupType :type "/Game/Blueprints/PickUps/BP_DefenderPickup_Base Class Reference"))
  (bind _spawnheight (`self.SpawnHeight`))
  (bind _pickupmaxspawnradius (`self.PickupMaxSpawnRadius`))
  (bind _returnvalue (* _pickupmaxspawnradius (`KismetMathLibrary.RandomFloatInRange` -1.0 1.0)))
  (bind _returnvalue_2 (`KismetMathLibrary.Sqrt` (- (`KismetMathLibrary.Square` _pickupmaxspawnradius) (`KismetMathLibrary.Square` _returnvalue))))
  ;[1 1 1] Spawn Pickups
  ;;[1 1 1] Randomize positiv or negative vector
  (if (`KismetMathLibrary.RandomBool`)
    (set `self.SpawnPos` (`KismetMathLibrary.MakeVector` _returnvalue _returnvalue_2 _spawnheight))
    (else
      (set `self.SpawnPos` (`KismetMathLibrary.MakeVector` (* _returnvalue -1.0) (* _returnvalue_2 -1.0) _spawnheight))))
  (`|SpawnActorFromClass` PickupType (`KismetMathLibrary.MakeTransform` (+ (`self.K2_GetActorLocation`) (`self.SpawnPos`))) "AdjustIfPossibleButAlwaysSpawn" "OverrideRootScale" null self bShouldRespawn PickupType null))

(event `self.ReceiveAnyDamage`
  (params (Damage :type "Float (single-precision)") (DamageType :type "DamageType Object Reference") (InstigatedBy :type "Controller Object Reference") (DamageCauser :type "Actor Object Reference"))
  (bind _bp_healthcomponent (`self.BP_HealthComponent`))
  ;[1 1 1] Handle Damage
  ;;[1 1 1] Exclude friendly fire
  (cast `/Game/Blueprints/Projectiles/BP_AIProjectile_Base` DamageCauser
    (:`CastFailed`
      (if (not (`self.bShieldActive`))
        (`/Game/Blueprints/Components/BP_HealthComponent.Remote: Event any Damage` _bp_healthcomponent Damage DamageType InstigatedBy DamageCauser)
        ;[1 1 1] Generate Energy Pickup on Damage
        ;;[1 1 1] Proceed only, if there is some HP left
        (if (> (`/Game/Blueprints/Components/BP_HealthComponent.CurrentHealth` _bp_healthcomponent) 0.0)
          ;;[1 1 1] Does it has recieved enough damage?
          (set `self.Current_DamageRecieved` (+ (`self.Current_DamageRecieved`) Damage))
          (if (> (`self.Current_DamageRecieved`) (`self.DamageRecievedB4PickUp`))
            ;;[1 1 1] Spawn a pickup and reset the counter
            (`self.Server_SpawnPickup` false (`self.PickUpTypeDamaged`))
            (set `self.Current_DamageRecieved` 0.0)))))))

(fn `UserConstructionScript`)